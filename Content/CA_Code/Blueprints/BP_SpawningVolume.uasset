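; Spawning volume that scatters a resource actor class across the landscape inside its bounds, on BeginPlay, on a looping timer or both.
; SpawnResources uses a fixed count or derives one from the bounds' XY area and a reciprocal density.
; Each spawn line-traces vertically at random XY, placing the actor on the first Landscape hit.
; The spawn cap is checked only at BeginPlay; timer spawns neither check nor update the total.
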(event `self.ReceiveBeginPlay`
  ;[1 1 1] Spawn on begin play, timer or both
  (if (and (`self.Spawn On Begin Play`) (< (`self.Total Number Spawned`) (`self.Max Number Spawned`)))
    (`self.Spawn Resources` (`self.Spawn Number`) (`self.Spawn Resource`))
    (set `self.Total Number Spawned` (+ (`self.Spawn Number`) (`self.Total Number Spawned`))))
  (if (and (`self.Spawn On Timer`) (< (`self.Total Number Spawned`) (`self.Max Number Spawned`)))
    (`KismetSystemLibrary.K2_SetTimerDelegate` (delegate `Spawn Resources On Timer`) (`self.Timer Length`) true)))

(event `Spawn Resources On Timer`
  ;[1 1 1] Spawn on begin play, timer or both
  (`self.Spawn Resources` (`self.Spawn Number`) (`self.Spawn Resource`)))

(fn `Spawn Resources`
  (params (`Spawn Number` :type Integer) (`Spawn Resource` :type "/Game/CA_Code/Blueprints/ResourceActors/BP_MasterResource Class Reference"))
  (locals (`Spawn Amount Local` :type Integer :default 99999) (`L Spawn Resource` :type "/Game/CA_Code/Blueprints/ResourceActors/BP_MasterResource Class Reference") (`L X Random Float` :type "Float (double-precision)") (`L Y Random Float` :type "Float (double-precision)"))
  (bind (_origin _boxextent) (`self.GetActorBounds` false))
  (bind _x (.x _boxextent))
  (bind _y (.y _boxextent))
  (bind _x_2 (.x (+ _origin (`KismetMathLibrary.MakeVector` (`KismetMathLibrary.RandomFloatInRange` (- _x (* _x 2.0)) _x) (`KismetMathLibrary.RandomFloatInRange` (- _y (* _y 2.0)) _y) (.z _origin)))))
  (bind _y_2 (.y (+ _origin (`KismetMathLibrary.MakeVector` (`KismetMathLibrary.RandomFloatInRange` (- _x (* _x 2.0)) _x) (`KismetMathLibrary.RandomFloatInRange` (- _y (* _y 2.0)) _y) (.z _origin)))))
  ;[0.05522 1 0.02144] Set local variables
  (set `local.Spawn Amount Local` `Spawn Number`)
  (set `local.L Spawn Resource` `Spawn Resource`)
  ;[1 0.2114 0.2346] Density or fix Amount?
  (if (`self.IsByDensity`)
    ;[0.03449 0 1] Get the size of the spawner's box
    (bind _output_get (set `self.SizeOfSpawnerBox` (* (* (.x (`.BoxExtent` (`self.GetActorBounds` false))) 2.0) (* (.y (`.BoxExtent` (`self.GetActorBounds` false))) 2.0))))
    ;[1 0.8382 0] Determine appropriate amount by density
    (bind _output_get_2 (set `self.Amount from Density` (`KismetMathLibrary.FTrunc` (/ _output_get (`self.SpawnerDensity Reziproke`)))))
    (set `local.Spawn Amount Local` _output_get_2))
  ;[1 1 1] Loop for the number of actors to spawn
  (for _ (range 1 (+ (`local.Spawn Amount Local`) 1))
    ;[1 1 1] Set random floats
    (set `local.L X Random Float` (`KismetMathLibrary.RandomFloatInRange` 0.1 1.5))
    (set `local.L Y Random Float` (`KismetMathLibrary.RandomFloatInRange` 0.1 1.5))
    ;[0.2357 1 0.7777] place resources on the landscape
    (bind _outhits (`KismetSystemLibrary.LineTraceMultiForObjects` (`KismetMathLibrary.MakeVector` _x_2 _y_2 100000.0) (`KismetMathLibrary.MakeVector` _x_2 _y_2 -100000.0) (`|MakeArray` "ObjectTypeQuery1" :!type "EObjectTypeQuery Enum")))
    (for _array_element _outhits
      (bind (_bblockinghit _binitialoverlap _time _distance _location _impactpoint _normal _impactnormal _physmat _hitactor) (`GameplayStatics.BreakHitResult` _array_element))
      (cast `Landscape` _hitactor)
      (`|ExecutionSequence`
        (:`then_0`
          ;[1 1 1] Spawn actor at random location
          (`|SpawnActorFromClass` (`local.L Spawn Resource`) (`KismetMathLibrary.Conv_VectorToTransform` _location) "AlwaysSpawn" "OverrideRootScale" null 1000 null))
        (:`then_1`
          (break))))))

(fn `UserConstructionScript`)