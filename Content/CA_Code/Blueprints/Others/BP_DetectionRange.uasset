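; BP_DetectionRange is a detection sphere actor that trails a target actor, typically a BP_MasterUnit.
; OnSpawned sets the sphere radius; for a unit, it registers itself as that unit's DetectionRange and starts a looping quarter-second timer to follow it.
; Non-unit targets only get a one-time snap to their location.
; The actor destroys itself when its target is invalid, and CheckOverlapping is an empty stub.
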(event `On Spawned`
  (params (`Follow Actor` :type "Actor Object Reference") (`Detection Zone Size` :type "Float (double-precision)"))
  (`/Engine/EditorBlueprintResources/StandardMacros.IsValid` `Follow Actor`
    (:`Is Valid`
      (set `self.Following Actor` `Follow Actor`)
      (`SphereComponent.SetSphereRadius` (`self.Detection Sphere`) `Detection Zone Size` true)
      (bind _asbp_master_unit (cast `/Game/CA_Code/Blueprints/UnitActors/BP_MasterUnit` (`self.Following Actor`))
        (:`then`
          (set `self.Following Unit` _asbp_master_unit)
          (`KismetSystemLibrary.K2_SetTimerDelegate` (delegate `Follow Actor`) 0.25 true)
          (set `/Game/CA_Code/Blueprints/UnitActors/BP_MasterUnit.Detection Range` self (`self.Following Unit`)))
        (:`CastFailed`
          (`self.K2_SetActorLocationAndRotation` (`self.K2_GetActorLocation` (`self.Following Actor`)) :!label _label))))
    (:`Is Not Valid`
      (`self.K2_DestroyActor` :!label _label_2))))

(event `Follow Actor`
  (`/Engine/EditorBlueprintResources/StandardMacros.IsValid` (`self.Following Actor`)
    (:`Is Valid`
      (goto _label))
    (:`Is Not Valid`
      (goto _label_2))))

(fn `Check Overlapping`
  (locals (`Overlapping Unit` :type "/Game/CA_Code/Blueprints/UnitActors/BP_MasterUnit Object Reference")))

(fn `UserConstructionScript`)