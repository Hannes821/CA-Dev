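; Blueprint that starts the game's background music on BeginPlay when IsMusicOn is set.
; PlayBackgroundMusic spawns CA_MS_Game as a 2D sound, caches it in CurrentMusicBG to avoid spawning while one is valid, and flags MusicPlayingInPlayer.
; A separate PlayIntroVideo graph, not called from the event graph, adds CA_IntroWidget to the viewport on first main menu open, with a debug print and short delay.
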(event `self.ReceiveBeginPlay`
  (if (`self.IsMusicOn`)
    ;[0.2514 0.2753 1] Add MainMenuMusic
    (`self.PlayBackgroundMusic`)))

(fn `PlayBackgroundMusic`
  (returns (CurrentMusicPlaying :type "AudioComponent Object Reference"))
  (`self.Current Music BG`
    (:`then`)
    (:`else`
      (bind _returnvalue (`GameplayStatics.SpawnSound2D` "/Game/CA_Audio/Music/Recorded/CA_MS_Game.CA_MS_Game" 1.0 1.0 0.0 null))
      (bind _output_get (set `self.Current Music BG` _returnvalue))
      (set `self.Music Playing in Player` true)
      (return _output_get))))

(fn `UserConstructionScript`)