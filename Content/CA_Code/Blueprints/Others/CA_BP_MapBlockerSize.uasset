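; Map blocker actor whose box collision defines the area used to limit RTS pawn camera movement.
; GetSize returns the box's scaled extent.
; GetSize2 returns world-space min and max corners by offsetting the actor location by that extent, serving as the camera bounds.
; The event graph and construction script hold no logic.
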(fn `GetSize`
  (returns (ScaleBoxXYZ :type "Vector Structure"))
  (return (`BoxComponent.GetScaledBoxExtent` (`self.BoxCollision`))))

(fn `GetSize2`
  (returns (min :type "Vector Structure") (max :type "Vector Structure"))
  (bind _returnvalue (`self.K2_GetActorLocation`))
  (bind _returnvalue_2 (* (`BoxComponent.GetScaledBoxExtent` (`self.BoxCollision`)) 1.0))
  ;[0 0.03398 1] getting the extension size of our map blocker as a base to limit movement of camera in the RTSPAWN
  (return (- _returnvalue _returnvalue_2) (+ _returnvalue _returnvalue_2)))

(fn `UserConstructionScript`)