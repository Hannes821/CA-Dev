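; Main menu music player that starts the background playlist, after the intro widget ends if the game instance has not yet flagged it played.
; SetMusicOn/Off stores the catalogue track and, on the macro's "No Custom Music Playing" branch, mutes the playlist and binds to that track's finish.
; On finish, the same check gates respawning the playlist as 2D sound.
; The check reads the music widget's pressed flags, finding it by interface.
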(event `self.ReceiveBeginPlay`
  (bind _asca_gi_game_instance_01 (cast `/Game/CA_Code/Blueprints/Player/CA_GI_GameInstance01` (`GameplayStatics.GetGameInstance`)))
  (if (`/Game/CA_Code/Blueprints/Player/CA_GI_GameInstance01.IntroWasPlayed` _asca_gi_game_instance_01)
    (`self.StartPlayMusic`)
    (else
      (bind _returnvalue (`|CreateWidget` "/Game/Movies/CA_IntroWidget.CA_IntroWidget_C"))
      (add `/Game/Movies/CA_IntroWidget.OnIntroEnd` _returnvalue (delegate `StartPlayMusic`))
      (`UserWidget.AddToViewport` _returnvalue 0)
      (set `/Game/CA_Code/Blueprints/Player/CA_GI_GameInstance01.IntroWasPlayed` true _asca_gi_game_instance_01))))

(event `StartPlayMusic`
  ;[0.2514 0.2753 1] Add MainMenuMusic
  (`self.PlayBackgroundMusic` (`self.Music Playlist MainMenu`)))

(event `/Game/CA_Code/Blueprints/Interfaces/BPI_Level-Music.SetMusicOn/Off`
  (params (CurrentMusicShowing :type "AudioComponent Object Reference"))
  ;[0 1 0.1929] if custom music is played by the widget for our music catalogue, then we mute the background music, and after its done, we add the backgroundmusic again!
  (set `self.Shown Music` CurrentMusicShowing)
  (set `self.Music Playing MM` false)
  (`self.IsCustomMusicFromMusicMenuPlayed`
    (:`NoCustomMusicPlaying`
      (`AudioComponent.AdjustVolume` (`self.Current Music Playlist`) 0.0 0.0 "Linear")
      (add `AudioComponent.OnAudioFinished` (`self.Shown Music`) (delegate `OnAudioFinished_Event`)))))

(event `OnAudioFinished_Event`
  ;[0 1 0.1929] if custom music is played by the widget for our music catalogue, then we mute the background music, and after its done, we add the backgroundmusic again!
  (`self.IsCustomMusicFromMusicMenuPlayed`
    (:`NoCustomMusicPlaying`
      ;;[0.2514 0.2753 1] Add MainMenuMusic again
      (`self.PlayBackgroundMusic` (`self.Music Playlist MainMenu`)))))

(fn `CheckIfCustomMusicAlreadyPlayed`
  (bind _foundwidgets (`WidgetBlueprintLibrary.GetAllWidgetsWithInterface` "/Game/CA_Code/Blueprints/Interfaces/BPI_Level-Music.BPI_Level-Music_C"))
  (bind _asca_mw_music (cast `/Game/CA_Code/Blueprints/Widgets/MainMenu/2D_Widgets/History_SubMenus/CA_MW-Music` (`|GetArrayItem` _foundwidgets)))
  (if (or (`/Game/CA_Code/Blueprints/Widgets/MainMenu/2D_Widgets/History_SubMenus/CA_MW-Music.IsPressedM1` _asca_mw_music) (`/Game/CA_Code/Blueprints/Widgets/MainMenu/2D_Widgets/History_SubMenus/CA_MW-Music.IsPressedM2` _asca_mw_music) (`/Game/CA_Code/Blueprints/Widgets/MainMenu/2D_Widgets/History_SubMenus/CA_MW-Music.IsPressedM3` _asca_mw_music) (`/Game/CA_Code/Blueprints/Widgets/MainMenu/2D_Widgets/History_SubMenus/CA_MW-Music.IsPressedM4` _asca_mw_music) (`/Game/CA_Code/Blueprints/Widgets/MainMenu/2D_Widgets/History_SubMenus/CA_MW-Music.IsPressedM5` _asca_mw_music))
    _))

(fn `PlayBackgroundMusic`
  (params (`Music Playlist` :type "SoundBase Object Reference"))
  (returns (IsMusicPlaying :type Boolean) (CurrentMusicPlaylist :type "AudioComponent Object Reference"))
  (bind _returnvalue (`GameplayStatics.SpawnSound2D` `Music Playlist` 1.0 1.0 0.0 null))
  (bind _output_get (set `self.Current Music Playlist` _returnvalue))
  (bind _output_get_2 (set `self.Music Playing MM` true))
  (return _output_get_2 _output_get))

(fn `UserConstructionScript`)