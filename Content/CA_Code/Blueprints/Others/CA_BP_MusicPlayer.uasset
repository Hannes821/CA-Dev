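; Music player actor that shows the intro widget on BeginPlay, then after the intro delay starts the instrumental background playlist as main menu music.
; SetMusicOn/Of receives another audio component, mutes the background music instantly and binds to that component's OnAudioFinished.
; When that audio ends, it spawns a fresh playlist sound rather than restoring the muted one, with MusicPlayingMM tracking the menu music state.
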(event `self.ReceiveBeginPlay`
  ;[0 1 0.2726] intro video
  (bind _returnvalue (`|CreateWidget` "/Game/Movies/CA_IntroWidget.CA_IntroWidget_C"))
  (`UserWidget.AddToViewport` _returnvalue 0)
  (`KismetSystemLibrary.Delay` (`self.Intro Duration`))
  ;[0.2514 0.2753 1] Add MainMenuMusic
  (bind _returnvalue_2 (`GameplayStatics.SpawnSound2D` "/Game/CA_Audio/Music/Recorded/Playlist_Instrumental_CA.Playlist_Instrumental_CA" 1.0 1.0 0.0 null))
  (set `self.Current Music BG` _returnvalue_2)
  (set `self.Music Playing MM` true))

(event `/Game/CA_Code/Blueprints/Interfaces/BPI_CA_MMLevelToPlayMusicWidget.SetMusicOn/Of`
  (params (CurrentMusicShowing :type "AudioComponent Object Reference"))
  (bind _output_get (set `self.Shown Music` CurrentMusicShowing))
  (`KismetSystemLibrary.PrintString` (`KismetSystemLibrary.GetDisplayName` _output_get))
  (`KismetSystemLibrary.PrintString` "XXXXXX!")
  (set `self.Music Playing MM` false)
  (`AudioComponent.AdjustVolume` (`self.Current Music BG`) 0.0 0.0 "Linear")
  (add `AudioComponent.OnAudioFinished` (`self.Shown Music`) (delegate `OnAudioFinished_Event`)))

(event `OnAudioFinished_Event`
  ;[0.2514 0.2753 1] Add MainMenuMusic again
  (bind _returnvalue (`GameplayStatics.SpawnSound2D` "/Game/CA_Audio/Music/Recorded/Playlist_Instrumental_CA.Playlist_Instrumental_CA" 1.0 1.0 0.0 null))
  (set `self.Current Music BG` _returnvalue)
  (set `self.Music Playing MM` true))

(fn `UserConstructionScript`)