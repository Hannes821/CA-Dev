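; Blueprint function library with a helper that finds the actor of a given class nearest to a target location.
; FindNearestActorOfClass gets all actors of that class and loops through them, comparing each one's distance to the target against the closest recorded so far.
; It returns the nearest actor along with its distance and location.
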(fn `Find Nearest Actor Of Class`
  (params (Class :type "Actor Class Reference") (TargetLocation :type "Vector Structure"))
  (returns (NearestActor :type "Actor Object Reference") (NearestDistance :type "Float (double-precision)") (NearestActorLocation :type "Vector Structure"))
  (locals (Loc_NearestDistance :type "Float (double-precision)" :default 10000.0) (Loc_NearestActor :type "Actor Object Reference") (Loc_NearestActorLocation :type "Vector Structure"))
  (bind _outactors (`GameplayStatics.GetAllActorsOfClass` null Class))
  (for _array_element _outactors
    (bind _returnvalue (`Actor.K2_GetActorLocation` _array_element))
    (bind _returnvalue_2 (`KismetMathLibrary.Vector_Distance` _returnvalue (`local.TargetLocation`)))
    ;[1 1 1] get relative distance to others.
    (if (< _returnvalue_2 (`local.Loc_NearestDistance`))
      ;[1 1 1] set newest closest
      (set `local.Loc_NearestDistance` _returnvalue_2)
      (set `local.Loc_NearestActor` _array_element)
      (set `local.Loc_NearestActorLocation` _returnvalue)))
  (return (`local.Loc_NearestActor`) (`local.Loc_NearestDistance`) (`local.Loc_NearestActorLocation`)))