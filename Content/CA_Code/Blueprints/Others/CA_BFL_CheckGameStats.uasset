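; Blueprint function library for reading and incrementing named game stats stored on the game instance.
; A helper casts the game instance to CA_GI_GameInstance01, giving the other functions access to its GameStats map.
; AddToGameStats adds a value to an existing entry and ignores names not already in the map.
; ReadGameStats returns the value stored under a given name.
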(fn `AddToGameStats`
  (params (StatName :type String) (Value :type Integer))
  (locals (LocalStatName :type String) (LocalStatValue :type Integer))
  (set `local.LocalStatName` StatName)
  (set `local.LocalStatValue` Value)
  (bind _gameinstance (`self.GetGameStats` null))
  (bind _gamestats (`/Game/CA_Code/Blueprints/Player/CA_GI_GameInstance01.GameStats` _gameinstance))
  (bind (_value _returnvalue) (`BlueprintMapLibrary.Map_Find` _gamestats (`local.LocalStatName`)))
  (if _returnvalue
    (`BlueprintMapLibrary.Map_Add` _gamestats (`local.LocalStatName`) (+ (`local.LocalStatValue`) _value))))

(fn `GetGameStats`
  (returns (GameInstance :type "/Game/CA_Code/Blueprints/Player/CA_GI_GameInstance01 Object Reference"))
  (bind _asca_gi_game_instance_01 (cast `/Game/CA_Code/Blueprints/Player/CA_GI_GameInstance01` (`GameplayStatics.GetGameInstance` null)))
  (return _asca_gi_game_instance_01))

(fn `ReadGameStats`
  (params (GameStatName :type String))
  (returns (GameStatValue :type Integer))
  (locals (TemporaryReadingStatName :type String))
  (set `local.TemporaryReadingStatName` GameStatName)
  (bind _gameinstance (`self.GetGameStats` null))
  (return (`BlueprintMapLibrary.Map_Find` (`/Game/CA_Code/Blueprints/Player/CA_GI_GameInstance01.GameStats` _gameinstance) (`local.TemporaryReadingStatName`))))