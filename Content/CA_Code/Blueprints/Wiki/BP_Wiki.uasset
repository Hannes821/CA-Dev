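; BP_Wiki is an item info lookup that serves wiki entries, including names and descriptions, by IndividualTag.
; InitWiki copies every row of the WikiData table into WikiMap, keyed by tag.
; GetInfoByTag reads that map, falling back to NoneItem with an IsNone flag.
; GetNameAndDescription wraps it, but its branch is inverted: found tags return "Unknown" text, while missing tags return NoneItem's text with IsNone false.
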(fn `Get Name and Description`
  (params (IndividualTag :type "GameplayTag Structure"))
  (returns (Name :type Text) (Description :type Text) (IsNone :type Boolean))
  (bind (_iteminfo _isnone) (`self.GetInfoByTag` IndividualTag))
  (if _isnone
    (bind (_individualtag _alltags _name _description) (break `/Game/CA_Code/Blueprints/Wiki/Base_object_info` _iteminfo))
    (return _name _description false)
    (else
      (return "Name Unknown" "Description Unknown" true))))

(fn `GetInfoByTag`
  (params (IndividualTag :type "GameplayTag Structure"))
  (returns (ItemInfo :type "/Game/CA_Code/Blueprints/Wiki/Base_object_info Structure") (IsNone :type Boolean))
  (bind (_value _returnvalue) (`BlueprintMapLibrary.Map_Find` (`self.WikiMap`) IndividualTag))
  (if _returnvalue
    (return _value false)
    (else
      (return (`self.NoneItem`) true))))

(fn `InitWiki`
  ;[1 1 1] Just WikiData->GetAllRows<> in c++
  (bind _outrownames (`DataTableFunctionLibrary.GetDataTableRowNames` (`self.WikiData`)))
  (for _array_element _outrownames
    (bind _returnvalue (`|GetDataTableRow` (`self.WikiData`) _array_element)
      (:`then`
        (`BlueprintMapLibrary.Map_Add` (`self.WikiMap`) (`.IndividualTag_13_050D4ADF463E5CEB9E6E5D97077ABC60` (break `/Game/CA_Code/Blueprints/Wiki/Base_object_info` _returnvalue)) _returnvalue)))))