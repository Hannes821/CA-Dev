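; Game state Blueprint that tracks connected players for the player list UI and creates the game's wiki object.
; UpdatePlayerListInGameState copies PlayerArray into AllPlayerStates, whose OnRep refreshes every CA_WB_PlayerList widget.
; The construction script builds and initialises a BP_Wiki instance stored as GameWiki.
; OnGameEndEvaluation gathers player names into a list and only prints a debug message.
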(event `OnGameEndEvaluation`
  (for _array_element (`self.PlayerArray`)
    (`KismetArrayLibrary.Array_Add` (`self.PlayersNameList`) (`PlayerState.GetPlayerName` _array_element)))
  (`KismetSystemLibrary.PrintString` "We have a list of player names now.-"))

(event `UpdatePlayerListInGameState`
  (set `self.AllPlayerStates` (`self.PlayerArray`)))

(fn `Init Wiki`
  (bind _returnvalue (`|GenericCreateObject` "/Game/CA_Code/Blueprints/Wiki/BP_Wiki.BP_Wiki_C"))
  (bind _output_get (set `self.GameWiki` _returnvalue))
  (`/Game/CA_Code/Blueprints/Wiki/BP_Wiki.InitWiki` _output_get))

(fn `OnRep_AllPlayerStates`
  (bind _foundwidgets (`WidgetBlueprintLibrary.GetAllWidgetsOfClass` "/Game/CA_Code/Blueprints/Player/CA_WB_PlayerList.CA_WB_PlayerList_C" false))
  (for _array_element _foundwidgets
    (`/Game/CA_Code/Blueprints/Player/CA_WB_PlayerList.UpdatePlayerListWidget` _array_element)))

(fn `UserConstructionScript`
  (`self.Init Wiki`))