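; Camera pawn that edge-scrolls across the world when the cursor nears the viewport edges.
; MouseX and MouseY axis events run every tick, normalise cursor position against viewport size, and offset the actor along world Y and X respectively.
; Movement is ScrollSpeed scaled by delta seconds for frame-rate independence.
; Trigger bands are asymmetric, much wider at the left and top than at the right and bottom.
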(event `InputAxisKey|MouseX`
  (params (AxisValue :type "Float (single-precision)"))
  (bind (_returnvalue_x _returnvalue_y) (`KismetMathLibrary.BreakVector2D` (`WidgetLayoutLibrary.GetViewportSize`)))
  (bind _returnvalue (* (`GameplayStatics.GetWorldDeltaSeconds`) (`self.ScrollSpeed`)))
  (bind _returnvalue_2 (/ (`PlayerController.GetMousePosition` (`GameplayStatics.GetPlayerController` 0)) _returnvalue_x))
  ;[1 1 1] Edge Scrolling
  ;;[1 1 1] evey tick
  (if (> _returnvalue_2 0.98)
    ;;[1 1 1] mouse X event effect moving camera to side (y) in world
    (`self.K2_AddActorWorldOffset` (`KismetMathLibrary.MakeVector` 0.0 _returnvalue))
    (elif (< _returnvalue_2 0.2)
      (`self.K2_AddActorWorldOffset` (`KismetMathLibrary.MakeVector` 0.0 (* _returnvalue -1.0))))))

(event `InputAxisKey|MouseY`
  (params (AxisValue :type "Float (single-precision)"))
  (bind (_returnvalue_x _returnvalue_y) (`KismetMathLibrary.BreakVector2D` (`WidgetLayoutLibrary.GetViewportSize`)))
  (bind _returnvalue (* (`GameplayStatics.GetWorldDeltaSeconds`) (`self.ScrollSpeed`)))
  (bind _returnvalue_2 (/ (`.LocationY` (`PlayerController.GetMousePosition` (`GameplayStatics.GetPlayerController` 0))) _returnvalue_y))
  ;[1 1 1] Edge Scrolling
  ;;[1 1 1] evey tick
  (if (> _returnvalue_2 0.98)
    ;;[1 1 1] mouse Y event effect moving camera to front/back (x) in world
    (`self.K2_AddActorWorldOffset` (`KismetMathLibrary.MakeVector` (* _returnvalue -1.0)))
    (elif (< _returnvalue_2 0.2)
      (`self.K2_AddActorWorldOffset` (`KismetMathLibrary.MakeVector` _returnvalue)))))

(fn `UserConstructionScript`)