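; CA_PlayerState is a player state Blueprint that gives the player starting resources through its CAResourceStorageComponent.
; On BeginPlay it binds DebugResources to the component's resource value change event, then adds StartResources.
; DebugResources is currently empty, as the ResDebug helper that prints the resource type and new count on screen is disconnected.
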(event `self.ReceiveBeginPlay`
  (bind _ca_resourcestoragecomponent (`self.CA_ResourceStorageComponent`))
  (add `/Game/CA_Code/Blueprints/ActorsComponents/ResourceStorage/CA_ResourceStorageComponent.OnResourceValueChange` _ca_resourcestoragecomponent (delegate `DebugResources`))
  (`/Game/CA_Code/Blueprints/ActorsComponents/ResourceStorage/CA_ResourceStorageComponent.Add Resources` _ca_resourcestoragecomponent (`self.StartResources`)))

(event `DebugResources`
  (params (ResoourceType :type "/Game/CA_Code/Blueprints/Others/E_CA_Resources Enum" :default "NewEnumerator0") (NewCount :type Integer) (Owner :type "Actor Object Reference")))

(fn `ResDebug`
  (params (ResType :type "/Game/CA_Code/Blueprints/Others/E_CA_Resources Enum" :default "NewEnumerator0") (Count :type Integer))
  (`KismetSystemLibrary.PrintString` (`KismetStringLibrary.Concat_StrStr` "Resource " (`|GetEnumeratorNameAsString` ResType) " new value" (`KismetStringLibrary.Conv_IntToString` Count)) true true (struct :`R` 0.033035 :`G` 1.0 :`A` 1.0) 10.0))

(fn `UserConstructionScript`)