(fn `Add New Building`
  (params (`New Building In` :type "/Game/CA_Code/Blueprints/BuildingActors/MasterBuilding Object Reference"))
  (`KismetArrayLibrary.Array_Add` (`self.Buildings Owned`) `New Building In`)
  (return))

(fn `Add New Unit`
  (params (`Unit In` :type "/Game/CA_Code/Blueprints/UnitActors/BP_MasterUnit Object Reference"))
  (if (> (`/Game/CA_Code/Blueprints/UnitActors/BP_MasterUnit.MeleeDamage` `Unit In`) 0.0)
    (`KismetArrayLibrary.Array_Add` (`self.Defence Units`) `Unit In`))
  (`KismetArrayLibrary.Array_Add` (`self.Units Owned`) `Unit In`)
  (return))

(fn `Add Resources`
  (params (`+ Wood` :type Integer) (`+ Stone` :type Integer) (`+ Brick` :type Integer) (`+ Food` :type Integer))
  (locals (`Wood L` :type Integer) (`Stone L` :type Integer) (`Brick L` :type Integer) (`Food L` :type Integer))
  (set `local.Wood L` `+ Wood`)
  (set `local.Stone L` `+ Stone`)
  (set `local.Brick L` `+ Brick`)
  (set `local.Food L` `+ Food`)
  (set `self.Wood` (+ (`self.Wood`) (`local.Wood L`)))
  (set `self.Stone` (+ (`self.Stone`) (`local.Stone L`)))
  (set `self.Brick` (+ (`self.Brick`) (`local.Brick L`)))
  (set `self.Food` (+ (`self.Food`) (`local.Food L`)))
  (return))

(fn `Check Building Health`
  (returns (`Return Value` :type Boolean) (`Building Repair` :type "/Game/CA_Code/Blueprints/BuildingActors/MasterBuilding Object Reference"))
  (locals (`Repair Building L` :type "/Game/CA_Code/Blueprints/BuildingActors/MasterBuilding Object Reference"))
  (bind _repair_building_l (`local.Repair Building L`))
  (for _array_element (`self.Buildings Owned`)
    (if (not (`/Game/CA_Code/Blueprints/ActorsComponents/AttributeComponents/BaseAttributeComponent.IsFull` (`/Game/CA_Code/Blueprints/BuildingActors/MasterBuilding.StabilityComponent` _array_element)))
      (set `local.Repair Building L` _array_element)
      (break)))
  (return (`KismetSystemLibrary.IsValid` _repair_building_l) _repair_building_l))

(fn `Check Requierments`
  (params (`Unit Checking` :type "/Game/CA_Code/Blueprints/UnitActors/BP_MasterUnit Class Reference"))
  (locals (`Unit L` :type "/Game/CA_Code/Blueprints/UnitActors/BP_MasterUnit Class Reference") (`Selected Building` :type "/Game/CA_Code/Blueprints/BuildingActors/MasterBuilding Object Reference")))

(fn `Construct Starter Units`
  (params (`Priority 1` :type "/Game/CA_Code/Blueprints/UnitActors/BP_MasterUnit Class Reference") (`Priority 2` :type "/Game/CA_Code/Blueprints/UnitActors/BP_MasterUnit Class Reference") (`Priority 3` :type "/Game/CA_Code/Blueprints/UnitActors/BP_MasterUnit Class Reference") (`Priority 4` :type "/Game/CA_Code/Blueprints/UnitActors/BP_MasterUnit Class Reference"))
  (locals (`Can get Wood` :type Boolean) (`Can get Stone` :type Boolean) (`Unit Priority` :type "Array of /Game/CA_Code/Blueprints/UnitActors/BP_MasterUnit Class Reference") (NewLocalVar_0 :type "/Game/CA_Code/Blueprints/Others/E_CA_Resources Enum") (NewLocalVar_1 :type "/Game/CA_Code/Blueprints/Others/S_AIBuilding Structure" :default (struct :`1` "/Script/Engine.BlueprintGeneratedClass'\"/Game/CA_Code/Blueprints/BuildingActors/BA01_FarmersBarn.BA01_FarmersBarn_C\"'")) (`Can Build` :type Boolean)))

(fn `Deduct Resources`
  (params (`Wood -` :type Integer) (`Stone -` :type Integer) (`Brick -` :type Integer) (`Food -` :type Integer))
  (set `self.Wood` (- (`self.Wood`) `Wood -`))
  (set `self.Stone` (- (`self.Stone`) `Stone -`))
  (set `self.Brick` (- (`self.Brick`) `Brick -`))
  (set `self.Food` (- (`self.Food`) `Food -`))
  (return))

(fn `Defence Building Placement`
  (params (`Defence Building In` :type "/Game/CA_Code/Blueprints/BuildingActors/MasterBuilding Class Reference") (`Max Towers Per Building` :type Integer :default 2))
  (returns (`Can Build Out` :type Boolean) (`Build Location Out` :type "Vector Structure"))
  (locals (`Index L` :type Integer) (`Build Location L` :type "Vector Structure") (`Can Place L` :type Boolean) (`Trace Expansion L` :type "Float (double-precision)") (`Low Tower L` :type Integer :default 1) (`Building Defending L` :type "/Game/CA_Code/Blueprints/BuildingActors/MasterBuilding Object Reference") (`Defence Class L` :type "/Game/CA_Code/Blueprints/BuildingActors/MasterBuilding Class Reference") (`Max Towers L` :type Integer) (`Array Element L` :type "/Game/CA_Code/Blueprints/BuildingActors/MasterBuilding Object Reference"))
  (bind _array_element_l (`local.Array Element L`))
  (bind _building_defending_l (`local.Building Defending L`))
  (bind (_returnvalue_roll _returnvalue_pitch _returnvalue_yaw) (`KismetMathLibrary.BreakRotator` (`self.K2_GetActorRotation` (`local.Building Defending L`))))
  (bind _towers (`/Game/CA_Code/Blueprints/BuildingActors/MasterBuilding.Towers` (`local.Array Element L`)))
  (bind _returnvalue (`StaticMesh.GetBoundingBox` (`.BuildingStaticMesh_3_732171C843913D8B686F2BA9E84231A6` (break `/Game/CA_Code/Blueprints/Others/S_StaticMesh` (`.Building Static Mesh` (defaults `Object` (`local.Defence Class L`)))))))
  (bind _returnvalue_2 (+ (* (`KismetMathLibrary.Conv_RotatorToVector` (`KismetMathLibrary.MakeRotator` _returnvalue_roll _returnvalue_pitch (+ _returnvalue_yaw (+ (`KismetMathLibrary.Conv_IntToDouble` (* (`local.Index L`) 36)) (`KismetMathLibrary.Conv_IntToDouble` (* (`/Game/CA_Code/Blueprints/BuildingActors/MasterBuilding.Towers` (`local.Building Defending L`)) 120)))))) (+ 1100.0 (* (`local.Trace Expansion L`) 400.0))) (`self.K2_GetActorLocation` (`local.Building Defending L`))))
  (set `local.Max Towers L` `Max Towers Per Building`)
  (set `local.Low Tower L` 1)
  (set `local.Defence Class L` `Defence Building In`)
  (set `local.Building Defending L` null)
  (for _array_element (`self.Buildings Owned`)
    (set `local.Array Element L` _array_element)
    (if (`/Game/CA_Code/Blueprints/BuildingActors/MasterBuilding.Defence Building` _array_element)
      _
      (elif (< (`/Game/CA_Code/Blueprints/BuildingActors/MasterBuilding.Towers` (`local.Array Element L`)) (`local.Max Towers L`))
        (if (== _towers 0)
          (if (< _towers (`local.Low Tower L`))
            (set `local.Building Defending L` _array_element_l)
            (break)
            (else
              (set `local.Low Tower L` (`/Game/CA_Code/Blueprints/BuildingActors/MasterBuilding.Towers` (`local.Array Element L`))))))
        (set `local.Building Defending L` _array_element_l)
        (else
          (set `local.Building Defending L` null)))))
  (`/Engine/EditorBlueprintResources/StandardMacros.IsValid` (`local.Building Defending L`)
    (:`Is Valid`
      (set `/Game/CA_Code/Blueprints/BuildingActors/MasterBuilding.Towers` (+ (`/Game/CA_Code/Blueprints/BuildingActors/MasterBuilding.Towers` _building_defending_l) 1) _building_defending_l)
      (for _index (range 11) :!label _label
        (set `local.Index L` _index)
        (bind (_outhit _returnvalue_3) (`KismetSystemLibrary.BoxTraceSingle` (+ _returnvalue_2 (0.0 0.0 300000.0)) (- _returnvalue_2 (0.0 0.0 30000.0)) (`KismetMathLibrary.MakeVector` (.x (`.Max` (break `Box` _returnvalue))) (.y (`.Max` (break `Box` _returnvalue)))) (struct) "TraceTypeQuery1"))
        (if _returnvalue_3
          (bind (_bblockinghit _binitialoverlap _time _distance _location _impactpoint _normal _impactnormal _physmat _hitactor) (`GameplayStatics.BreakHitResult` _outhit))
          (bind _returnvalue_4 (`GameplayStatics.GetObjectClass` _hitactor))
          (if (or (== _returnvalue_4 "/Script/Landscape.Landscape") (== _returnvalue_4 "/Script/Landscape.LandscapeProxy"))
            (set `local.Build Location L` _location)
            (set `local.Can Place L` true)
            (break)
            (else
              _)))
        (set `local.Can Place L` false))
      (if (`local.Can Place L`)
        (return true (`local.Build Location L`))
        (elif (< (`local.Trace Expansion L`) 3.0)
          (set `local.Trace Expansion L` (+ (`local.Trace Expansion L`) 1.0))
          (goto _label)
          (else
            (return false (0.0 0.0 0.0))))))
    (:`Is Not Valid`
      (return false (0.0 0.0 0.0)))))

(fn `Get Attacking Units`
  (returns (`Units Out` :type "Array of /Game/CA_Code/Blueprints/UnitActors/BP_MasterUnit Object Reference"))
  (return (`self.Attacking Units`)))

(fn `Get Next Building`
  (params (`Array In` :type "Array of /Game/CA_Code/Blueprints/BuildingActors/MasterBuilding Class Reference"))
  (returns (`Allow Build` :type Boolean) (`Building Out` :type "/Game/CA_Code/Blueprints/BuildingActors/MasterBuilding Class Reference"))
  (locals (`Index L` :type Integer) (`Next Building L` :type Boolean) (`Building Class L` :type "/Game/CA_Code/Blueprints/BuildingActors/MasterBuilding Class Reference") (`Defence Building L` :type "/Game/CA_Code/Blueprints/BuildingActors/MasterBuilding Class Reference") (`Array L` :type "Array of /Game/CA_Code/Blueprints/BuildingActors/MasterBuilding Class Reference") (`H Unit Cap L` :type Integer))
  (bind _building_class_l (`local.Building Class L`))
  (bind _defence_building_l (`local.Defence Building L`))
  (bind _output (`|GetArrayItem` (`local.Array L`) (`local.Index L`)))
  (set `local.Array L` `Array In`)
  (if (< (- (`self.Max Units`) (`self.Current Units`)) 1)
    (if (< (`self.Max Units`) (`self.Max Unit Max`))
      (for _array_element (`local.Array L`)
        (bind (_assigned_builder _building_material_instance _rts_pawn _required_slacked_lime _required_iron _unit_capacity) (defaults `Object` _array_element))
        (if (> _unit_capacity (`local.H Unit Cap L`))
          (set `local.H Unit Cap L` _unit_capacity)
          (set `local.Building Class L` _array_element)))
      (if (`KismetSystemLibrary.IsValidClass` (`local.Building Class L`))
        (return true (`local.Building Class L`))
        (else
          _))))
  (set `local.Index L` 0)
  (for _array_element_2 (`self.Buildings Owned`) :!label _label
    (if (`KismetSystemLibrary.IsValidClass` _output)
      (if (== (`GameplayStatics.GetObjectClass` _array_element_2) _output)
        (if (`.Defence Building` (defaults `Object` _output))
          (set `local.Defence Building L` _output))
        (set `local.Next Building L` true)
        (break)
        (else
          (set `local.Next Building L` false)
          (set `local.Building Class L` _output)))))
  (if (`local.Next Building L`)
    (if (<= (`local.Index L`) (`KismetArrayLibrary.Array_Length` (`local.Array L`)))
      (set `local.Index L` (+ (`local.Index L`) 1))
      (goto _label)
      (else
        _))
    (elif (`KismetSystemLibrary.IsValidClass` _building_class_l)
      (return true _building_class_l)
      (else
        _)))
  (if (`KismetSystemLibrary.IsValidClass` _defence_building_l)
    (return true _defence_building_l)
    (else
      (return false null))))

(fn `Get Unit`
  (params (`Get By Resource` :type "/Game/CA_Code/Blueprints/ResourceActors/BP_MasterResource Class Reference") (`Get By Builder` :type Boolean) (`Get By Can Attack` :type Boolean) (`Return Array` :type Boolean) (`Attack Damge Filter` :type "Float (double-precision)"))
  (returns (`Unit Out` :type "/Game/CA_Code/Blueprints/UnitActors/BP_MasterUnit Object Reference") (`Units Out` :type "Array of /Game/CA_Code/Blueprints/UnitActors/BP_MasterUnit Object Reference"))
  (locals (Resource :type "/Game/CA_Code/Blueprints/ResourceActors/BP_MasterResource Class Reference") (Builder :type Boolean) (Attack :type Boolean) (`Selected Unit` :type "/Game/CA_Code/Blueprints/UnitActors/BP_MasterUnit Object Reference") (`Return Array L` :type Boolean) (`Selected Units L` :type "Array of /Game/CA_Code/Blueprints/UnitActors/BP_MasterUnit Object Reference") (`Array Element L` :type "/Game/CA_Code/Blueprints/UnitActors/BP_MasterUnit Object Reference"))
  (bind _resource (`local.Resource`))
  (bind _meleedamage (`/Game/CA_Code/Blueprints/UnitActors/BP_MasterUnit.MeleeDamage` (`local.Array Element L`)))
  (set `local.Return Array L` `Return Array`)
  (set `local.Resource` `Get By Resource`)
  (set `local.Builder` `Get By Builder`)
  (set `local.Attack` `Get By Can Attack`)
  (for _array_element (`self.Units Owned`)
    (bind _output_get (set `local.Array Element L` _array_element))
    (`/Engine/EditorBlueprintResources/StandardMacros.IsValid` _output_get
      (:`Is Valid`
        (if (`KismetSystemLibrary.IsValidClass` _resource)
          (if (== (`/Game/CA_Code/Blueprints/UnitActors/BP_MasterUnit.Resource Unit Can Collect` _array_element) _resource)
            (set `local.Selected Unit` (`local.Array Element L`))
            (if (`local.Return Array L`)
              (`KismetArrayLibrary.Array_Add` (`local.Selected Units L`) (`local.Array Element L`))
              (else
                (break))))
          (elif (`local.Builder`)
            (if (`/Game/CA_Code/Blueprints/UnitActors/BP_MasterUnit.Builder` (`local.Array Element L`))
              (set `local.Selected Unit` (`local.Array Element L`))
              (if (`local.Return Array L`)
                (`KismetArrayLibrary.Array_Add` (`local.Selected Units L`) (`local.Array Element L`))
                (else
                  (break))))
            (elif (`local.Attack`)
              (if (> `Attack Damge Filter` 0.0)
                (if (> _meleedamage `Attack Damge Filter`)
                  (if (> _meleedamage 0.0) :!label _label
                    (set `local.Selected Unit` (`local.Array Element L`))
                    (if (`local.Return Array L`)
                      (`KismetArrayLibrary.Array_Add` (`local.Selected Units L`) (`local.Array Element L`))
                      (else
                        (break)))))
                (else
                  (goto _label)))))))))
  (return (`local.Selected Unit`) (`local.Selected Units L`)))

(fn `Get Unit Count`
  (params (`Unit Class` :type "/Game/CA_Code/Blueprints/UnitActors/BP_MasterUnit Class Reference"))
  (returns (`Unit Count` :type Integer))
  (locals (Unit :type "/Game/CA_Code/Blueprints/UnitActors/BP_MasterUnit Class Reference") (Count :type Integer))
  (set `local.Unit` `Unit Class`)
  (for _array_element (`self.Units Owned`)
    (if (== (`GameplayStatics.GetObjectClass` _array_element) (`local.Unit`))
      (set `local.Count` (+ (`local.Count`) 1))))
  (return (`local.Count`)))

(fn `Remove Buildings`
  (params (`Remove Building` :type "/Game/CA_Code/Blueprints/BuildingActors/MasterBuilding Object Reference"))
  (`KismetArrayLibrary.Array_RemoveItem` (`self.Buildings Owned`) `Remove Building`)
  (return))

(fn `Remove Units`
  (params (`Remove Unit` :type "/Game/CA_Code/Blueprints/UnitActors/BP_MasterUnit Object Reference"))
  (`KismetArrayLibrary.Array_RemoveItem` (`self.Units Owned`) `Remove Unit`)
  (set `self.Current Units` (- (`self.Current Units`) 1))
  (`KismetArrayLibrary.Array_RemoveItem` (`self.Attacking Units`) `Remove Unit`)
  (`KismetArrayLibrary.Array_RemoveItem` (`self.Defence Units`) `Remove Unit`)
  (return))

(fn `Requiered Units`
  (returns (Wood :type Boolean) (Stone :type Boolean))
  (locals (`Can Get Wood` :type Boolean) (`Can Get Stone` :type Boolean))
  (for _array_element (`self.Buildings Owned`)
    (bind _allowedresources (`/Game/CA_Code/Blueprints/ActorsComponents/ResourceStorage/CA_ResourceStorageComponent.GetAllowedResources` (`/Game/CA_Code/Blueprints/BuildingActors/MasterBuilding.CA_ResourceStorageComponent` _array_element)))
    (if (`BlueprintSetLibrary.Set_Contains` _allowedresources "NewEnumerator56")
      (set `local.Can Get Wood` true)
      (elif (`BlueprintSetLibrary.Set_Contains` _allowedresources "NewEnumerator20")
        (set `local.Can Get Stone` true))))
  (return (`local.Can Get Wood`) (`local.Can Get Stone`)))

(fn `Set Building Actions`
  (params (Referance :type "/Game/CA_Code/Blueprints/BuildingActors/MasterBuilding Object Reference"))
  (locals (`Building Reference` :type "/Game/CA_Code/Blueprints/BuildingActors/MasterBuilding Object Reference"))
  (bind (_assigned_builder _building_material_instance _rts_pawn _required_slacked_lime _required_iron _mesh_reset_materials _resource_to_generate _unit_attacking _ai_name_enum _ai_player _generation_amount _generation_speed _convert_amount) (defaults `Object` (`GameplayStatics.GetObjectClass` (`local.Building Reference`))))
  (set `local.Building Reference` Referance)
  (if (or (> _generation_amount 0) (> _convert_amount 0))
    (`/Game/CA_Code/Blueprints/BuildingActors/MasterBuilding.Building has Highest Priority` (`local.Building Reference`))
    (return)
    (else
      (return))))

(fn `Sort Unit Prioritys`
  (params (Units :type "Array of /Game/CA_Code/Blueprints/UnitActors/BP_MasterUnit Class Reference") (Resource :type "/Game/CA_Code/Blueprints/ResourceActors/BP_MasterResource Class Reference") (Builder :type Boolean) (`Can Attack` :type Boolean))
  (locals (`Resource L` :type "/Game/CA_Code/Blueprints/ResourceActors/BP_MasterResource Class Reference") (`Unit L` :type "/Game/CA_Code/Blueprints/UnitActors/BP_MasterUnit Class Reference") (`Builder L` :type Boolean) (`Units L` :type "Array of /Game/CA_Code/Blueprints/UnitActors/BP_MasterUnit Class Reference") (`Can Attack L` :type Boolean) (`Highist attack` :type "Float (double-precision)")))

(fn `UserConstructionScript`)