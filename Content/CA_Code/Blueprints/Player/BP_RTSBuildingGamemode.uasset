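; BP_RTSBuildingGamemode is the RTS game mode that tracks connected player controllers.
; PostLogin and OnLogout add or remove BP_RTSController references in an array, then trigger UpdatePlayerList.
; After a short delay, that event tells CA_BP_GameState to update its player list.
; KickPlayer ignores its PlayerID input and calls OwningClientKickPlayer on the first stored controller.
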(event `self.K2_PostLogin`
  (params (NewPlayer :type "PlayerController Object Reference"))
  (bind _asbp_rtscontroller (cast `/Game/CA_Code/Blueprints/Player/BP_RTSController` NewPlayer))
  (`KismetArrayLibrary.Array_Add` (`self.AllPlayerControllersRefs`) _asbp_rtscontroller)
  (`self.UpdatePlayerList` :!label _label))

(event `UpdatePlayerList`
  (`KismetSystemLibrary.Delay` 0.3)
  (bind _asca_bp_game_state (cast `/Game/CA_Code/Blueprints/Player/CA_BP_GameState` (`GameplayStatics.GetGameState`)))
  (`/Game/CA_Code/Blueprints/Player/CA_BP_GameState.UpdatePlayerListInGameState` _asca_bp_game_state))

(event `self.K2_OnLogout`
  (params (ExitingController :type "Controller Object Reference"))
  (bind _asbp_rtscontroller (cast `/Game/CA_Code/Blueprints/Player/BP_RTSController` ExitingController))
  (`KismetArrayLibrary.Array_RemoveItem` (`self.AllPlayerControllersRefs`) _asbp_rtscontroller)
  (goto _label))

(fn `KickPlayer`
  (params (PlayerID :type Integer))
  (`/Game/CA_Code/Blueprints/Player/BP_RTSController.OwningClient_KickPlayer` (`|GetArrayItem` (`self.AllPlayerControllersRefs`))))

(fn `UserConstructionScript`)