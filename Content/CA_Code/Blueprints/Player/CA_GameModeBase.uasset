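; CA_GameModeBase is the game mode that gives each joining player an RTS pawn at a random start camp.
; Construction gathers all CA_PlayerStartCamp actors; each new player possesses a BP_RTSPawn spawned at a camp's camera location, receives that camp, which then leaves the pool to prevent sharing.
; BeginPlay adds the input mapping context, player list widget and Game-and-UI input with locked mouse, only for player controller 0.
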(event `self.ReceiveBeginPlay`
  (bind _returnvalue (pcsubsystem `EnhancedInputLocalPlayerSubsystem` (`GameplayStatics.GetPlayerController` 0)))
  (`/Engine/EditorBlueprintResources/StandardMacros.IsValid` _returnvalue
    (:`Is Valid`
      (message `EnhancedInputSubsystemInterface.AddMappingContext` _returnvalue "/Game/CA_Code/Inputs/IMC_CAECE.IMC_CAECE" 0 (struct))
      (if (`Controller.IsLocalPlayerController` (`GameplayStatics.GetPlayerController` 0))
        (bind _returnvalue_2 (`|CreateWidget` "/Game/CA_Code/Blueprints/Player/CA_WB_PlayerList.CA_WB_PlayerList_C" (`GameplayStatics.GetPlayerController` 0)))
        (`UserWidget.AddToViewport` _returnvalue_2 0)
        (`WidgetBlueprintLibrary.SetInputMode_GameAndUIEx` (`GameplayStatics.GetPlayerController` 0) null "LockAlways")
        (else
          (`KismetSystemLibrary.PrintString` "NOT LOCAL PLAYER CONTROLLER"))))
    (:`Is Not Valid`
      (`KismetSystemLibrary.PrintString` "Player Controlled Invalid"))))

(event `self.HandleStartingNewPlayer`
  (params (NewPlayer :type "PlayerController Object Reference"))
  ;[1 1 1] get random start location
  (set `self.SelectedPlayerStartCamp` (`KismetArrayLibrary.Array_Random` (`self.PlayerStartCamps`)))
  (bind _returnvalue (`|SpawnActorFromClass` "/Game/CA_Code/Blueprints/Player/BP_RTSPawn.BP_RTSPawn_C" (`SceneComponent.K2_GetComponentToWorld` (`/Game/CA_Code/Blueprints/Player/CA_PlayerStartCamp.CameraLocation` (`self.SelectedPlayerStartCamp`))) "Undefined" "MultiplyWithRoot" null null))
  (`Controller.Possess` NewPlayer _returnvalue)
  (message `/Game/CA_Code/Blueprints/Interfaces/BPI_PlayerStart.SetupPlayerStart` NewPlayer (`self.SelectedPlayerStartCamp`))
  ;[1 1 1] make sure not 2 players at the same location!
  (`KismetArrayLibrary.Array_RemoveItem` (`self.PlayerStartCamps`) (`self.SelectedPlayerStartCamp`)))

(event `self.K2_PostLogin`
  (params (NewPlayer :type "PlayerController Object Reference")))

(event `self.K2_OnLogout`
  (params (ExitingController :type "Controller Object Reference")))

(fn `UserConstructionScript`
  (bind _outactors (`GameplayStatics.GetAllActorsOfClass` "/Game/CA_Code/Blueprints/Player/CA_PlayerStartCamp.CA_PlayerStartCamp_C"))
  (set `self.PlayerStartCamps` _outactors))