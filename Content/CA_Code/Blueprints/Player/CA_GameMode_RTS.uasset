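; RTS game mode that tracks player controllers on login and logout, then triggers a delayed player list refresh in the GameState.
; Helper functions define base colours and eight two-tone team palettes, but colour assignment is unfinished and none are called here.
; KickPlayer ignores its ID and always targets the first controller.
; Victory condition events are empty stubs, and the AI player spawn call is disconnected.
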(event `self.K2_PostLogin`
  (params (NewPlayer :type "PlayerController Object Reference"))
  (bind _asbp_rtscontroller (cast `/Game/CA_Code/Blueprints/Player/BP_RTSController` NewPlayer))
  (`KismetArrayLibrary.Array_Add` (`self.AllPlayerControllersRefs`) _asbp_rtscontroller)
  (`self.UpdatePlayerList` :!label _label))

(event `self.K2_OnLogout`
  (params (ExitingController :type "Controller Object Reference"))
  (bind _asbp_rtscontroller (cast `/Game/CA_Code/Blueprints/Player/BP_RTSController` ExitingController))
  (`KismetArrayLibrary.Array_RemoveItem` (`self.AllPlayerControllersRefs`) _asbp_rtscontroller)
  (goto _label))

(event `UpdatePlayerList`
  (`KismetSystemLibrary.Delay` 0.3)
  (bind _asca_bp_game_state (cast `/Game/CA_Code/Blueprints/Player/CA_BP_GameState` (`GameplayStatics.GetGameState`)))
  (`/Game/CA_Code/Blueprints/Player/CA_BP_GameState.UpdatePlayerListInGameState` _asca_bp_game_state))

(event `KeepConquered`)

(event `CastleLordDead`)

(event `Trade Route Established`)

(fn `AssignColours`
  (bind _asca_bp_game_state (cast `/Game/CA_Code/Blueprints/Player/CA_BP_GameState` (`GameplayStatics.GetGameState`)))
  (for (_array_element _array_index) (`GameStateBase.PlayerArray` _asca_bp_game_state)
    (`/Engine/EditorBlueprintResources/StandardMacros.IsValid` _array_element
      (:`Is Valid`
        (bind _output_get (set `self.Array Index` _array_index))
        (for (_array_element_2 _array_index_2) (`self.VirtualColourList`)
          (if (== _output_get _array_index_2)
            _))
        (set `self.PlayerColourMap` (`|MakeMap` (`PlayerState.GetPlayerController` _array_element) _array_element_2))))))

(fn `GetBaseColours`
  (set `self.BaseColourGold` (0.7 0.4 0.0))
  (set `self.BaseColourSilver` (0.7 0.7 0.7))
  (set `self.BaseColourRed` (0.25 0.015 0.015))
  (set `self.BaseColourBlue` (0.0125 0.01 0.25))
  (set `self.BaseColourGreen` (0.01 0.06 0.02))
  (set `self.BaseColourBlack` (0.01 0.01 0.01))
  (`KismetSystemLibrary.PrintString` "Base colours have been set"))

(fn `GetPlayerColours`
  (bind _basecoloursilver (`self.BaseColourSilver`))
  (bind _player01_silverred (`self.Player01_SilverRed`))
  (bind _player02_silverblue (`self.Player02_SilverBlue`))
  (bind _player03_silvergreen (`self.Player03_SilverGreen`))
  (bind _player04_silverblack (`self.Player04_SilverBlack`))
  (bind _player05_goldred (`self.Player05_GoldRed`))
  (bind _player06_goldblue (`self.Player06_GoldBlue`))
  (bind _player07_goldgreen (`self.Player07_GoldGreen`))
  (bind _player08_goldblack (`self.Player08_GoldBlack`))
  (bind _basecolourgold (`self.BaseColourGold`))
  (`KismetArrayLibrary.Array_Clear` (`self.TeamColours`))
  (`KismetArrayLibrary.Array_Add` _player01_silverred _basecoloursilver)
  (`KismetArrayLibrary.Array_Add` _player01_silverred (`self.BaseColourRed`))
  (`KismetArrayLibrary.Array_Add` _player02_silverblue _basecoloursilver)
  (`KismetArrayLibrary.Array_Add` _player02_silverblue (`self.BaseColourBlue`))
  (`KismetArrayLibrary.Array_Add` _player03_silvergreen _basecoloursilver)
  (`KismetArrayLibrary.Array_Add` _player03_silvergreen (`self.BaseColourGreen`))
  (`KismetArrayLibrary.Array_Add` _player04_silverblack _basecoloursilver)
  (`KismetArrayLibrary.Array_Add` _player04_silverblack (`self.BaseColourBlack`))
  (`KismetArrayLibrary.Array_Add` _player05_goldred _basecolourgold)
  (`KismetArrayLibrary.Array_Add` _player05_goldred (`self.BaseColourRed`))
  (`KismetArrayLibrary.Array_Add` _player06_goldblue _basecolourgold)
  (`KismetArrayLibrary.Array_Add` _player06_goldblue (`self.BaseColourBlue`))
  (`KismetArrayLibrary.Array_Add` _player07_goldgreen _basecolourgold)
  (`KismetArrayLibrary.Array_Add` _player07_goldgreen (`self.BaseColourGreen`))
  (`KismetArrayLibrary.Array_Add` _player08_goldblack _basecolourgold)
  (`KismetArrayLibrary.Array_Add` _player08_goldblack (`self.BaseColourBlack`))
  (`KismetSystemLibrary.PrintString` "Team Colours have been set!"))

(fn `KickPlayer`
  (params (PlayerID :type Integer))
  (`/Game/CA_Code/Blueprints/Player/BP_RTSController.OwningClient_KickPlayer` (`|GetArrayItem` (`self.AllPlayerControllersRefs`))))

(fn `SpawnAIPlayer`
  (bind _returnvalue (`|SpawnActorFromClass` "/Game/CA_Code/Blueprints/Player/BP_AIPlayer.BP_AIPlayer_C" (`KismetMathLibrary.MakeTransform` (0.0 0.0 0.0)) "Undefined" "OverrideRootScale" null null))
  (set `/Game/CA_Code/Blueprints/Player/BP_AIPlayer.AI Name` "NewEnumerator0" _returnvalue))

(fn `UserConstructionScript`)