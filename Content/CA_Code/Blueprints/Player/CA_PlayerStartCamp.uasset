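; Player start camp actor that periodically brings new villagers to its owning player.
; On BeginPlay it picks a road sign mesh from a map keyed by owner player number and starts a looping timer.
; Each timer tick spawns a villager at StartUnit01 if the player has open beds and is popular, passing on owner number and clutter meshes.
; Spawning is skipped if collision cannot be resolved, and debug prints report the result.
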(event `OnTimerTriggers`
  ;[0.2301 0.3074 0.6719] check if conditions are met to get villagers
  (if (`self.PlayerHasOpenBeds`)
    (if (`self.PlayerisPopular`)
      ;[0.3953 1 0.5183] Get new villagers
      (bind _returnvalue (`|SpawnActorFromClass` "/Game/CA_Code/Blueprints/UnitActors/BP_Unit_Civil_Villager.BP_Unit_Civil_Villager_C" (`KismetMathLibrary.MakeTransform` (`SceneComponent.K2_GetComponentLocation` (`self.StartUnit01`))) "AdjustIfPossibleButDontSpawnIfColliding" "MultiplyWithRoot" null "NewEnumerator4" (`self.OwnerPlayerNr`) (`self.Unit Clutter Meshes`) null))
      (if (`KismetSystemLibrary.IsValid` _returnvalue)
        (bind _returnvalue_2 (`KismetSystemLibrary.GetDisplayName` _returnvalue))
        (`KismetSystemLibrary.PrintString` _returnvalue_2)
        (`KismetSystemLibrary.PrintString` "was successfully spawned" true true (struct :`R` 0.110872 :`G` 1.0 :`A` 1.0) 10.0)
        (else
          (`KismetSystemLibrary.PrintString` _returnvalue_2)
          (`KismetSystemLibrary.PrintString` "we must have failed" true true (struct :`R` 1.0 :`B` 0.060741 :`A` 1.0) 10.0))))))

(event `self.ReceiveBeginPlay`
  ;[1 1 1] set a unique road sign per player number.
  (`StaticMeshComponent.SetStaticMesh` (`self.RoadSign`) (`BlueprintMapLibrary.Map_Find` (`self.RoadSignsMap`) (`self.OwnerPlayerNr`)))
  (`KismetSystemLibrary.K2_SetTimerDelegate` (delegate `OnTimerTriggers`) 10.0 true))

(fn `UserConstructionScript`)