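; Game instance that hosts online sessions and stores per-player identity and colour data.
; HostSession creates an eight-player session, then opens the dark main-menu level as a listen server.
; Functions define base colours, build eight two-colour player pairs, and map player controllers to name, house, banner, colour and title, which GetPlayerInfo returns with a validity flag.
; An event caches building and unit data-table row names, but its binding never runs.
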(event `OnEventBeginPlay_Event`
  (bind _outrownames (`DataTableFunctionLibrary.GetDataTableRowNames` "/Game/CA_Code/DataTables/CA_BuildingsBuiltDatatable.CA_BuildingsBuiltDatatable"))
  (set `self.ArrayBuildingsBuild` _outrownames)
  (bind _outrownames_2 (`DataTableFunctionLibrary.GetDataTableRowNames` "/Game/CA_Code/DataTables/CA_UnitsSpawnedDatatable.CA_UnitsSpawnedDatatable"))
  (set `self.ArrayUnitsSpawned` _outrownames_2))

(event `HostSession`
  ;[1 1 1] host session
  (`CreateSessionCallbackProxy.CreateSession` (`GameplayStatics.GetPlayerController` 0) 8
    (:`OnSuccess`
      (`GameplayStatics.OpenLevelBySoftObjectPtr` "/Game/CA_Maps/CA_MainMenu_DarkBackground.CA_MainMenu_DarkBackground" true "?listen")
      (`KismetSystemLibrary.PrintString` "A new session was launched!" true true (struct :`G` 1.0 :`B` 0.056588 :`A` 1.0) 10.0))))

(fn `GetPlayerInfo`
  (params (PlayerController :type "PlayerController Object Reference"))
  (returns (House :type Text) (Name :type Text) (Colour :type Integer) (Title :type Text) (Banner :type "MaterialInstance Object Reference") (IsAllCorrect :type Boolean))
  (bind (_value _returnvalue) (`BlueprintMapLibrary.Map_Find` (`self.Player Banner Ref`) (`local.PlayerController`)))
  (bind (_value_2 _returnvalue_2) (`BlueprintMapLibrary.Map_Find` (`self.Player House Ref`) (`local.PlayerController`)))
  (bind (_value_3 _returnvalue_3) (`BlueprintMapLibrary.Map_Find` (`self.Player Name Ref`) (`local.PlayerController`)))
  (bind (_value_4 _returnvalue_4) (`BlueprintMapLibrary.Map_Find` (`self.Player Colour Ref`) (`local.PlayerController`)))
  (bind (_value_5 _returnvalue_5) (`BlueprintMapLibrary.Map_Find` (`self.Player Title Ref`) (`local.PlayerController`)))
  (return _value_2 _value_3 _value_4 _value_5 _value (and _returnvalue_2 _returnvalue_3 _returnvalue_4 _returnvalue_5 _returnvalue)))

(fn `Set Player Banner W Controller Ref`
  (params (`Controller Ref` :type "Controller Object Reference (by ref)") (`Banner Material In Ref` :type "MaterialInstance Object Reference (by ref)"))
  (`BlueprintMapLibrary.Map_Add` (`self.Player Banner Ref`) `Controller Ref` `Banner Material In Ref`))

(fn `Set Player Colour W Controller Ref`
  (params (Key :type "Controller Object Reference (by ref)") (Value :type "Integer (by ref)"))
  (`BlueprintMapLibrary.Map_Add` (`self.Player Colour Ref`) Key Value))

(fn `Set Player House W Controller Ref`
  (params (`Controller Ref` :type "Controller Object Reference (by ref)") (House :type "Text (by ref)"))
  (`BlueprintMapLibrary.Map_Add` (`self.Player House Ref`) `Controller Ref` House))

(fn `Set Player Name W Controller Ref`
  (params (PlayerControllerRef :type "Controller Object Reference") (PlayerName :type Text))
  (`BlueprintMapLibrary.Map_Add` (`self.Player Name Ref`) PlayerControllerRef PlayerName))

(fn `Set Player Title W Controller Ref`
  (params (`Controller Ref` :type "Controller Object Reference (by ref)") (Title :type "Text (by ref)"))
  (`BlueprintMapLibrary.Map_Add` (`self.Player Title Ref`) `Controller Ref` Title))

(fn `SetGameColours`
  (set `self.BaseColourGold` (0.7 0.4 0.0))
  (set `self.BaseColourSilver` (0.7 0.7 0.7))
  (set `self.BaseColourRed` (0.25 0.015 0.015))
  (set `self.BaseColourBlue` (0.0125 0.01 0.25))
  (set `self.BaseColourGreen` (0.01 0.06 0.02))
  (set `self.BaseColourBlack` (0.01 0.01 0.01))
  (`KismetSystemLibrary.PrintString` "Base colours have been set"))

(fn `SetPlayerColours`
  (bind _basecoloursilver (`self.BaseColourSilver`))
  (bind _player01_silverred (`self.Player01_SilverRed`))
  (bind _player02_silverblue (`self.Player02_SilverBlue`))
  (bind _player03_silvergreen (`self.Player03_SilverGreen`))
  (bind _player04_silverblack (`self.Player04_SilverBlack`))
  (bind _player05_goldred (`self.Player05_GoldRed`))
  (bind _player06_goldblue (`self.Player06_GoldBlue`))
  (bind _player07_goldgreen (`self.Player07_GoldGreen`))
  (bind _player08_goldblack (`self.Player08_GoldBlack`))
  (bind _basecolourgold (`self.BaseColourGold`))
  (`KismetArrayLibrary.Array_Clear` (`self.TeamColours`))
  (`KismetArrayLibrary.Array_Add` _player01_silverred _basecoloursilver)
  (`KismetArrayLibrary.Array_Add` _player01_silverred (`self.BaseColourRed`))
  (`KismetArrayLibrary.Array_Add` _player02_silverblue _basecoloursilver)
  (`KismetArrayLibrary.Array_Add` _player02_silverblue (`self.BaseColourBlue`))
  (`KismetArrayLibrary.Array_Add` _player03_silvergreen _basecoloursilver)
  (`KismetArrayLibrary.Array_Add` _player03_silvergreen (`self.BaseColourGreen`))
  (`KismetArrayLibrary.Array_Add` _player04_silverblack _basecoloursilver)
  (`KismetArrayLibrary.Array_Add` _player04_silverblack (`self.BaseColourBlack`))
  (`KismetArrayLibrary.Array_Add` _player05_goldred _basecolourgold)
  (`KismetArrayLibrary.Array_Add` _player05_goldred (`self.BaseColourRed`))
  (`KismetArrayLibrary.Array_Add` _player06_goldblue _basecolourgold)
  (`KismetArrayLibrary.Array_Add` _player06_goldblue (`self.BaseColourBlue`))
  (`KismetArrayLibrary.Array_Add` _player07_goldgreen _basecolourgold)
  (`KismetArrayLibrary.Array_Add` _player07_goldgreen (`self.BaseColourGreen`))
  (`KismetArrayLibrary.Array_Add` _player08_goldblack _basecolourgold)
  (`KismetArrayLibrary.Array_Add` _player08_goldblack (`self.BaseColourBlack`))
  (`KismetSystemLibrary.PrintString` "Team Colours have been set!"))