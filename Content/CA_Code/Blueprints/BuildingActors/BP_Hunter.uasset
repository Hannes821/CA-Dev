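; BP_Hunter is a hunter building in the RTS that recruits and upgrades units and stores resources.
; Its construction script extends the parent's, setting up compatible storage for Wood and Bark and a maximum stability.
; Events hide the RTS pawn's HUD and recruit the building's unit on the highest-priority event.
; The abandon-button event, despite its name, triggers a food-costed unit upgrade to carrying amount and time.
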(event `Set HUD Visibilitys_1`
  (`/Game/CA_Code/Blueprints/Player/BP_RTSPawn.Set HUD Visibilitys` (`self.RTS Pawn`) "Hidden"))

(event `self.Building has Highest Priority`
  (`self.Recruit Unit` (`self.Recruitment Unit`)))

(event `self.Building to be abandoned Button clicked`
  (`self.Upgrade Units` 2 1.0 3 (`self.Recruitment Unit`) 0.0 0.0 200))

(fn `UserConstructionScript`
  (`parent.UserConstructionScript`)
  ;[1 1 1] wood and bark resource setup
  (bind _output_get (set `self.ResourceStorageType1` "Wood"))
  (bind _output_get_2 (set `self.ResourceStorageType2` "Bark"))
  (set `self.ResourceStorageTypeVariety` 2)
  (set `self.ResourceStorageType1Count` 0)
  (set `self.ResourcesCompatibleStorage` (`|MakeArray` _output_get _output_get_2))
  (set `self.Max Stability` 50.0))