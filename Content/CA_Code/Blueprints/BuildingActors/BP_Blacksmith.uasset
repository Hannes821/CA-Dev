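; BP_Blacksmith is a blacksmith building actor that shows a fire effect once it is built.
; Each Tick runs the parent logic, then sets the fire particle system's visibility, children included, from ConstructionComplete.
; The construction script runs the parent's script and adds the Building.Typ.Tannery gameplay tag, which does not match the blacksmith name.
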(event `self.ReceiveTick`
  (params (DeltaSeconds :type "Float (single-precision)"))
  (`parent.ReceiveTick` DeltaSeconds)
  (if (`self.Construction Complete`)
    (`SceneComponent.SetVisibility` (`self.ParticleSystemFire`) true true)
    (else
      (`SceneComponent.SetVisibility` (`self.ParticleSystemFire`) false true))))

(fn `UserConstructionScript`
  (locals (NewLocalVar :type "GameplayTag Structure"))
  (`parent.UserConstructionScript`)
  (`BlueprintGameplayTagLibrary.AddGameplayTag` (`self.Tag Container_0`) (struct :`TagName` "Building.Typ.Tannery")))