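; Construction-script spline actor that builds a crenelated wall along CASpline, with support pillars at its points.
; It fills each spline segment with stretched spline meshes, swaps in addon meshes at listed indices and can level them into horizontal steps.
; Pillars are instanced static meshes rotated by spline point type.
; Optionally it snaps points to terrain by line trace or deforms the Landscape along the spline via EditorApplySpline.
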(fn `UserConstructionScript`
  (locals (NewLocalVar :type "Transform Structure") (CurrentTransform :type "Transform Structure"))
  (bind _currentsplineindex (`self.CurrentSplineIndex`))
  (bind _caspline (`self.CASpline`))
  (bind _deformwidth (`self.DeformWidth`))
  (bind _deformoffset (`self.DeformOffset`))
  (bind _caspline_2 (`self.CASpline`))
  (bind _caspline_3 (`self.CASpline`))
  (bind _returnvalue (`SplineComponent.GetDistanceAlongSplineAtSplinePoint` _caspline _currentsplineindex))
  (bind _returnvalue_2 (`SplineComponent.GetTransformAtSplinePoint` (`self.CASpline`) (`self.CurrentSplineIndex`) "Local" false))
  (bind _returnvalue_3 (`SplineComponent.GetTransformAtSplinePoint` (`self.CASpline`) (`self.CurrentSplineIndex`) "Local" false))
  (bind _returnvalue_4 (`SplineComponent.GetTransformAtSplinePoint` (`self.CASpline`) (`self.CurrentSplineIndex`) "Local" false))
  (bind _location (.location (`SplineComponent.GetTransformAtSplinePoint` (`self.CASpline`) (`self.CurrentSplineIndex`) "Local" false)))
  (bind _scale (.scale (`SplineComponent.GetTransformAtSplinePoint` (`self.CASpline`) (`self.CurrentSplineIndex`) "Local" false)))
  (`parent.UserConstructionScript`)
  (set `self.StaticMeshWallSegment` "/Game/CA_Buildings/Meshes/StoneWalls/Crenelationsv2.Crenelationsv2")
  (bind _staticmeshwallsegment (`self.StaticMeshWallSegment`)
    (:`then`
      (`|ExecutionSequence`
        (:`then_0`
          ;[0 0.4544 1] conform to landscape
          (if (`self.bConformToLandscape`)
            (set `self.bDeformLandscape` false)
            (for _index (range (`SplineComponent.GetNumberOfSplinePoints` (`self.CASpline`)))
              (bind (_returnvalue_x _returnvalue_y _returnvalue_z) (`KismetMathLibrary.BreakVector` (`SplineComponent.GetLocationAtSplinePoint` (`self.CASpline`) _index "World")))
              (bind _outhit (`KismetSystemLibrary.LineTraceSingle` (`KismetMathLibrary.MakeVector` _returnvalue_x _returnvalue_y (+ _returnvalue_z 2000.0)) (`KismetMathLibrary.MakeVector` _returnvalue_x _returnvalue_y (- _returnvalue_z 2000.0)) "TraceTypeQuery1"))
              (`SplineComponent.SetLocationAtSplinePoint` (`self.CASpline`) _index (`.Location` (`GameplayStatics.BreakHitResult` _outhit)) "World" true))))
        (:`then_1`
          ;[1 1 1] set the intersection /end of spline segments (angle/cut off) covering static mesh
          (bind _returnvalue_5 (`AddComponent|NODE_AddInstancedStaticMeshComponent-0`))
          (bind _output_get (set `self.PIllarInstanceStaticMesh` _returnvalue_5))
          (`StaticMeshComponent.SetStaticMesh` _output_get (`self.StaticMeshSegmentIntersectionSupportBeam`)))
        (:`then_2`
          (bind (_returnvalue_min _returnvalue_max) (break `Box` (`StaticMesh.GetBoundingBox` _staticmeshwallsegment)))
          (bind _returnvalue_x_2 (`KismetMathLibrary.BreakVector` (- _returnvalue_max _returnvalue_min)))
          ;[1 1 1] calc mesh length
          (set `self.MeshLength` _returnvalue_x_2))
        (:`then_3`
          (for _index_2 (range (+ (- (`SplineComponent.GetNumberOfSplinePoints` _caspline) 2) 1))
            (set `self.CurrentSplineIndex` _index_2)
            ;[1 1 1] is it a corner spline point (does it need support beams?)
            (`|ExecutionSequence`
              (:`then_0`
                ;[0 1 0.1733] before we start, we need a start support beam.
                (if (< (`self.CurrentSplineIndex`) 1)
                  (`InstancedStaticMeshComponent.AddInstance` (`self.PIllarInstanceStaticMesh`) (`KismetMathLibrary.MakeTransform` (.location _returnvalue_3) (`KismetMathLibrary.MakeRotator` 0.0 0.0 (+ (.yaw (.rotation _returnvalue_3)) 90.0)) (.scale _returnvalue_3)) false)))
              (:`then_1`
                (set `self.CurrentSplineSegmentStartPosition` _returnvalue)
                (bind _output_get_2 (set `self.CurrentSplineSegmentLength` (- (`SplineComponent.GetDistanceAlongSplineAtSplinePoint` _caspline (+ _currentsplineindex 1)) _returnvalue)))
                (bind _output_get_3 (set `self.NrOfMeshSegmentsPerCurrentSplineSegment` (/ _output_get_2 (`self.MeshLength`))))
                ;[1 0 0] do we need a new segment?
                (if (> _output_get_3 0)
                  (bind _output_get_4 (set `self.StretchedMeshSegmentLength` (/ (`self.CurrentSplineSegmentLength`) (`self.NrOfMeshSegmentsPerCurrentSplineSegment`))))
                  ;[1 1 1] in this case, rather scale down than up
                  ; (less stretching)
                  (if (not (< _output_get_4 (* (`self.MeshLength`) 1.5)))
                    (set `self.StretchedMeshSegmentLength` (/ (`self.StretchedMeshSegmentLength`) 2.0))
                    (set `self.NrOfMeshSegmentsPerCurrentSplineSegment` (* (`self.NrOfMeshSegmentsPerCurrentSplineSegment`) 2)))
                  ;[1 1 1] adding segments until done!
                  (for _index_3 (range (`self.NrOfMeshSegmentsPerCurrentSplineSegment`))
                    (`/Engine/EditorBlueprintResources/StandardMacros.IncrementInt` (`self.CurrentStoneWallAddonIndex`)
                      (:`  `
                        (bind _returnvalue_6 (`AddComponent|NODE_AddSplineMeshComponent-0`))
                        (bind _returnvalue_7 (- (`self.CalculateDistanceToMesh` _index_3) 1.0))
                        (bind _returnvalue_8 (+ (`self.CalculateDistanceToMesh` (+ _index_3 1)) 1.0))
                        (bind (_outstartposition _outendposition) (`self.MakeWallsLevelHorizontallySegmented` (`SplineComponent.GetLocationAtDistanceAlongSpline` _caspline_3 _returnvalue_7 "Local") (`SplineComponent.GetLocationAtDistanceAlongSpline` _caspline_2 _returnvalue_8 "Local")))
                        (`SplineMeshComponent.SetStartAndEnd` _returnvalue_6 _outstartposition (`self.MakeTangentsLevelHorizontallySegmented` (`KismetMathLibrary.ClampVectorSize` (`SplineComponent.GetTangentAtDistanceAlongSpline` _caspline_3 _returnvalue_7 "Local") 1.0 (`self.StretchedMeshSegmentLength`))) _outendposition (`self.MakeTangentsLevelHorizontallySegmented` (`KismetMathLibrary.ClampVectorSize` (`SplineComponent.GetTangentAtDistanceAlongSpline` _caspline_2 _returnvalue_8 "Local") 1.0 (`self.StretchedMeshSegmentLength`))) true)
                        (`StaticMeshComponent.SetStaticMesh` _returnvalue_6 (cast `StaticMesh` (`KismetMathLibrary.SelectObject` (`self.WallAddonStaticMesh`) (`self.StaticMeshWallSegment`) (`KismetArrayLibrary.Array_Contains` (`self.StoneWallAddonPosition`) (`self.CurrentStoneWallAddonIndex`))) :!pure true))
                        (`SceneComponent.K2_AttachToComponent` _returnvalue_6 (`self.CASpline`) "None" "KeepRelative" "KeepRelative" "KeepRelative" true))))))
              (:`then_2`
                ;[0 1 0.1733] Side Support Pillars for curved walls
                (if (`|EnumEquality` (`SplineComponent.GetSplinePointType` (`self.CASpline`) (`self.CurrentSplineIndex`)) "Curve")
                  ;[0 1 0.1733] rear
                  (`InstancedStaticMeshComponent.AddInstance` (`self.PIllarInstanceStaticMesh`) (`KismetMathLibrary.MakeTransform` (.location (`SplineComponent.GetTransformAtSplinePoint` (`self.CASpline`) (`self.CurrentSplineIndex`) "Local" false)) (`KismetMathLibrary.MakeRotator` 0.0 0.0 (.yaw (.rotation (`SplineComponent.GetTransformAtSplinePoint` (`self.CASpline`) (`self.CurrentSplineIndex`) "Local" false)))) (.scale (`SplineComponent.GetTransformAtSplinePoint` (`self.CASpline`) (`self.CurrentSplineIndex`) "Local" false))) false)
                  (else
                    ;[0 1 0.1733] linear
                    (if (`|EnumEquality` (`SplineComponent.GetSplinePointType` (`self.CASpline`) (`self.CurrentSplineIndex`)) "Linear")
                      ;[0 1 0.1733] rear
                      (`InstancedStaticMeshComponent.AddInstance` (`self.PIllarInstanceStaticMesh`) (`KismetMathLibrary.MakeTransform` _location (`KismetMathLibrary.MakeRotator` 0.0 0.0 (.yaw (.rotation (`SplineComponent.GetTransformAtSplinePoint` (`self.CASpline`) (`self.CurrentSplineIndex`) "Local" false)))) _scale) false)
                      (`InstancedStaticMeshComponent.AddInstance` (`self.PIllarInstanceStaticMesh`) (`KismetMathLibrary.MakeTransform` _location (`KismetMathLibrary.MakeRotator` 0.0 0.0 (+ (.yaw (.rotation (`SplineComponent.GetTransformAtSplinePoint` (`self.CASpline`) (`self.CurrentSplineIndex`) "Local" false))) 180.0)) _scale) false)
                      (else
                        ;[0 1 0.1733] clamped curve
                        (if (`|EnumEquality` (`SplineComponent.GetSplinePointType` (`self.CASpline`) (`self.CurrentSplineIndex`)) "CurveClamped")
                          (`InstancedStaticMeshComponent.AddInstance` (`self.PIllarInstanceStaticMesh`) (`KismetMathLibrary.MakeTransform` (.location _returnvalue_4) (`KismetMathLibrary.MakeRotator` 0.0 0.0 (+ (.yaw (.rotation _returnvalue_4)) (.yaw (.rotation (`SplineComponent.GetTransformAtSplinePoint` (`self.CASpline`) (+ (`self.CurrentSplineIndex`) 1) "Local" false))) 45.0)) (.scale _returnvalue_4)) false)))))))))
          ;[1 1 1] end pillar
          ;;[1 1 1] last index
          (`/Engine/EditorBlueprintResources/StandardMacros.IncrementInt` (`self.CurrentSplineIndex`)
            (:`  `
              ;[0 1 0.1733] End Pillar
              (`InstancedStaticMeshComponent.AddInstance` (`self.PIllarInstanceStaticMesh`) (`KismetMathLibrary.MakeTransform` (.location _returnvalue_2) (`KismetMathLibrary.MakeRotator` 0.0 0.0 (- (.yaw (.rotation _returnvalue_2)) 90.0)) (.scale _returnvalue_2)) false))))
        (:`then_4`
          ;[0 0.4544 1] deform landscape approach
          (if (`self.bDeformLandscape`)
            (bind _outactors (`GameplayStatics.GetAllActorsOfClass` "/Script/Landscape.Landscape"))
            (`LandscapeProxy.EditorApplySpline` _outactors (`self.CASpline`) _deformwidth _deformwidth _deformoffset _deformoffset 0.0 0.0 20 true true null (`self.LandscapeLayerName`))))))
    (:`else`)))