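; BA04_AnimalMeadow is a child building actor for an animal meadow, tagged as a Barn building type in its construction script.
; It responds to building events: gaining highest priority calls GenerateResources, and the stop button clears the IsGenerating flag.
; The abandon button event is an empty stub, and the generation logic itself is not defined in this graph.
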(event `self.Building STOP Button clicked`
  (set `self.Is Generating` false))

(event `self.Building has Highest Priority`
  (`self.Generate Resources`))

(event `self.Building to be abandoned Button clicked`)

(fn `UserConstructionScript`
  (`parent.UserConstructionScript`)
  (`BlueprintGameplayTagLibrary.AddGameplayTag` (`self.Tag Container_0`) (struct :`TagName` "Building.Typ.Barn")))