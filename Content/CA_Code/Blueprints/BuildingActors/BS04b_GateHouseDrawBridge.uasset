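; BS04b_GateHouseDrawBridge is a gatehouse drawbridge building actor whose current logic is an animation demo loop.
; On BeginPlay it issues open/close, broken-open and broken animations back to back on the Drawbridge, repeating while a counter is below ten and printing that count.
; The loop has no delay, so each non-looping play call immediately overrides the previous one.
; Its priority and abandon events are empty, and construction defers to the parent.
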(event `self.Building has Highest Priority`)

(event `self.ReceiveBeginPlay`
  (bind _drawbridge (`self.Drawbridge`))
  (bind _loopingarraydemo (`self.LoopingArrayDemo`))
  (`SkeletalMeshComponent.PlayAnimation` _drawbridge "/Game/CA_Buildings/Meshes/StoneWalls/Gate/animated/Drawbridge_Open_Close.Drawbridge_Open_Close" false :!label _label)
  (`SkeletalMeshComponent.PlayAnimation` _drawbridge "/Game/CA_Buildings/Meshes/StoneWalls/Gate/animated/DrawBridge_BrokenOpen.DrawBridge_BrokenOpen" false)
  (`SkeletalMeshComponent.PlayAnimation` _drawbridge "/Game/CA_Buildings/Meshes/StoneWalls/Gate/animated/Drawbridge_Broken.Drawbridge_Broken" false)
  (if (< _loopingarraydemo 10)
    (bind _result (`/Engine/EditorBlueprintResources/StandardMacros.IncrementInt` _loopingarraydemo)
      (:`  `
        (bind _output_get (set `self.LoopingArrayDemo` _result))
        (`KismetSystemLibrary.PrintString` (`KismetStringLibrary.Conv_IntToString` _output_get))
        (`KismetSystemLibrary.PrintString` "Loop Number")
        (goto _label)))))

(event `self.Building to be abandoned Button clicked`)

(fn `UserConstructionScript`
  (`parent.UserConstructionScript`))