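; CA_Projectile is an arcing projectile actor that launches at a homing target and applies damage on hit, filtered by team number unless friendly fire is on.
; On BeginPlay it computes a toss velocity from constant or distance-scaled speed, favoring a high arc beyond a threshold.
; A looping timer enables homing once within activation distance of the target.
; It destroys itself after its lifetime or shortly after stopping.
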(event `self.ReceiveBeginPlay`
  (`PrimitiveComponent.IgnoreActorWhenMoving` (`self.Collision`) (`self.IgnoredActors`) true)
  (`self.Setup Target`)
  (`KismetSystemLibrary.K2_SetTimerDelegate` (delegate `Destroy`) (`self.LifeTime`))
  (if (and (> (`self.HomingActivationDistance`) 0.0) (`KismetSystemLibrary.IsValid` (`self.HomingSceneComponent`)))
    (bind _returnvalue (`KismetSystemLibrary.K2_SetTimerDelegate` (delegate `CheckDistanceForHoming`) 0.5 true))
    (set `self.DistanceForHomingTimer` _returnvalue)))

(event `Destroy`
  (`self.K2_DestroyActor`))

(event `CheckDistanceForHoming`
  (bind _homingscenecomponent (`self.HomingSceneComponent`))
  (`/Engine/EditorBlueprintResources/StandardMacros.IsValid` _homingscenecomponent
    (:`Is Valid`
      (if (< (`KismetMathLibrary.Vector_Distance` (`self.K2_GetActorLocation`) (`SceneComponent.K2_GetComponentLocation` _homingscenecomponent)) (`self.HomingActivationDistance`))
        (set `ProjectileMovementComponent.bIsHomingProjectile` true (`self.ProjectileMovement`))
        (`KismetSystemLibrary.K2_ClearAndInvalidateTimerHandle` (`self.DistanceForHomingTimer`) :!label _label)))
    (:`Is Not Valid`
      (goto _label))))

(event `self.ReceiveTick`
  (params (DeltaSeconds :type "Float (single-precision)")))

(event `self.ProjectileMovement.OnProjectileStop`
  (params (ImpactResult :type "HitResult Structure (by ref)"))
  (`PrimitiveComponent.SetCollisionEnabled` (`self.Collision`) "NoCollision")
  (`KismetSystemLibrary.Delay` 5.0)
  (`self.K2_DestroyActor`))

(event `self.Collision.OnComponentHit`
  (params (HitComponent :type "PrimitiveComponent Object Reference") (OtherActor :type "Actor Object Reference") (OtherComp :type "PrimitiveComponent Object Reference") (NormalImpulse :type "Vector Structure") (Hit :type "HitResult Structure (by ref)"))
  (`self.Damage` HitComponent OtherActor OtherComp NormalImpulse Hit))

(fn `CanApplyDamage`
  (params (Actor :type "Object Object Reference"))
  (returns (ReturnValue :type Boolean))
  (if (`self.FriendlyFire `)
    (return true)
    (else
      (bind _teamnumber (message `/Game/CA_Code/Blueprints/Interfaces/BPI_CA_TagsAndInfo.GetTeamNumber` Actor))
      (return (!= _teamnumber (`self.TeamNumber`))))))

(fn `Damage`
  (params (HitComponent :type "PrimitiveComponent Object Reference") (`Other Actor` :type "Object Object Reference") (`Other Comp` :type "PrimitiveComponent Object Reference") (NormalImpulse :type "Vector Structure") (Hit :type "HitResult Structure (by ref)"))
  (bind (_bblockinghit _binitialoverlap _time _distance _location _impactpoint _normal _impactnormal _physmat _hitactor) (`GameplayStatics.BreakHitResult` Hit))
  (bind _returnvalue (`self.GetOwner`))
  (if (`self.CanApplyDamage` _hitactor)
    (`GameplayStatics.ApplyDamage` _hitactor (`self.BaseDamage`) (`AIBlueprintHelperLibrary.GetAIController` _returnvalue) _returnvalue (`self.DamageType`))))

(fn `Get Launch Speed By Distance`
  (params (Distance :type "Float (double-precision)"))
  (returns (Speed :type "Float (double-precision)"))
  (return (`KismetMathLibrary.MapRangeClamped` Distance (`self.MinDistance`) (`self.MaxDistance `) 1000.0 (* (`KismetMathLibrary.Sqrt` (* (`KismetMathLibrary.Abs` (`MovementComponent.GetGravityZ` (`self.ProjectileMovement`))) (`self.MaxDistance `))) (`self.SpeedSafetyMargin `)))))

(fn `Setup Target`
  (bind _homingtarget (`self.HomingTarget`))
  (bind _returnvalue (`self.GetComponentByClass` _homingtarget "/Script/Engine.SceneComponent"))
  (`/Engine/EditorBlueprintResources/StandardMacros.IsValid` _homingtarget
    (:`Is Valid`
      (`/Engine/EditorBlueprintResources/StandardMacros.IsValid` _returnvalue
        (:`Is Valid`
          (bind _output_get (set `self.HomingSceneComponent` _returnvalue))
          (set `ProjectileMovementComponent.HomingTargetComponent` _output_get (`self.ProjectileMovement`))
          (`self.Velocity Setup` (`self.K2_GetActorLocation`) (`SceneComponent.K2_GetComponentLocation` (`self.HomingSceneComponent`))))))))

(fn `UserConstructionScript`)

(fn `Velocity Setup`
  (params (StartLocation :type "Vector Structure") (EndLocation :type "Vector Structure"))
  (locals (Speed :type "Float (double-precision)" :default 0.0))
  (bind _returnvalue (`KismetMathLibrary.Vector_Distance` StartLocation EndLocation))
  (if (`self.UseConstLaunchSpeed`)
    (set `local.Speed` (`self.ConstLaunchSpeed`))
    (else
      (set `local.Speed` (`self.Get Launch Speed By Distance` _returnvalue))))
  (bind _tossvelocity (`GameplayStatics.BlueprintSuggestProjectileVelocity` StartLocation (`self.AddDistortion` EndLocation) (`local.Speed`) 0.0 "DoNotTrace" 0.0 (not (< _returnvalue (`self.HighArcThreshold `))) true))
  (set `MovementComponent.Velocity` _tossvelocity (`self.ProjectileMovement`)))