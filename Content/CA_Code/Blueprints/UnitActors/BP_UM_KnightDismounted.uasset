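; BP_UM_KnightDismounted is a unit actor Blueprint defining the dismounted knight, a melee combat unit.
; Its Construction Script runs the parent's, then overwrites inherited stats for sight, movement, melee combat, defense, ambush and morale.
; AttackRange is assigned twice in that chain, so the final zero value wins.
; The Event Graph holds only disabled stubs, so this Blueprint adds no runtime logic of its own.
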(fn `UserConstructionScript`
  (`parent.UserConstructionScript`)
  (set `self.LineOfSight` 25)
  (set `self.BlockRate` 0.8)
  (set `self.MovementSpeed` 8.0)
  (set `self.Attack Speed` 1.0)
  (set `self.MeleeDamage` 5.0)
  (set `self.AttackRange` 1.0)
  (set `self.AttackRange` 0.0)
  (set `self.AmbushPower` 2)
  (set `self.AccuracyMelee` 0.9)
  (set `self.EvadeRate` 0.1)
  (set `self.MoraleMax` 125.0)
  (set `self.MoraleCurrent` 125.0))