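; Archived dummy enemy villager unit whose construction script adds the villager unit gameplay tag and assigns it to player team 2.
; The event graph holds only disconnected logic: a health widget update and a draft repair loop for overlapping MasterBuilding actors with animation, sound and delay.
; That draft never runs and writes zero to building stability rather than the incremented value.
; The Auto_Build/Repair function is an empty stub.
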(fn `Auto_Build/Repair`)

(fn `UserConstructionScript`
  (`parent.UserConstructionScript`)
  (`BlueprintGameplayTagLibrary.AddGameplayTag` (`self.Tag Container_0`) (struct :`TagName` "Unit.Typ.Villager"))
  (set `self.PlayerTeamNr` 2))