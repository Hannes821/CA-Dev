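; Base animal unit that simulates hunger and stamina to drive AI behavior, assigned to player number 9.
; On BeginPlay, looping timers raise hunger at a randomized interval and drain stamina at a fixed one.
; Each update refreshes its overhead progress bar, then sets hungry or tired flags on the actor and Blackboard near the limits.
; Tick is disabled, and older health-bar logic is left unconnected.
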(event `self.ReceiveBeginPlay`
  (bind _hungerlevelrate (`self.HungerLevelRate`))
  ;[1 1 1] Begin Play
  (`parent.ReceiveBeginPlay`)
  (set `self.OwnerPlayerNr` 9)
  ;;[1 1 1] Set I AmIAlive? to true
  (set `self.AmI Alive?Deprecated` true)
  ;;[1 1 1] Set Hunger level to 0 and increase hunger at the "Hunger Level Rate"
  (set `self.HungerLevel` 0.0)
  (`KismetSystemLibrary.K2_SetTimer` null "UpdateHungerLevel" (`KismetMathLibrary.RandomFloatInRange` (/ _hungerlevelrate 2.0) _hungerlevelrate) true)
  ;;[1 1 1] Set Stamina level to 100 and decrease stamina at the "Stamina Level Rate"
  (set `self.StaminaLevel` 100.0)
  (`KismetSystemLibrary.K2_SetTimer` null "UpdateStaminaLevel" (`self.StaminaLevelRate`) true))

(fn `Update Stamina Level`
  (bind _bbkey_amitired_ (`self.BBKey_AmITired?`))
  (set `self.StaminaLevel` (`KismetMathLibrary.FMax` (`KismetMathLibrary.FMin` (- (`self.StaminaLevel`) 1.0) 100.0)))
  (bind _asattack_animal_stat_widget_blueprint (cast `/Game/CA_Units/Gaia/AttackAnimal_Wolf/Wolf/Blueprints/ParentClassBlueprints/AttackAnimal_Stat_WidgetBlueprint` (`WidgetComponent.GetUserWidgetObject` (`self.OverHeadStatBar`))))
  (`ProgressBar.SetPercent` (`/Game/CA_Units/Gaia/AttackAnimal_Wolf/Wolf/Blueprints/ParentClassBlueprints/AttackAnimal_Stat_WidgetBlueprint.ProgressBar_Stamina` _asattack_animal_stat_widget_blueprint) (/ (`self.StaminaLevel`) 100.0))
  (if (<= (`self.StaminaLevel`) 1.0)
    (set `self.AmITired?` true)
    (`BlackboardComponent.SetValueAsBool` (`AIBlueprintHelperLibrary.GetBlackboard` null) _bbkey_amitired_ true)
    (else
      (set `self.AmITired?` false)
      (`BlackboardComponent.SetValueAsBool` (`AIBlueprintHelperLibrary.GetBlackboard` null) _bbkey_amitired_ false))))

(fn `UpdateHungerLevel`
  (bind _bbkey_amihungry_ (`self.BBKey_AmIHungry?`))
  (set `self.HungerLevel` (`KismetMathLibrary.FMin` (+ (`self.HungerLevel`) 1.0) 100.0))
  (bind _asattack_animal_stat_widget_blueprint (cast `/Game/CA_Units/Gaia/AttackAnimal_Wolf/Wolf/Blueprints/ParentClassBlueprints/AttackAnimal_Stat_WidgetBlueprint` (`WidgetComponent.GetUserWidgetObject` (`self.OverHeadStatBar`))))
  (`ProgressBar.SetPercent` (`/Game/CA_Units/Gaia/AttackAnimal_Wolf/Wolf/Blueprints/ParentClassBlueprints/AttackAnimal_Stat_WidgetBlueprint.ProgressBar_Hunger` _asattack_animal_stat_widget_blueprint) (/ (`self.HungerLevel`) 100.0))
  (if (>= (`self.HungerLevel`) 99.0)
    (set `self.AmIHungry?` true)
    (`BlackboardComponent.SetValueAsBool` (`AIBlueprintHelperLibrary.GetBlackboard` null) _bbkey_amihungry_ true)
    (else
      (set `self.AmIHungry?` false)
      (`BlackboardComponent.SetValueAsBool` (`AIBlueprintHelperLibrary.GetBlackboard` null) _bbkey_amihungry_ false))))

(fn `UserConstructionScript`
  (`parent.UserConstructionScript`))