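; Villager dummy unit Blueprint whose construction script sets player number 3 and applies that player's faction material to the mesh.
; The event graph holds an unconnected auto-repair draft that never runs: it finds overlapping damaged buildings, then loops hammer animation, sound and delayed health increments.
; That draft only increments a local health copy, never writing it back to the building's StabilityComponent.
; The AutoBuildRepair function is an empty stub.
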(fn `Auto_Build/Repair`)

(fn `UserConstructionScript`
  (bind (_value _returnvalue) (`BlueprintMapLibrary.Map_Find` (`self.UnitsFactionMaterial`) (`self.PlayerNumber`)))
  (set `self.PlayerNumber` 3)
  (if _returnvalue
    (`PrimitiveComponent.SetMaterial` (`self.Mesh`) 0 _value)
    (`parent.UserConstructionScript`)))