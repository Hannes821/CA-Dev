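; Civilian villager unit Blueprint, with an unfinished prototype for automatically building or repairing buildings it overlaps.
; Disconnected event-graph logic finds MasterBuilding actors overlapping the capsule, and a separate fragment loops a builder animation, sound and timed health increment until full health.
; None of this runs: the health values are placeholders and the AutoBuildRepair function is empty.
; The construction script only calls its parent.
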(fn `Auto_Build/Repair`)

(fn `UserConstructionScript`
  (`parent.UserConstructionScript`))