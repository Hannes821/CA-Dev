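; CA_MasterActor is a base actor that shows or hides selection feedback when it is selected or unselected.
; OnSelected and OnUnselected events call Selected and Unselected, which pass true or false to ChangeSelectionVisibility.
; That function sets widget visibility on every CA_WidgetComponent found on the actor, then toggles the visibility of the selection ring component.
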(event `/Game/CA_Code/Blueprints/Interfaces/BPI_Selectable.OnSelected`
  (`self.Selected`))

(event `/Game/CA_Code/Blueprints/Interfaces/BPI_Selectable.OnUnselected`
  (`self.Unselected`))

(fn `Change Selection Visibility`
  (params (NewVisibility :type Boolean))
  (`|ExecutionSequence`
    (:`then_0`
      (for _array_element (`self.K2_GetComponentsByClass` "/Game/CA_Code/Blueprints/ActorsComponents/UnitSelection/CA_WidgetComponent.CA_WidgetComponent_C")
        (`/Game/CA_Code/Blueprints/ActorsComponents/UnitSelection/CA_WidgetComponent.Set Widget Visibility` _array_element (`local.NewVisibility`) false)))
    (:`then_1`
      (`SceneComponent.SetVisibility` (`self.CA_SelectionRingComp`) NewVisibility false))))

(fn `Selected`
  (`self.Change Selection Visibility` true))

(fn `Unselected`
  (`self.Change Selection Visibility` false))

(fn `UserConstructionScript`)