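; Arrow projectile actor that sticks into the body it hits and deals damage.
; On mesh overlap it line-traces along its own length against the hit component, playing only a sound on glancing or boneless hits.
; Otherwise it disables physics and collision, attaches to the hit bone, and sinks in by a slightly randomized depth based on the target's armour gameplay tags.
; With a valid instigator it then applies damage and draws debug output.
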(event `self.StaticMeshArrow.OnComponentBeginOverlap`
  (params (OverlappedComponent :type "PrimitiveComponent Object Reference") (OtherActor :type "Actor Object Reference") (OtherComp :type "PrimitiveComponent Object Reference") (OtherBodyIndex :type Integer) (bFromSweep :type Boolean) (SweepResult :type "HitResult Structure (by ref)"))
  (bind _instigator (`self.Instigator`))
  (set `self.TargetActor` OtherActor)
  (bind _output_get (set `self.TargetComponent` OtherComp))
  (`self.LineTraceTarget` _output_get)
  (if (or (< (`KismetMathLibrary.Abs` (`KismetMathLibrary.Dot_VectorVector` (`self.Hit Normal`) (`self.GetActorForwardVector`))) 0.5) (== (`self.TargetBone`) "None"))
    (`GameplayStatics.PlaySound2D` null 1.0 1.0 0.0 null null)
    (else
      ;[1 1 1] attach arrow to body of target
      (`self.SetActorEnableCollision` false)
      (`PrimitiveComponent.SetSimulatePhysics` (`self.StaticMeshArrow`) false)
      (`self.K2_AttachToComponent` (`self.TargetComponent`) (`self.TargetBone`) "KeepWorld" "KeepWorld" "KeepWorld")
      ;[1 1 1] Penetration depth
      (`self.Check Target Penetration Depth` (`self.TargetActor`))
      (`self.ApplyPenetrationDepthToTarget`)
      ;[1 1 1] Damage
      (`/Engine/EditorBlueprintResources/StandardMacros.IsValid` _instigator
        (:`Is Valid`
          (`GameplayStatics.ApplyDamage` (`self.TargetActor`) 10.0 (`Pawn.GetController` _instigator) self)
          ;[1 1 1] Debug
          (`KismetSystemLibrary.PrintString` (`KismetStringLibrary.BuildString_Name` (`KismetSystemLibrary.GetDisplayName` (`self.TargetComponent`)) "" (`self.TargetBone`)))
          (`KismetSystemLibrary.DrawDebugArrow` (`self.HitLocation`) (+ (`self.HitLocation`) (* (`self.Hit Normal`) (`self.DebugPenetrationDepth`))) 0.0 (struct :`G` 1.0 :`B` 1.0 :`A` 1.0))
          (`KismetSystemLibrary.DrawDebugArrow` (`self.K2_GetActorLocation`) (0.0 0.0 0.0) 0.0 (struct :`R` 1.0 :`G` 1.0 :`A` 1.0)))))))

(fn `ApplyPenetrationDepthToTarget`
  (`self.K2_SetActorLocation` (+ (`self.HitLocation`) (* (`self.GetActorForwardVector`) (+ (`KismetMathLibrary.RandomFloatInRange` 0.0 3.0) (`self.PenetrationDepth`))))))

(fn `Check Target Penetration Depth`
  (params (TargetActorRef :type "Object Object Reference"))
  (returns (PenetrationDepth :type "Float (double-precision)"))
  (message `GameplayTagAssetInterface.HasAnyMatchingGameplayTags` TargetActorRef (`self.UnarmouredTargets`))
  (if true
    (set `self.PenetrationDepth` 10.0)
    (return (`self.PenetrationDepth`))
    (else
      (message `GameplayTagAssetInterface.HasAnyMatchingGameplayTags` TargetActorRef (`self.LightArmouredTargets`))
      (if true
        (set `self.PenetrationDepth` 5.0)
        (return (`self.PenetrationDepth`))
        (else
          (message `GameplayTagAssetInterface.HasAnyMatchingGameplayTags` TargetActorRef (`self.HeavyArmouredTargets`))
          (if true
            (set `self.PenetrationDepth` 1.0)
            (return (`self.PenetrationDepth`))))))))

(fn `CheckIfArrowShouldStick`
  (if (or (< (`KismetMathLibrary.Abs` (`KismetMathLibrary.Dot_VectorVector` (`self.Hit Normal`) (`self.GetActorForwardVector`))) 0.5) (== (`self.TargetBone`) "None"))
    (return)
    (else
      (return))))

(fn `LineTraceTarget`
  (params (TargetComponent :type "PrimitiveComponent Object Reference"))
  (returns (HitLocation :type "Vector Structure") (HitNormal :type "Vector Structure") (TargetBone :type Name))
  (bind _staticmesharrow (`self.StaticMeshArrow`))
  (bind _returnvalue (`SceneComponent.K2_GetComponentLocation` _staticmesharrow))
  (bind _returnvalue_2 (`SceneComponent.GetForwardVector` _staticmesharrow))
  (bind (_min _max) (`StaticMeshComponent.GetLocalBounds` _staticmesharrow))
  (bind (_hitlocation _hitnormal _bonename) (`PrimitiveComponent.K2_LineTraceComponent` TargetComponent (+ _returnvalue (* _returnvalue_2 (.x _min))) (+ _returnvalue (* _returnvalue_2 (.x _max))) true true true))
  (bind _output_get (set `self.HitLocation` _hitlocation))
  (bind _output_get_2 (set `self.Hit Normal` _hitnormal))
  (bind _output_get_3 (set `self.TargetBone` _bonename))
  (return _output_get _output_get_2 _output_get_3))

(fn `UserConstructionScript`)