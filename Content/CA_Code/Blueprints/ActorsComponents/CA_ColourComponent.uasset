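; Actor component that defines the colour palette and the two-colour scheme for eight players.
; SetBaseColours fills the six base colours, which SetPlayerColour combines into primary and secondary maps keyed by player number.
; A metallic primary, silver or gold, pairs with one of four secondary colours to give eight unique combinations.
; The event graph is empty, and an older per-player array setup is left disconnected.
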(fn `SetBaseColours`
  (set `self.BaseColourGold` (0.7 0.4 0.0))
  (set `self.BaseColourSilver` (0.7 0.7 0.7))
  (set `self.BaseColourRed` (0.25 0.015 0.015))
  (set `self.BaseColourBlue` (0.0125 0.01 0.25))
  (set `self.BaseColourGreen` (0.01 0.06 0.02))
  (set `self.BaseColourBlack` (0.01 0.01 0.01))
  (`KismetSystemLibrary.PrintString` "Base colours have been set"))

(fn `SetPlayerColour`
  (bind _basecoloursilver (`self.BaseColourSilver`))
  (bind _basecolourgold (`self.BaseColourGold`))
  (set `self.PrimaryColourMap` (`|MakeMap` 1 _basecoloursilver 2 _basecoloursilver 3 _basecoloursilver 4 _basecoloursilver 5 _basecolourgold 6 _basecolourgold 7 _basecolourgold 8 _basecolourgold))
  (set `self.SecondaryColourMap` (`|MakeMap` 1 (`self.BaseColourRed`) 2 (`self.BaseColourBlue`) 3 (`self.BaseColourGreen`) 4 (`self.BaseColourBlack`) 5 (`self.BaseColourRed`) 6 (`self.BaseColourBlue`) 7 (`self.BaseColourGreen`) 8 (`self.BaseColourBlack`))))