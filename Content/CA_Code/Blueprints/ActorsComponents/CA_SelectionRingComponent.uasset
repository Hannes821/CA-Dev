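; CA_SelectionRingComponent is an actor component that tracks its owner's health, despite the selection-ring name.
; It starts at MaxHealth and binds to the owner's OnTakeAnyDamage, subtracting damage through a clamped SetHealth that broadcasts the new value and delta.
; Reaching zero fires a zero-health event, after which damage is ignored and TryToHeal fails, as it also does at full health.
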(event `self.ReceiveBeginPlay`
  (`self.SetHealth` (`self.MaxHealth`))
  (add `Actor.OnTakeAnyDamage` (`self.GetOwner`) (`|CreateDelegate` :!event `OnTakeAnyDamage`)))

(fn `GetHealth`
  (returns (CurrentHealth :type "Float (double-precision)"))
  (return (`self.CurrentHealth`)))

(fn `GetHealthPercent`
  (returns (HealthPercent :type "Float (double-precision)"))
  (return (/ (`self.CurrentHealth`) (`self.MaxHealth`))))

(fn `GetMaxHealth`
  (returns (MaxHealth :type "Float (double-precision)"))
  (return (`self.MaxHealth`)))

(fn `Is FullHealth`
  (returns (IsFull :type Boolean))
  (return (`KismetMathLibrary.NearlyEqual_FloatFloat` (`self.CurrentHealth`) (`self.MaxHealth`) 0.001)))

(fn `IsZeroHealth`
  (returns (IsZeroHealth :type Boolean))
  (return (`KismetMathLibrary.NearlyEqual_FloatFloat` (`self.CurrentHealth`))))

(fn `On Zero Health`
  (params (InstigatedBy :type "Controller Object Reference"))
  (`self.OnZeroHealth`))

(fn `OnTakeAnyDamage`
  (params (DamagedActor :type "Actor Object Reference") (Damage :type "Float (single-precision)") (DamageType :type "DamageType Object Reference") (InstigatedBy :type "Controller Object Reference") (DamageCauser :type "Actor Object Reference"))
  (bind _iszerohealth (`self.IsZeroHealth`))
  (if (not (or _iszerohealth (`KismetMathLibrary.NearlyEqual_FloatFloat` Damage)))
    (`self.SetHealth` (- (`self.CurrentHealth`) Damage))
    (bind _iszerohealth_2 (`self.IsZeroHealth`))
    (if _iszerohealth_2
      (`self.On Zero Health` InstigatedBy))))

(fn `SetHealth`
  (params (NewHealth :type "Float (double-precision)"))
  (locals (DeltaHealth :type "Float (double-precision)"))
  (bind _returnvalue (`KismetMathLibrary.FClamp` NewHealth 0.0 (`self.MaxHealth`)))
  (bind _output_get (set `local.DeltaHealth` (- _returnvalue (`self.CurrentHealth`))))
  (bind _output_get_2 (set `self.CurrentHealth` _returnvalue))
  (`self.OnHealthChanged` _output_get_2 _output_get)
  (return))

(fn `TryToHeal`
  (params (HealValue :type "Float (double-precision)"))
  (returns (Healed :type Boolean))
  (if (> (`KismetMathLibrary.SignOfFloat` HealValue) 0.0)
    (bind _isfull (`self.Is FullHealth`))
    (bind _iszerohealth (`self.IsZeroHealth`))
    (if (or _iszerohealth _isfull)
      (return false)
      (else
        (`self.SetHealth` (+ HealValue (`self.CurrentHealth`)))
        (return true)))
    (else
      (return false))))