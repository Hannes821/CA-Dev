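; Actor component that makes its owner a workplace, tracking assigned worker units up to a maximum count.
; Assignment passes optional team, class and required-component filters, and assigning or unassigning fires events.
; It binds each worker's zero-health and destroyed events, pruning dead or invalid entries on death.
; It also exposes a workplace-specific behavior tree, and Abandon switches all workers back to their default tree.
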(fn `Abandon`
  (locals (AllUnits :type "Array of /Game/CA_Code/Blueprints/UnitActors/BP_MasterUnit Object Reference"))
  (bind _output_get (set `local.AllUnits` (`self.CurrentWorkers`)))
  (for _array_element _output_get
    (`/Game/CA_Code/Blueprints/Interfaces/BPI_UnitOrders.ToDefaultBT` _array_element)))

(fn `AssignWorker `
  (params (Unit :type "/Game/CA_Code/Blueprints/UnitActors/BP_MasterUnit Object Reference"))
  (returns (WasAssigned :type Boolean))
  (`/Engine/EditorBlueprintResources/StandardMacros.IsValid` Unit
    (:`Is Valid`
      (if (and (`self.CanAssignWorker` Unit) (not (`KismetArrayLibrary.Array_Contains` (`self.CurrentWorkers`) Unit)))
        (`self.BindWorkerEvent` (`local.Unit`))
        (`KismetArrayLibrary.Array_Add` (`self.CurrentWorkers`) (`local.Unit`))
        (`self.OnWorkerAssigned ` (`self.GetOwner`) (`local.Unit`))
        (return true)
        (else
          (return false))))
    (:`Is Not Valid`
      (return false))))

(fn `BindWorkerEvent`
  (params (Worker :type "/Game/CA_Code/Blueprints/UnitActors/BP_MasterUnit Object Reference"))
  (add `/Game/CA_Code/Blueprints/ActorsComponents/AttributeComponents/HealthComponent.OnZeroHealth` (`/Game/CA_Units/BP_CharacterBaseWithHealthP.HealthComponent` Worker) (`|CreateDelegate` :!event `On Worker Death`))
  (add `Actor.OnDestroyed` Worker (`|CreateDelegate` :!event `On Worker Death`)))

(fn `CanAssignWorker`
  (params (Unit :type "/Game/CA_Code/Blueprints/UnitActors/BP_MasterUnit Object Reference"))
  (returns (CanAssign :type Boolean))
  (return (and (`self.IsUnitAllowedToWork` Unit) (not (`self.IsFull`)))))

(fn `Check Unit Class`
  (params (Unit :type "Object Object Reference"))
  (returns (CanWork :type Boolean))
  (if (`self.UseUnitClassFilter`)
    (bind _result (`BlueprintSetLibrary.Set_ToArray` (`self.AllowedUnits`)))
    (for _array_element _result
      (if (`KismetMathLibrary.ClassIsChildOf` (`GameplayStatics.GetObjectClass` Unit) _array_element)
        (return true)))
    (return false)
    (else
      (return true))))

(fn `CheckUnitBehavior`
  (params (Unit :type "/Game/CA_Code/Blueprints/UnitActors/BP_MasterUnit Object Reference (by ref)"))
  (returns (CanWork :type Boolean))
  (if (`self.RequireBehaviorComponent`)
    (return (`KismetSystemLibrary.IsValid` (`Actor.GetComponentByClass` Unit (`self.RequiredBehaviorComponent`))))
    (else
      (return true))))

(fn `CheckUnitTeam`
  (params (Unit :type "Actor Object Reference"))
  (returns (CanWork :type Boolean))
  (if (`self.CheckTeam`)
    (bind _result (message `/Game/CA_Code/Blueprints/Interfaces/BPI_CA_TagsAndInfo.CheckSameTeam` (`self.GetOwner`) Unit))
    (return _result)
    (else
      (return true))))

(fn `Get Required Behavior Component`
  (returns (RequireBehaviorComponent :type Boolean) (RequiredBehaviorComponent :type "/Game/CA_Code/Blueprints/ActorsComponents/BehaviorComponents/BehaviorComponent Class Reference"))
  (return (`self.RequireBehaviorComponent`) (`self.RequiredBehaviorComponent`)))

(fn `Get Specific BT`
  (returns (SpecificBehaviorTree :type "BehaviorTree Soft Object Reference"))
  (return (`self.SpecificBehaviorTree`)))

(fn `GetMaxCount`
  (returns (MaxWorkersCount :type Integer))
  (return (`self.MaxWorkersCount`)))

(fn `GetWorkerCount`
  (returns (Count :type Integer))
  (return (`KismetArrayLibrary.Array_Length` (`self.CurrentWorkers`))))

(fn `GetWorkers`
  (returns (Workers :type "Array of /Game/CA_Code/Blueprints/UnitActors/BP_MasterUnit Object Reference"))
  (return (`self.CurrentWorkers`)))

(fn `IsFull`
  (returns (IsFull :type Boolean))
  (return (>= (`KismetArrayLibrary.Array_Length` (`self.CurrentWorkers`)) (`self.MaxWorkersCount`))))

(fn `IsUnitAllowedToWork`
  (params (Unit :type "/Game/CA_Code/Blueprints/UnitActors/BP_MasterUnit Object Reference"))
  (returns (CanWork :type Boolean))
  (if (`self.CheckUnitTeam` Unit)
    (if (`self.Check Unit Class` (`local.Unit`))
      (return (`self.CheckUnitBehavior` (`local.Unit`)))
      (else
        (return false)))
    (else
      (return false))))

(fn `IsWorkerAssigned`
  (params (Unit :type "/Game/CA_Code/Blueprints/UnitActors/BP_MasterUnit Object Reference"))
  (returns (IsAssigned :type Boolean))
  (return (`KismetArrayLibrary.Array_Contains` (`self.CurrentWorkers`) Unit)))

(fn `On Worker Death`
  (params (Actor :type "Actor Object Reference"))
  (locals (CopyWorkers :type "Array of /Game/CA_Code/Blueprints/UnitActors/BP_MasterUnit Object Reference"))
  (bind _currentworkers (`self.CurrentWorkers`))
  (bind (_arrayindex _arrayelement) (`/Engine/EditorBlueprintResources/StandardMacros.ReverseForEachLoop` _currentworkers)
    (:`LoopBody`
      (if (or (not (`KismetSystemLibrary.IsValid` _arrayelement)) (== _arrayelement Actor))
        (`KismetArrayLibrary.Array_Remove` _currentworkers _arrayindex)))
    (:`Completed`
      (`self.OnWorkerUnassigned` (`self.GetOwner`)))))

(fn `Unassigne Worker`
  (params (Unit :type "/Game/CA_Code/Blueprints/UnitActors/BP_MasterUnit Object Reference"))
  (returns (WasUnassigned :type Boolean))
  (bind _returnvalue (`KismetArrayLibrary.Array_RemoveItem` (`self.CurrentWorkers`) Unit))
  (if _returnvalue
    (`self.UnbindWorkerEvent` (`local.Unit`))
    (`self.OnWorkerUnassigned` (`self.GetOwner`) (`local.Unit`))
    (return true)
    (else
      (return false))))

(fn `UnbindWorkerEvent`
  (params (Worker :type "/Game/CA_Code/Blueprints/UnitActors/BP_MasterUnit Object Reference"))
  (remove `/Game/CA_Code/Blueprints/ActorsComponents/AttributeComponents/HealthComponent.OnZeroHealth` (`/Game/CA_Units/BP_CharacterBaseWithHealthP.HealthComponent` Worker) (`|CreateDelegate` :!event `On Worker Death`))
  (remove `Actor.OnDestroyed` Worker (`|CreateDelegate` :!event `On Worker Death`)))