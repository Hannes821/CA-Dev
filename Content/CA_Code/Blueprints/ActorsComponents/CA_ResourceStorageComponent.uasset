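; Actor component that stores an owner's resources as type-to-count pairs, with functions to add, query and withdraw them.
; Adds can be filtered by an allowed-type list and capped by per-type limits or a global fallback, with overflow computed by modulo and returned.
; Batch withdrawal checks every amount before reducing any, while single withdrawal checks only that the type exists.
; Count changes fire a value-change notification carrying the owner.
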(fn `Add Resource`
  (params (Resource :type "/Game/CA_Code/Blueprints/Others/E_CA_Resources Enum" :default "NewEnumerator0") (Count :type Integer))
  (returns (Success :type Boolean) (OverflowType :type "/Game/CA_Code/Blueprints/Others/E_CA_Resources Enum") (OverflowCount :type Integer))
  (if (<= Count 0)
    (return false Resource 0)
    (else
      (if (`self.AllowedResourcesOnly`)
        (if (`BlueprintSetLibrary.Set_Contains` (`self.AllowedResources`) Resource)
          _
          (else
            (return false Resource Count))))
      (if (`self.HasLimits`)
        (bind _value (`self.GetLimit` Resource))
        (bind _count (`self.GetResourceCount` Resource))
        (bind (_correctaddvalue _overflow) (`self.CalculateOverflow` Count _count _value))
        (bind _success (`self.AddResourceToMap` Resource _correctaddvalue))
        (return _success Resource _overflow)
        (else
          (bind _success_2 (`self.AddResourceToMap` Resource Count))
          (return _success_2 Resource 0))))))

(fn `Add Resources`
  (params (Resources :type "Map of /Game/CA_Code/Blueprints/Others/E_CA_Resources Enum to Integer"))
  (returns (Overflow :type "Map of /Game/CA_Code/Blueprints/Others/E_CA_Resources Enum to Integer"))
  (locals (CurrentOverflow :type "Map of /Game/CA_Code/Blueprints/Others/E_CA_Resources Enum to Integer"))
  (bind _keys (`BlueprintMapLibrary.Map_Keys` Resources))
  (for _array_element _keys
    (bind (_success _overflowtype _overflowcount) (`self.Add Resource` _array_element (`BlueprintMapLibrary.Map_Find` Resources _array_element)))
    (if (> _overflowcount 0)
      (`BlueprintMapLibrary.Map_Add` (`local.CurrentOverflow`) _overflowtype _overflowcount)))
  (return (`local.CurrentOverflow`)))

(fn `AddResourceToMap`
  (params (Type :type "/Game/CA_Code/Blueprints/Others/E_CA_Resources Enum" :default "NewEnumerator0") (Count :type Integer))
  (returns (Success :type Boolean))
  (bind (_value _returnvalue) (`BlueprintMapLibrary.Map_Find` (`self.CurrentResources`) Type))
  (if (<= Count 0)
    (return false)
    (else
      (`|ExecutionSequence`
        (:`then_0`
          (if _returnvalue
            (`BlueprintMapLibrary.Map_Add` (`self.CurrentResources`) Type (+ _value Count))
            (else
              (`BlueprintMapLibrary.Map_Add` (`self.CurrentResources`) Type Count))))
        (:`then_1`
          (`self.OnResourceValueChange` Type (`BlueprintMapLibrary.Map_Find` (`self.CurrentResources`) Type) (`self.GetOwner`))
          (return true))))))

(fn `CalculateOverflow`
  (params (AddendValue :type Integer) (CurrentValue :type Integer) (Limit :type Integer))
  (returns (CorrectAddValue :type Integer) (Overflow :type Integer))
  (bind _returnvalue (mod (+ AddendValue CurrentValue) Limit))
  (return (- AddendValue _returnvalue) _returnvalue))

(fn `CanStoreResourceType`
  (params (ResourceType :type "/Game/CA_Code/Blueprints/Others/E_CA_Resources Enum" :default "NewEnumerator0"))
  (returns (CanBeStored :type Boolean))
  (if (`self.AllowedResourcesOnly`)
    (return (`BlueprintSetLibrary.Set_Contains` (`self.AllowedResources`) ResourceType))
    (else
      (return true))))

(fn `GetAllowedResources`
  (returns (AllowedResources :type "Set of /Game/CA_Code/Blueprints/Others/E_CA_Resources Enum"))
  (return (`self.AllowedResources`)))

(fn `GetLimit`
  (params (ResourceType :type "/Game/CA_Code/Blueprints/Others/E_CA_Resources Enum" :default "NewEnumerator0"))
  (returns (Value :type Integer))
  (bind (_value _returnvalue) (`BlueprintMapLibrary.Map_Find` (`self.LimitsSpecificResources`) ResourceType))
  (if (`self.HasLimits`)
    (if _returnvalue
      (return _value)
      (else
        (return (`self.GlobalLimit`))))
    (else
      (return -1))))

(fn `GetLimitsInfo`
  (returns (HasLimits :type Boolean) (GlobalLimit :type Integer) (LimitsSpecificResources :type "Map of /Game/CA_Code/Blueprints/Others/E_CA_Resources Enum to Integer"))
  (bind _haslimits (`self.HasLimits`))
  (if _haslimits
    (return _haslimits (`self.GlobalLimit`) (`self.LimitsSpecificResources`))
    (else
      (return false 0))))

(fn `GetResourceCount`
  (params (ResourceType :type "/Game/CA_Code/Blueprints/Others/E_CA_Resources Enum" :default "NewEnumerator0"))
  (returns (Count :type Integer))
  (bind (_value _returnvalue) (`BlueprintMapLibrary.Map_Find` (`self.CurrentResources`) ResourceType))
  (if _returnvalue
    (return _value)
    (else
      (return 0))))

(fn `GetStoredResources`
  (returns (CurrentResources :type "Map of /Game/CA_Code/Blueprints/Others/E_CA_Resources Enum to Integer"))
  (return (`self.CurrentResources`)))

(fn `HasEnoughResource `
  (params (Type :type "/Game/CA_Code/Blueprints/Others/E_CA_Resources Enum" :default "NewEnumerator0") (RequiredCount :type Integer))
  (returns (Has :type Boolean))
  (bind (_value _returnvalue) (`BlueprintMapLibrary.Map_Find` (`self.CurrentResources`) Type))
  (if (> RequiredCount 0)
    (if _returnvalue
      (return (<= RequiredCount _value))
      (else
        _)))
  (return false))

(fn `Is Allowed Resources Only`
  (returns (AllowedResourcesOnly :type Boolean))
  (return (`self.AllowedResourcesOnly`)))

(fn `ReduceResource`
  (params (Resource :type "/Game/CA_Code/Blueprints/Others/E_CA_Resources Enum" :default "NewEnumerator0") (Count :type Integer))
  (returns (Success :type Boolean))
  (bind (_value _returnvalue) (`BlueprintMapLibrary.Map_Find` (`self.CurrentResources`) Resource))
  (bind _returnvalue_2 (- _value Count))
  (if (<= Count 0)
    (return false)
    (elif _returnvalue
      (if (== _returnvalue_2 0)
        (`BlueprintMapLibrary.Map_Remove` (`self.CurrentResources`) Resource)
        (else
          (`BlueprintMapLibrary.Map_Add` (`self.CurrentResources`) Resource _returnvalue_2)))
      (`self.OnResourceValueChange` Resource _returnvalue_2 (`self.GetOwner`))
      (return true)
      (else
        (return false)))))

(fn `TryGetResource`
  (params (ResourceType :type "/Game/CA_Code/Blueprints/Others/E_CA_Resources Enum" :default "NewEnumerator0") (Count :type Integer))
  (returns (GetType :type "/Game/CA_Code/Blueprints/Others/E_CA_Resources Enum") (GetCount :type Integer) (Success :type Boolean))
  (bind _success (`self.ReduceResource` ResourceType Count))
  (if _success
    (return ResourceType Count true)
    (else
      (return ResourceType 0 false))))

(fn `TryGetResources`
  (params (ReduceResources :type "Map of /Game/CA_Code/Blueprints/Others/E_CA_Resources Enum to Integer"))
  (returns (Resources :type "Map of /Game/CA_Code/Blueprints/Others/E_CA_Resources Enum to Integer") (Success :type Boolean))
  (locals (ResourcesToGet :type "Map of /Game/CA_Code/Blueprints/Others/E_CA_Resources Enum to Integer"))
  (bind _output_get (set `local.ResourcesToGet` ReduceResources))
  (bind _keys (`BlueprintMapLibrary.Map_Keys` _output_get))
  (for _array_element _keys
    (bind _has (`self.HasEnoughResource ` _array_element (`BlueprintMapLibrary.Map_Find` (`local.ResourcesToGet`) _array_element)))
    (if (not _has)
      (return _ false)))
  (for _array_element_2 _keys
    (`self.ReduceResource` _array_element_2 (`BlueprintMapLibrary.Map_Find` (`local.ResourcesToGet`) _array_element_2)))
  (return (`local.ResourcesToGet`) true))