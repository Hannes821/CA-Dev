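; BP_WoodResource is a tree resource actor that supplies Wood, with a randomly chosen tree mesh.
; After the parent construction script, it picks a random row from CA_TreesDataTable, applies that mesh, sets its resource type and name, and unhides itself.
; The index increment and missing-row reset have no lasting effect, since each construction re-randomises the index.
; A disconnected random resource-level modifier is marked for removal and never runs.
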(fn `UserConstructionScript`
  (`parent.UserConstructionScript`)
  ;[0.1291 1 0] functional switch of base meshes
  ;;[0 0.1055 1] get in my data table
  (bind _output_get (set `self.TreeTableRef` "/Game/CA_Code/Blueprints/ResourceActors/CA_TreesDataTable.CA_TreesDataTable"))
  (bind _output_get_2 (set `self.CurrentTreeIndex` (`KismetMathLibrary.RandomInteger` 49)))
  ;;[1 0.1226 0] get the mesh
  (bind _returnvalue (`|GetDataTableRow` _output_get (`KismetStringLibrary.Conv_StringToName` (`KismetStringLibrary.Conv_IntToString` _output_get_2)))
    (:`then`
      ;;[0.02531 1 0] set my resource mesh to that table mesh
      (`StaticMeshComponent.SetStaticMesh` (`self.ResourceMesh`) (`.Mesh_8_0CEF6DF647C1051D40385B949E83F52B` (break `/Game/CA_Code/Blueprints/ResourceActors/CA_TreesDataTableStruct` _returnvalue)))
      ;;[1 0.9538 0] incrementally increase the local variable
      (bind _result (`/Engine/EditorBlueprintResources/StandardMacros.IncrementInt` (`self.CurrentTreeIndex`))
        (:`  `
          (set `self.CurrentTreeIndex` _result)
          ;[1 1 1] show them who i am.
          (set `self.ResourceType` self)
          (set `self.ResourceName` "Wood")
          (`self.SetActorHiddenInGame` false))))
    (:`RowNotFound`
      ;;[1 0.8811 0] here we go back to 0 for our counter
      (set `self.CurrentTreeIndex` 0))))