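; Base actor for a neutral resource deposit, holding one resource type in a CAResourceStorageComponent.
; The construction script fills storage, optionally randomizes mesh scale and yaw, and sizes the selection ring to match.
; Storage events relay value changes and handle depletion, while interface functions supply type, tag and widget info.
; DeductResources is a stub and map-fog visibility logic is disconnected; widget info reads CurrentResources, set only at construction.
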(event `self.ReceiveTick`
  (params (DeltaSeconds :type "Float (single-precision)")))

(event `Destroy Deposit`
  (`KismetSystemLibrary.PrintString` "No more resources")
  (`SceneComponent.SetVisibility` (`self.DefaultSceneRoot`) false false)
  (`self.K2_DestroyActor`))

(event `self.ReceiveBeginPlay`
  (add `/Game/CA_Code/Blueprints/ActorsComponents/ResourceStorage/CA_ResourceStorageComponent.OnResourceValueChange` (`self.CA_ResourceStorageComponent`) (`|CreateDelegate` :!event `OnChangeResource`)))

(event `OnChangeResource`
  (params (ResoourceType :type "/Game/CA_Code/Blueprints/Others/E_CA_Resources Enum" :default "NewEnumerator55") (NewCount :type Integer) (Owner :type "Actor Object Reference"))
  (`self.OnChangeResourcesValue` self NewCount (`self.FullResources`)))

(fn `CheckSameTeam`
  (params (Actor :type "Actor Object Reference"))
  (returns (Result :type Boolean))
  (return false))

(fn `Deduct Resources`
  (params (`Deduct Amount` :type Integer))
  (returns (`Resources Remaining` :type Boolean))
  ;[1 1 1] Deduct the resources from this resource
  (if (> (`self.Current Resources`) `Deduct Amount`)
    _))

(fn `GetOwnerController`
  (returns (OwnerController :type "Controller Object Reference"))
  (return null))

(fn `GetOwnerInfoForWidget`
  (returns (Info :type "/Game/CA_Code/Blueprints/Widgets/MasterWidget/Panels/InfoWidget/ST_BaseActorInfo Structure"))
  (return (make `/Game/CA_Code/Blueprints/Widgets/MasterWidget/Panels/InfoWidget/ST_BaseActorInfo` (`self.IndividualTag`) 0 "" "" 0.0 0.0 0.0 0.0 0 0.0 0.0 false 0 "" (`KismetMathLibrary.Conv_IntToDouble` (/ (`self.Current Resources`) (`self.FullResources`))) "" (`KismetTextLibrary.Conv_StringToText` (`KismetStringLibrary.Concat_StrStr` (`KismetStringLibrary.Conv_IntToString` (`self.Current Resources`)) "/" (`KismetStringLibrary.Conv_IntToString` (`self.FullResources`)))))))

(fn `GetOwnerMainTag`
  (returns (IndividualTag :type "GameplayTag Structure"))
  (return (`self.IndividualTag`)))

(fn `GetResourceType`
  (returns (Type :type "/Game/CA_Code/Blueprints/Others/E_CA_Resources Enum"))
  (return (`|GetArrayItem` (`self.ResourceTypeE`))))

(fn `GetTeamNumber`
  (returns (TeamNumber :type Integer))
  (return 0))

(fn `GetTriggerBounds`
  (returns (Origin :type "Vector Structure") (BoxExtent :type "Vector Structure") (SphereRadius :type "Float (double-precision)"))
  (return (0.0 0.0 0.0) (0.0 0.0 0.0) 0.0))

(fn `Init Storage Component`
  (`/Game/CA_Code/Blueprints/ActorsComponents/ResourceStorage/CA_ResourceStorageComponent.Add Resource` (`self.CA_ResourceStorageComponent`) (`|GetArrayItem` (`self.ResourceTypeE`)) (`self.FullResources`))
  (add `/Game/CA_Code/Blueprints/ActorsComponents/ResourceStorage/CA_ResourceStorageComponent.OnEmptyStorage` (`self.CA_ResourceStorageComponent`) (`|CreateDelegate` :!event `Destroy Deposit`)))

(fn `IsEmpty`
  (returns (IsEmpty :type Boolean))
  (bind _isempty (`/Game/CA_Code/Blueprints/ActorsComponents/ResourceStorage/CA_ResourceStorageComponent.IsEmpty` (`self.CA_ResourceStorageComponent`)))
  (return _isempty))

(fn `UserConstructionScript`
  (bind _returnvalue (`KismetMathLibrary.RandomFloatInRange` (`self.Min Mesh Size`) (`self.Max Mesh Size`)))
  (`self.Init Storage Component`)
  ;[0 1 0.3639] Set Resources
  (set `self.Current Resources` (`self.FullResources`))
  ;[1 0 0] If True Use Random Size
  (if (`self.Use Random Size`)
    ;[0.09194 1 0] Set 3D World Size
    (`SceneComponent.SetWorldScale3D` (`self.ResourceMesh`) (`KismetMathLibrary.MakeVector` _returnvalue _returnvalue _returnvalue)))
  ;[1 0 0] If True Use Random Rotation
  (if (`self.Use Random Rotation`)
    ;[0.3109 0.2587 1] Set Random Rotation
    (`SceneComponent.K2_SetWorldRotation` (`self.ResourceMesh`) (`KismetMathLibrary.MakeRotator` 0.0 0.0 (`KismetMathLibrary.RandomFloatInRange` 0.0 360.0)) false false))
  ;[1 0.8988 0.0868] Set the selection ring size
  (`SceneComponent.SetWorldScale3D` (`self.CA_SelectionRingComp`) (`SceneComponent.K2_GetComponentScale` (`self.ResourceMesh`)))
  (`self.SetActorHiddenInGame` false))