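; Base NPC pig character with physics-driven floppy ears and tail, health, draining stamina and an optional overhead stat widget.
; Tick turns the widget toward the player and optionally tilts the mesh to the ground normal from a downward trace.
; A looping timer drains stamina, while damage reduces health; both feed hurt, tired and alive states to the Blackboard.
; At zero health it stops AI movement, ragdolls from the spine and destroys itself after a delay.
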(event `self.ReceiveBeginPlay`
  (bind _physicalanimationdata (make `PhysicalAnimationData` true 200.0 100.0 200.0 100.0))
  (bind _mesh (`self.Mesh`))
  (bind _earphysics_blend_weight (`self.EarPhysics_Blend_Weight`))
  (bind _physicalanimation (`self.PhysicalAnimation`))
  (bind _returnvalue (`SkinnedMeshComponent.GetBoneName` _mesh (`SkinnedMeshComponent.GetBoneIndex` (`self.Mesh`) "Ear_R_1")))
  (bind _returnvalue_2 (`SkinnedMeshComponent.GetBoneName` _mesh (`SkinnedMeshComponent.GetBoneIndex` _mesh "Ear_L_1")))
  (bind _returnvalue_3 (`SkinnedMeshComponent.GetBoneName` _mesh (`SkinnedMeshComponent.GetBoneIndex` _mesh "Tail_1")))
  ;[1 1 1] Begin Play
  ;[1 1 1] Begin Play
  ;;[1 1 1] Set I AmIAlive? to true
  (set `self.AmI Alive?` true)
  ;;[1 1 1] Floppy Ears and Tail
  (`PhysicalAnimationComponent.SetSkeletalMeshComponent` _physicalanimation (`self.Mesh`))
  (`|ExecutionSequence`
    (:`then_0`
      (`PhysicalAnimationComponent.ApplyPhysicalAnimationSettingsBelow` _physicalanimation _returnvalue_2 _physicalanimationdata true)
      (`SkeletalMeshComponent.SetAllBodiesBelowSimulatePhysics` (`self.Mesh`) _returnvalue_2 true true)
      (`SkeletalMeshComponent.SetAllBodiesBelowPhysicsBlendWeight` (`self.Mesh`) _returnvalue_2 _earphysics_blend_weight false true))
    (:`then_1`
      (`PhysicalAnimationComponent.ApplyPhysicalAnimationSettingsBelow` _physicalanimation _returnvalue _physicalanimationdata true)
      (`SkeletalMeshComponent.SetAllBodiesBelowSimulatePhysics` (`self.Mesh`) _returnvalue true true)
      (`SkeletalMeshComponent.SetAllBodiesBelowPhysicsBlendWeight` (`self.Mesh`) _returnvalue _earphysics_blend_weight false true))
    (:`then_2`
      (`PhysicalAnimationComponent.ApplyPhysicalAnimationSettingsBelow` _physicalanimation _returnvalue_3 _physicalanimationdata true)
      (`SkeletalMeshComponent.SetAllBodiesBelowSimulatePhysics` (`self.Mesh`) _returnvalue_3 true true)
      (`SkeletalMeshComponent.SetAllBodiesBelowPhysicsBlendWeight` (`self.Mesh`) _returnvalue_3 (`self.TailPhysics_Blend_Weight`) false true)
      ;;[1 1 1] Set Stamina to 100%
      (set `self.StaminaLevel` 100.0)
      (`KismetSystemLibrary.K2_SetTimer` null "UpdateStaminaLevel" (`KismetMathLibrary.RandomFloatInRange` (/ 0.0 2.0) (`self.StaminaLevelRate`)) true)
      ;;[1 1 1] Draw overhead Health
      (if (`self.DrawOverheadStats?`)
        (bind _returnvalue_4 (`|CreateWidget` "/Game/Pigs/Blueprints/ParentClassBlueprints/Pig_Stat_WidgetBlueprint.Pig_Stat_WidgetBlueprint_C"))
        (set `self.Overhead Stat Bar` _returnvalue_4)
        ;;[1 1 1] Set  Health and Stamina bars
        (bind _aspig_stat_widget_blueprint (cast `/Game/Pigs/Blueprints/ParentClassBlueprints/Pig_Stat_WidgetBlueprint` (`WidgetComponent.GetUserWidgetObject` (`self.OverHeadStatBar`))))
        (`ProgressBar.SetPercent` (`/Game/Pigs/Blueprints/ParentClassBlueprints/Pig_Stat_WidgetBlueprint.ProgressBar_Health` _aspig_stat_widget_blueprint) (/ (`self.Health`) 100.0))
        (`ProgressBar.SetPercent` (`/Game/Pigs/Blueprints/ParentClassBlueprints/Pig_Stat_WidgetBlueprint.ProgressBar_Stamina` _aspig_stat_widget_blueprint) (/ (`self.StaminaLevel`) 100.0))
        (else
          (`SceneComponent.SetVisibility` (`self.OverHeadStatBar`) false false))))))

(event `self.ReceiveTick`
  (params (DeltaSeconds :type "Float (single-precision)"))
  (bind _returnvalue (`GameplayStatics.GetPlayerCharacter` 0))
  (bind _mesh (`self.Mesh`))
  (bind _overheadstatbar (`self.OverHeadStatBar`))
  (bind _overheadstatbar_2 (`self.OverHeadStatBar`))
  (bind _returnvalue_2 (`SceneComponent.K2_GetComponentRotation` _mesh))
  (bind _returnvalue_3 (`SceneComponent.K2_GetComponentLocation` (`self.Capsule`)))
  ;[1 1 1] Tick
  (`|ExecutionSequence`
    (:`then_0`
      ;[1 1 1] Rotate the overhead health bar toward player character 0
      (if (`self.DrawOverheadStats?`)
        (if (`self.RotateHealthBarToPlayer?`)
          (if (`KismetSystemLibrary.IsValid` _returnvalue)
            (`SceneComponent.K2_SetWorldRotation` _overheadstatbar (`KismetMathLibrary.MakeRotator` 0.0 0.0 (.yaw (`KismetMathLibrary.FindLookAtRotation` (`SceneComponent.K2_GetComponentLocation` _overheadstatbar) (`self.K2_GetActorLocation` _returnvalue)))) false false)
            (else
              (`SceneComponent.K2_SetWorldRotation` _overheadstatbar_2 (`KismetMathLibrary.MakeRotator` 0.0 0.0 (.yaw (`KismetMathLibrary.FindLookAtRotation` (`SceneComponent.K2_GetComponentLocation` _overheadstatbar_2) (`SceneComponent.K2_GetComponentLocation` (`self.FollowCamera`))))) false false))))))
    (:`then_3`
      ;[1 1 1] Orient to the ground
      (if (`self.Align to the ground?`)
        (bind (_outhit _returnvalue_4) (`KismetSystemLibrary.LineTraceSingle` _returnvalue_3 (+ _returnvalue_3 (0.0 0.0 -350.0)) "TraceTypeQuery1"))
        (if _returnvalue_4
          (bind (_bblockinghit _binitialoverlap _time _distance _location _impactpoint _normal) (`GameplayStatics.BreakHitResult` _outhit))
          (`SceneComponent.K2_SetWorldRotation` (`self.Mesh`) (`KismetMathLibrary.RInterpTo` _returnvalue_2 (`KismetMathLibrary.MakeRotator` (* (.roll (`KismetMathLibrary.MakeRotFromXZ` (`SceneComponent.GetForwardVector` _mesh) _normal)) (`self.OrientationRoll%`)) (* (.pitch (`KismetMathLibrary.MakeRotFromYZ` (`SceneComponent.GetRightVector` _mesh) _normal)) (`self.OrientationPitch%`)) (.yaw _returnvalue_2)) (`GameplayStatics.GetWorldDeltaSeconds`) 1.0) false false))))))

(event `self.ReceiveAnyDamage`
  (params (Damage :type "Float (single-precision)") (DamageType :type "DamageType Object Reference") (InstigatedBy :type "Controller Object Reference") (DamageCauser :type "Actor Object Reference"))
  (bind _mesh (`self.Mesh`))
  ;[1 1 1] Damage
  ;;[1 1 1] Event- Damage
  (`|ExecutionSequence`
    (:`then_0`
      ;;[1 1 1] Set "AmIHurt?" in the Blackboard to true
      (`BlackboardComponent.SetValueAsBool` (`AIBlueprintHelperLibrary.GetBlackboard` null) (`self.BBKey_AmIHurt?`) true))
    (:`then_1`
      ;;[1 1 1] Reduce Health
      (set `self.Health` (`KismetMathLibrary.FMax` (- (`self.Health`) Damage)))
      (`|ExecutionSequence`
        (:`then_0`
          ;;[1 1 1] Update HealthBar
          (if (`self.DrawOverheadStats?`)
            (bind _aspig_stat_widget_blueprint (cast `/Game/Pigs/Blueprints/ParentClassBlueprints/Pig_Stat_WidgetBlueprint` (`WidgetComponent.GetUserWidgetObject` (`self.OverHeadStatBar`))))
            (`ProgressBar.SetPercent` (`/Game/Pigs/Blueprints/ParentClassBlueprints/Pig_Stat_WidgetBlueprint.ProgressBar_Health` _aspig_stat_widget_blueprint) (/ (`self.Health`) 100.0))))
        (:`then_1`
          ;;[1 1 1] When health is below 0- Ragdoll
          (if (<= (`self.Health`) 0.0)
            (`SceneComponent.SetVisibility` (`self.OverHeadStatBar`) false false)
            (`Controller.StopMovement` (`AIBlueprintHelperLibrary.GetAIController` self))
            (`BlackboardComponent.SetValueAsBool` (`AIBlueprintHelperLibrary.GetBlackboard` self) (`self.BBKey_AmIAlive?`) false)
            (set `self.AmI Alive?` false)
            (`SkeletalMeshComponent.SetAllBodiesBelowSimulatePhysics` (`self.Mesh`) (`SkinnedMeshComponent.GetBoneName` _mesh (`SkinnedMeshComponent.GetBoneIndex` _mesh "Spine_1")) true true)
            (`PrimitiveComponent.SetCollisionEnabled` (`self.CapsuleComponent`) "NoCollision")
            (`PrimitiveComponent.SetCollisionEnabled` (`self.Capsule`) "NoCollision")
            (`KismetSystemLibrary.Delay` (`self.StayDeadBeforDestroyTime`))
            ;;;[1 1 1] Destroy Actor
            (`self.K2_DestroyActor`)
            (`KismetSystemLibrary.CollectGarbage`)))
        (:`then_2`
          ;;[1 1 1] We just got hurt- this is no time to stand around
          (set `self.PlayIdle?` false))))))

(fn `UpdateStaminaLevel`
  (bind _bbkey_amitired_ (`self.BBKey_AmITired?`))
  (set `self.StaminaLevel` (`KismetMathLibrary.FMax` (`KismetMathLibrary.FMin` (- (`self.StaminaLevel`) 1.0) 100.0)))
  (bind _aspig_stat_widget_blueprint (cast `/Game/Pigs/Blueprints/ParentClassBlueprints/Pig_Stat_WidgetBlueprint` (`WidgetComponent.GetUserWidgetObject` (`self.OverHeadStatBar`))))
  (`ProgressBar.SetPercent` (`/Game/Pigs/Blueprints/ParentClassBlueprints/Pig_Stat_WidgetBlueprint.ProgressBar_Stamina` _aspig_stat_widget_blueprint) (/ (`self.StaminaLevel`) 100.0))
  (if (<= (`self.StaminaLevel`) 1.0)
    (set `self.AmITired?` true)
    (`BlackboardComponent.SetValueAsBool` (`AIBlueprintHelperLibrary.GetBlackboard` null) _bbkey_amitired_ true)
    (else
      (set `self.AmITired?` false)
      (`BlackboardComponent.SetValueAsBool` (`AIBlueprintHelperLibrary.GetBlackboard` null) _bbkey_amitired_ false))))

(fn `UserConstructionScript`)