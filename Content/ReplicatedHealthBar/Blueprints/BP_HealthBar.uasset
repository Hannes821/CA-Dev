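; BP_HealthBar is a widget component that tracks its owner's health, max health and shield and displays them on a replicated health bar.
; It binds to the owner's damage event, draining shield before health, and offers heal, shield and max-health events.
; RepNotifies update the widget, rescaling fill and step ratio to health plus shield when that exceeds max health.
; BeginPlay also adds a test widget, and SpaceBar adds shield.
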(event `self.ReceiveBeginPlay`
  (add `Actor.OnTakeAnyDamage` (`self.GetOwner`) (delegate `OnTakeAnyDamage_Event`))
  (`self.CreateWidgetOnClient`)
  (`self.SetMaxHealthRatio`))

(event `Key|SpaceBar`
  (params (Key :type "Key Structure"))
  (:`Pressed`
    (`self.AddShield` 50.0)))

(event `AddShield`
  (params (Value :type "Float (double-precision)"))
  ;[0.277 0.5637 1] Add Shield
  (set `self.Shield` (+ (`self.Shield`) Value)))

(event `OnTakeAnyDamage_Event`
  (params (DamagedActor :type "Actor Object Reference") (Damage :type "Float (single-precision)") (DamageType :type "DamageType Object Reference") (InstigatedBy :type "Controller Object Reference") (DamageCauser :type "Actor Object Reference"))
  (bind _shield (`self.Shield`))
  ;[0.277 0.5637 1] OnTakeAnyDamage
  ;[0.277 0.5637 1] Remove shield if there is, otherwise, remove health
  (if (>= _shield Damage)
    (set `self.Shield` (- _shield Damage))
    (else
      (set `self.Health` (`KismetMathLibrary.FClamp` (- (`self.Health`) (- Damage (`self.Shield`))) 0.0 (`self.MaxHealth`)))
      (set `self.Shield` 0.0))))

(event `AddMaxHealth`
  (params (Value :type "Float (double-precision)"))
  (bind _returnvalue (+ (`self.MaxHealth`) Value))
  ;[0.277 0.5637 1] Add Max Health
  (if (> _returnvalue 0.0)
    (set `self.MaxHealth` _returnvalue)))

(event `RemoveShield`
  ;[0.277 0.5637 1] Remove shield
  (set `self.Shield` 0.0))

(event `Heal`
  (params (Value :type "Float (double-precision)"))
  (set `self.Health` (`KismetMathLibrary.FClamp` (+ (`self.Health`) Value) 0.0 (`self.MaxHealth`))))

(event `CreateWidgetOnClient`
  ;[0.8542 0.7797 0.2189] Create Test Widget
  (bind _returnvalue (`|CreateWidget` "/Game/ReplicatedHealthBar/Blueprints/WBP_TestReplicatedHealthBar.WBP_TestReplicatedHealthBar_C"))
  (`UserWidget.AddToViewport` _returnvalue 0))

(event `SetMaxHealthRatio`
  (bind _aswbp_replicated_health_bar (cast `/Game/ReplicatedHealthBar/Blueprints/WBP_ReplicatedHealthBar` (`self.GetWidget` self) :!pure true))
  ;[0.8542 0.7797 0.2189] Set Max Health Ratio (Called when Rep Notify Max Health change, so need to Set Health percent)
  (`/Game/ReplicatedHealthBar/Blueprints/WBP_ReplicatedHealthBar.SetMaxHealthRatio` _aswbp_replicated_health_bar (`self.GetMaxHealthRatio`))
  (`/Game/ReplicatedHealthBar/Blueprints/WBP_ReplicatedHealthBar.SetHealthPercent` _aswbp_replicated_health_bar (`self.GetHealthPercent`)))

(fn `CheckIfOverMaxHealth`
  (returns (ReturnValue :type Boolean))
  (return (<= (+ (`self.Health`) (`self.Shield`)) (`self.MaxHealth`))))

(fn `GetHealthPercent`
  (returns (ReturnValue :type "Float (double-precision)"))
  (if (`self.CheckIfOverMaxHealth`)
    ;[0.276 0.276 0.276] When health + shield under Max Health
    (return (/ (`self.Health`) (`self.MaxHealth`)))
    (else
      (return (/ (`self.Health`) (`self.GetTempMaxHealth`))))))

(fn `GetMaxHealthRatio`
  (returns (ReturnValue :type "Float (double-precision)"))
  (if (`self.CheckIfOverMaxHealth`)
    ;[0.276 0.276 0.276] When health + shield under Max Health
    (return (/ (`self.MaxHealth`) (`self.SmallBarHealthStep`)))
    (else
      (return (/ (`self.GetTempMaxHealth`) (`self.SmallBarHealthStep`))))))

(fn `GetTempMaxHealth`
  (returns (TempMaxHealth :type "Float (double-precision)"))
  (return (+ (`self.MaxHealth`) (- (+ (`self.Health`) (`self.Shield`)) (`self.MaxHealth`)))))

(fn `OnRep_Health`
  (`/Game/ReplicatedHealthBar/Blueprints/WBP_ReplicatedHealthBar.SetHealthPercent` (cast `/Game/ReplicatedHealthBar/Blueprints/WBP_ReplicatedHealthBar` (`self.GetWidget` self) :!pure true) (`self.GetHealthPercent`)))

(fn `OnRep_MaxHealth`
  (`self.SetMaxHealthRatio`))

(fn `OnRep_Shield`
  (`/Game/ReplicatedHealthBar/Blueprints/WBP_ReplicatedHealthBar.SetShield` (cast `/Game/ReplicatedHealthBar/Blueprints/WBP_ReplicatedHealthBar` (`self.GetWidget` self) :!pure true) (`KismetMathLibrary.SelectFloat` (/ (`self.Shield`) (`self.MaxHealth`)) (/ (`self.Shield`) (`self.GetTempMaxHealth`)) (`self.CheckIfOverMaxHealth`)))
  (`self.SetMaxHealthRatio`))