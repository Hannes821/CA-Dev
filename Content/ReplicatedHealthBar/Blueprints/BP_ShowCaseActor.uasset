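; BP_ShowCaseActor is a demo actor that exercises its BPHealthBar with random health changes.
; On BeginPlay it starts a looping timer, with an interval randomized once at under a second.
; Each tick of that timer randomly removes or adds shield, heals, raises or lowers max health, or damages the actor.
; Damage goes through ApplyDamageOnServer, which calls ApplyDamage with the actor as both target and causer.
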(event `ApplyDamageOnServer`
  (params (BaseDamage :type "Float (single-precision)"))
  (`GameplayStatics.ApplyDamage` self BaseDamage null self))

(event `self.ReceiveBeginPlay`
  (`KismetSystemLibrary.K2_SetTimerDelegate` (delegate `DoRandomThingToShowCase`) (`KismetMathLibrary.RandomFloatInRange` 0.6 1.0) true))

(event `DoRandomThingToShowCase`
  (bind _bp_healthbar (`self.BP_HealthBar`))
  (switch `int` (`KismetMathLibrary.RandomInteger` 6)
    (:`Default`
      (`self.ApplyDamageOnServer` 50.0 :!label _label))
    (:`0`
      (`/Game/ReplicatedHealthBar/Blueprints/BP_HealthBar.RemoveShield` _bp_healthbar))
    (:`1`
      (`/Game/ReplicatedHealthBar/Blueprints/BP_HealthBar.AddShield` _bp_healthbar 50.0))
    (:`2`
      (`/Game/ReplicatedHealthBar/Blueprints/BP_HealthBar.Heal` _bp_healthbar 50.0))
    (:`3`
      (goto _label))
    (:`4`
      (`/Game/ReplicatedHealthBar/Blueprints/BP_HealthBar.AddMaxHealth` _bp_healthbar 50.0))
    (:`5`
      (`/Game/ReplicatedHealthBar/Blueprints/BP_HealthBar.AddMaxHealth` _bp_healthbar -50.0))))

(fn `UserConstructionScript`)