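; BP_Sky is an environment actor providing an HDRI sky dome and exponential height fog, configured through exposed variables.
; The construction script creates a dynamic instance of MI_Skies for cubemap, tint, brightness and contrast, then sets dome yaw.
; It also configures fog visibility, color, density and altitude, with a global brightness scaling both sky and fog.
; Tick yaws the whole actor by a fixed amount each frame, without delta-time scaling.
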(event `self.ReceiveTick`
  (params (DeltaSeconds :type "Float (single-precision)"))
  ;[1 1 1] Rotation Speed
  (`self.K2_AddActorWorldRotation` (`KismetMathLibrary.MakeRotator` 0.0 0.0 (`self.HDRI_RotationSpeed`))))

(fn `UserConstructionScript`
  (`|ExecutionSequence`
    (:`then_0`
      ;[1 1 1] Material Instance
      (`SceneComponent.K2_SetWorldRotation` (`self.SM_SkyDome`) (struct) false false)
      (bind _returnvalue (`KismetMaterialLibrary.CreateDynamicMaterialInstance` "/Game/TreePackRealApple/Materials/Sky/MI_Skies.MI_Skies"))
      (bind _output_get (set `self.HDRI_MInst` _returnvalue))
      ;[1 1 1] HDRI Parameters
      (`PrimitiveComponent.SetMaterial` (`self.SM_SkyDome`) 0 _output_get)
      ;;[1 1 1] HDRI Brightness
      (`MaterialInstanceDynamic.SetScalarParameterValue` (`self.HDRI_MInst`) "HDRI_Brightness" (* (`self.HDRI_Brightness`) (`self.GlobalBrightness`)))
      (`MaterialInstanceDynamic.SetVectorParameterValue` (`self.HDRI_MInst`) "HDRI_Tint" (`self.HDRI_Tint`))
      (`MaterialInstanceDynamic.SetTextureParameterValue` (`self.HDRI_MInst`) "HDRI_Cubemap" (`self.HDRI_Cubemap`))
      ;;[1 1 1] Rotation
      (`SceneComponent.K2_SetWorldRotation` (`self.SM_SkyDome`) (`KismetMathLibrary.MakeRotator` 0.0 0.0 (`self.HDRI_Rotation`)) false false)
      (`MaterialInstanceDynamic.SetScalarParameterValue` (`self.HDRI_MInst`) "HDRI_Contrast" (`self.HDRI_Contrast`)))
    (:`then_1`
      ;[1 1 1] FogEnable
      (`SceneComponent.SetVisibility` (`self.ExponentialHeightFog`) (`self.UseFog`) false)
      ;[1 1 1] Fog Colors
      (`ExponentialHeightFogComponent.SetFogInscatteringColor` (`self.ExponentialHeightFog`) (* (`self.FogTint`) (`KismetMathLibrary.Conv_DoubleToLinearColor` (* (`self.GlobalBrightness`) (`self.FogBrightness`)))))
      ;[1 1 1] Fog Parameters
      (`ExponentialHeightFogComponent.SetFogMaxOpacity` (`self.ExponentialHeightFog`) (`self.FogMaxOpacity`))
      (`ExponentialHeightFogComponent.SetFogHeightFalloff` (`self.ExponentialHeightFog`) (`self.FogHeightFalloff`))
      (`ExponentialHeightFogComponent.SetFogDensity` (`self.ExponentialHeightFog`) (`self.FogDensity`))
      (`ExponentialHeightFogComponent.SetStartDistance` (`self.ExponentialHeightFog`) (`self.FogStartDistance`))
      (`SceneComponent.K2_SetWorldLocation` (`self.ExponentialHeightFog`) (`KismetMathLibrary.MakeVector` 0.0 0.0 (`self.FogAltitude`)) false false))))