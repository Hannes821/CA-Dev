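; Base character for AI attack animals, handling hunger, melee attacks, damage and death, with optional overhead stat bars.
; A hunger timer and damage events write hungry, angry and attacker keys to the Blackboard; the stamina update's timer is disconnected.
; Event-toggled gates face the enemy or attacker on Tick, while a socketed box knocks back and damages characters during attacks.
; Tick also optionally aligns the mesh to terrain; death ragdolls, then destroys the actor.
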(event `self.ReceiveBeginPlay`
  (bind _hungerlevelrate (`self.HungerLevelRate`))
  ;[1 1 1] Begin Play
  ;;[1 1 1] Begin Play
  ;;[1 1 1] Set I AmIAlive? to true
  (set `self.AmI Alive?` true)
  ;;[1 1 1] Set Hunger level to 0 and increase hunger at the "Hunger Level Tick Rate"
  (set `self.HungerLevel` 0.0)
  (`KismetSystemLibrary.K2_SetTimer` null "UpdateHungerLevel" (`KismetMathLibrary.RandomFloatInRange` (/ _hungerlevelrate 2.0) _hungerlevelrate) true)
  (set `self.StaminaLevel` 100.0)
  ;;[1 1 1] Draw overhead Health and Hunger bars
  (if (`self.DrawOverheadStats?`)
    (bind _returnvalue (`|CreateWidget` "/Game/CA_Units/Gaia/AttackAnimal_Boar/Boar/Blueprints/ParentClassBlueprints/AttackAnimal_Stat_WidgetBlueprint.AttackAnimal_Stat_WidgetBlueprint_C"))
    (set `self.Overhead Stat Bar` _returnvalue)
    ;;[1 1 1] Set  Health and Hunger bars
    (bind _asattack_animal_stat_widget_blueprint (cast `/Game/CA_Units/Gaia/AttackAnimal_Boar/Boar/Blueprints/ParentClassBlueprints/AttackAnimal_Stat_WidgetBlueprint` (`WidgetComponent.GetUserWidgetObject` (`self.OverHeadStatBar`))))
    (`ProgressBar.SetPercent` (`/Game/CA_Units/Gaia/AttackAnimal_Boar/Boar/Blueprints/ParentClassBlueprints/AttackAnimal_Stat_WidgetBlueprint.ProgressBar_Health` _asattack_animal_stat_widget_blueprint) (/ (`self.Health`) 100.0))
    (`ProgressBar.SetPercent` (`/Game/CA_Units/Gaia/AttackAnimal_Boar/Boar/Blueprints/ParentClassBlueprints/AttackAnimal_Stat_WidgetBlueprint.ProgressBar_Hunger` _asattack_animal_stat_widget_blueprint) (/ (`self.HungerLevel`) 100.0))
    (`ProgressBar.SetPercent` (`/Game/CA_Units/Gaia/AttackAnimal_Boar/Boar/Blueprints/ParentClassBlueprints/AttackAnimal_Stat_WidgetBlueprint.ProgressBar_Stamina` _asattack_animal_stat_widget_blueprint) (/ (`self.StaminaLevel`) 100.0))
    (else
      (`SceneComponent.SetVisibility` (`self.OverHeadStatBar`) false false))))

(event `self.ReceiveTick`
  (params (DeltaSeconds :type "Float (single-precision)"))
  (bind _mesh (`self.Mesh`))
  (bind _returnvalue (`BlackboardComponent.GetValueAsObject` (`AIBlueprintHelperLibrary.GetBlackboard` null) (`self.BBKey_ThisActorHurtMe`)))
  (bind _returnvalue_2 (`BlackboardComponent.GetValueAsObject` (`AIBlueprintHelperLibrary.GetBlackboard` null) (`self.BBKey_Enemy`)))
  (bind _returnvalue_3 (`SceneComponent.K2_GetComponentRotation` _mesh))
  (bind _returnvalue_4 (`SceneComponent.K2_GetComponentLocation` (`self.Capsule`)))
  (bind _camera (`/Game/CA_Code/Blueprints/Player/BP_RTSPawn.Camera` (cast `/Game/CA_Code/Blueprints/Player/BP_RTSPawn` (`GameplayStatics.GetPlayerPawn` 0) :!pure true)))
  ;[1 1 1] Tick
  (`|ExecutionSequence`
    (:`then_0`
      ;[1 1 1] Rotate the overhead health bar toward player character 0
      (if (`self.DrawOverheadStats?`)
        (if (`self.RotateHealthBarToPlayer?`)
          (if (`KismetSystemLibrary.IsValid` _camera)
            (`SceneComponent.K2_SetWorldRotation` (`self.OverHeadStatBar`) (`KismetMathLibrary.MakeRotator` 0.0 0.0 (.yaw (`KismetMathLibrary.FindLookAtRotation` (`SceneComponent.K2_GetComponentLocation` (`self.OverHeadStatBar`)) (`SceneComponent.K2_GetComponentLocation` _camera)))) false false)))))
    (:`then_1`
      ;[1 1 1] Attack Animation
      ;;[1 1 1] face the Enemy While Attacking
      (`/Engine/EditorBlueprintResources/StandardMacros.Gate` true :!label _label
        (:`Exit`
          (if (`KismetSystemLibrary.IsValid` _returnvalue_2)
            (bind _asactor (cast `Actor` _returnvalue_2))
            (`self.K2_SetActorRotation` (`KismetMathLibrary.MakeRotator` 0.0 0.0 (.yaw (`KismetMathLibrary.FindLookAtRotation` (`self.K2_GetActorLocation`) (`self.K2_GetActorLocation` _asactor)))))))))
    (:`then_2`
      ;;[1 1 1] face the Attacker While Attacking
      (`/Engine/EditorBlueprintResources/StandardMacros.Gate` true :!label _label_2
        (:`Exit`
          (if (`KismetSystemLibrary.IsValid` _returnvalue)
            (bind _asactor_2 (cast `Actor` _returnvalue))
            (`self.K2_SetActorRotation` (`KismetMathLibrary.MakeRotator` 0.0 0.0 (.yaw (`KismetMathLibrary.FindLookAtRotation` (`self.K2_GetActorLocation`) (`self.K2_GetActorLocation` _asactor_2)))))))))
    (:`then_3`
      ;[1 1 1] Orient to the ground
      (if (`self.Align to the ground?`)
        (bind (_outhit _returnvalue_5) (`KismetSystemLibrary.LineTraceSingle` _returnvalue_4 (+ _returnvalue_4 (0.0 0.0 -350.0)) "TraceTypeQuery1"))
        (if _returnvalue_5
          (bind (_bblockinghit _binitialoverlap _time _distance _location _impactpoint _normal) (`GameplayStatics.BreakHitResult` _outhit))
          (`SceneComponent.K2_SetWorldRotation` (`self.Mesh`) (`KismetMathLibrary.RInterpTo` _returnvalue_3 (`KismetMathLibrary.MakeRotator` (* (.roll (`KismetMathLibrary.MakeRotFromXZ` (`SceneComponent.GetForwardVector` _mesh) _normal)) (`self.OrientationRoll%`)) (* (.pitch (`KismetMathLibrary.MakeRotFromYZ` (`SceneComponent.GetRightVector` _mesh) _normal)) (`self.OrientationPitch%`)) (.yaw _returnvalue_3)) (`GameplayStatics.GetWorldDeltaSeconds`) 1.0) false false))))))

(event `RotateToFace_Enemy`
  ;[1 1 1] Attack Animation
  ;;[1 1 1] face the Enemy While Attacking
  (goto _label :!via `Open`))

(event `Stop_Facing_Enemy`
  ;[1 1 1] Attack Animation
  ;;[1 1 1] face the Enemy While Attacking
  (goto _label :!via `Close`))

(event `self.Box.OnComponentBeginOverlap`
  (params (OverlappedComponent :type "PrimitiveComponent Object Reference") (OtherActor :type "Actor Object Reference") (OtherComp :type "PrimitiveComponent Object Reference") (OtherBodyIndex :type Integer) (bFromSweep :type Boolean) (SweepResult :type "HitResult Structure (by ref)"))
  ;[1 1 1] Attack Animation
  ;;[1 1 1] KnockBack enemy and do damage while playing attack animation
  (for _array_element (`PrimitiveComponent.GetOverlappingActors` (`self.Box`) "/Script/Engine.Actor")
    (if (not (== (`GameplayStatics.GetObjectClass` _array_element) (`GameplayStatics.GetObjectClass` self)))
      (bind _ascharacter (cast `Character` _array_element))
      (if (`self.IsAttacking?`)
        (`/Engine/EditorBlueprintResources/StandardMacros.DoOnce` false :!label _label_3
          (:`Completed`
            (`self.LaunchCharacter` _ascharacter (`KismetMathLibrary.ClampVectorSize` (* (- (`self.K2_GetActorLocation` _ascharacter) (`SceneComponent.K2_GetComponentLocation` (`self.Mesh`))) 1.8) 0.0 800.0) false false)
            (`GameplayStatics.ApplyDamage` _ascharacter (`self.MeleeDamageAmount`) null self)
            (`KismetSystemLibrary.Delay` 1.0)
            (goto _label_3 :!via `Reset`)))))))

(event `self.Box.OnComponentEndOverlap`
  (params (OverlappedComponent :type "PrimitiveComponent Object Reference") (OtherActor :type "Actor Object Reference") (OtherComp :type "PrimitiveComponent Object Reference") (OtherBodyIndex :type Integer))
  ;[1 1 1] Attack Animation
  ;;[1 1 1] KnockBack enemy and do damage while playing attack animation
  (goto _label_3 :!via `Reset`))

(event `RotateToAttacker`
  ;[1 1 1] Attack Animation
  ;;[1 1 1] face the Attacker While Attacking
  (goto _label_2 :!via `Open`))

(event `Stop_Facing_Attacker`
  ;[1 1 1] Attack Animation
  ;;[1 1 1] face the Attacker While Attacking
  (goto _label_2 :!via `Close`))

(event `LaunchForwardForAttack`
  (bind _returnvalue (`self.GetMovementComponent`))
  (bind _updatedcomponent (`MovementComponent.UpdatedComponent` _returnvalue))
  ;[1 1 1] Attack Animation
  ;;[1 1 1] Launch Character Forward during attack animation
  (set `CharacterMovementComponent.GroundFriction` 2.0 (`self.CharacterMovement`))
  (`self.LaunchCharacter` (+ (`MovementComponent.Velocity` _returnvalue) (* (`SceneComponent.GetForwardVector` _updatedcomponent) 500.0) (* (`SceneComponent.GetUpVector` _updatedcomponent) 3.0)))
  (`KismetSystemLibrary.RetriggerableDelay` 1.0)
  (set `CharacterMovementComponent.GroundFriction` 4.0 (`self.CharacterMovement`)))

(event `self.ReceiveAnyDamage`
  (params (Damage :type "Float (single-precision)") (DamageType :type "DamageType Object Reference") (InstigatedBy :type "Controller Object Reference") (DamageCauser :type "Actor Object Reference"))
  (bind _bbkey_amiangry_ (`self.BBKey_AmIAngry?`))
  ;[1 1 1] Damage
  ;;[1 1 1] Event- Damage
  (`|ExecutionSequence`
    (:`then_0`
      ;;[1 1 1] Set "AmIAngry?" in the Blackboard to true for the AngerDuration then back to false
      (`BlackboardComponent.SetValueAsBool` (`AIBlueprintHelperLibrary.GetBlackboard` null) _bbkey_amiangry_ true)
      (`KismetSystemLibrary.Delay` (`self.AngerDuration`))
      (`BlackboardComponent.SetValueAsBool` (`AIBlueprintHelperLibrary.GetBlackboard` null) _bbkey_amiangry_ false))
    (:`then_1`
      ;;[1 1 1] Set ThisActorHurtMe in Blackboard
      (`BlackboardComponent.SetValueAsObject` (`AIBlueprintHelperLibrary.GetBlackboard` null) (`self.BBKey_ThisActorHurtMe`) DamageCauser)
      (`KismetSystemLibrary.Delay` (`self.AngerDuration`))
      (`BlackboardComponent.SetValueAsObject` (`AIBlueprintHelperLibrary.GetBlackboard` null) (`self.BBKey_ThisActorHurtMe`) null))
    (:`then_2`
      ;;[1 1 1] Reduce Health
      (set `self.Health` (`KismetMathLibrary.FMax` (- (`self.Health`) Damage)))
      (`|ExecutionSequence`
        (:`then_0`
          ;;[1 1 1] Update HealthBar
          (if (`self.DrawOverheadStats?`)
            (bind _asattack_animal_stat_widget_blueprint (cast `/Game/CA_Units/Gaia/AttackAnimal_Boar/Boar/Blueprints/ParentClassBlueprints/AttackAnimal_Stat_WidgetBlueprint` (`WidgetComponent.GetUserWidgetObject` (`self.OverHeadStatBar`))))
            (`ProgressBar.SetPercent` (`/Game/CA_Units/Gaia/AttackAnimal_Boar/Boar/Blueprints/ParentClassBlueprints/AttackAnimal_Stat_WidgetBlueprint.ProgressBar_Health` _asattack_animal_stat_widget_blueprint) (/ (`self.Health`) 100.0))))
        (:`then_1`
          ;;[1 1 1] When health is below 0- Ragdoll
          (if (<= (`self.Health`) 0.0)
            (`SceneComponent.SetVisibility` (`self.OverHeadStatBar`) false false)
            (set `self.AmI Alive?` false)
            (set `self.IsAttacking?` false)
            ;;;[1 1 1] Ragdoll Mesh
            (`PrimitiveComponent.SetSimulatePhysics` (`self.Mesh`) true)
            (`PrimitiveComponent.SetCollisionEnabled` (`self.CapsuleComponent`) "NoCollision")
            (`PrimitiveComponent.SetCollisionEnabled` (`self.Capsule`) "NoCollision")
            (set `CharacterMovementComponent.GravityScale` -3.0 (`self.CharacterMovement`))
            (`KismetSystemLibrary.Delay` 20.0)
            ;;;[1 1 1] Destroy Actor
            (`self.K2_DestroyActor`)
            (`KismetSystemLibrary.CollectGarbage`)))
        (:`then_2`
          ;;[1 1 1] We just got hurt- this is no time to stand around
          (set `self.PlayIdle?` false))))))

(fn `UpdateHungerLevel`
  (bind _bbkey_amihungry_ (`self.BBKey_AmIHungry?`))
  (set `self.HungerLevel` (`KismetMathLibrary.FMin` (+ (`self.HungerLevel`) 1.0) 100.0))
  (bind _asattack_animal_stat_widget_blueprint (cast `/Game/CA_Units/Gaia/AttackAnimal_Boar/Boar/Blueprints/ParentClassBlueprints/AttackAnimal_Stat_WidgetBlueprint` (`WidgetComponent.GetUserWidgetObject` (`self.OverHeadStatBar`))))
  (`ProgressBar.SetPercent` (`/Game/CA_Units/Gaia/AttackAnimal_Boar/Boar/Blueprints/ParentClassBlueprints/AttackAnimal_Stat_WidgetBlueprint.ProgressBar_Hunger` _asattack_animal_stat_widget_blueprint) (/ (`self.HungerLevel`) 100.0))
  (if (>= (`self.HungerLevel`) 99.0)
    (set `self.AmIHungry?` true)
    (`BlackboardComponent.SetValueAsBool` (`AIBlueprintHelperLibrary.GetBlackboard` null) _bbkey_amihungry_ true)
    (else
      (set `self.AmIHungry?` false)
      (`BlackboardComponent.SetValueAsBool` (`AIBlueprintHelperLibrary.GetBlackboard` null) _bbkey_amihungry_ false))))

(fn `UpdateStaminaLevel`
  (bind _bbkey_amitired_ (`self.BBKey_AmITired?`))
  (set `self.StaminaLevel` (`KismetMathLibrary.FMax` (`KismetMathLibrary.FMin` (- (`self.StaminaLevel`) 1.0) 100.0)))
  (bind _asattack_animal_stat_widget_blueprint (cast `/Game/CA_Units/Gaia/AttackAnimal_Boar/Boar/Blueprints/ParentClassBlueprints/AttackAnimal_Stat_WidgetBlueprint` (`WidgetComponent.GetUserWidgetObject` (`self.OverHeadStatBar`))))
  (`ProgressBar.SetPercent` (`/Game/CA_Units/Gaia/AttackAnimal_Boar/Boar/Blueprints/ParentClassBlueprints/AttackAnimal_Stat_WidgetBlueprint.ProgressBar_Stamina` _asattack_animal_stat_widget_blueprint) (/ (`self.StaminaLevel`) 100.0))
  (if (<= (`self.StaminaLevel`) 1.0)
    (set `self.AmITired?` true)
    (`BlackboardComponent.SetValueAsBool` (`AIBlueprintHelperLibrary.GetBlackboard` null) _bbkey_amitired_ true)
    (else
      (set `self.AmITired?` false)
      (`BlackboardComponent.SetValueAsBool` (`AIBlueprintHelperLibrary.GetBlackboard` null) _bbkey_amitired_ false))))

(fn `UserConstructionScript`
  (`SceneComponent.K2_AttachTo` (`self.Box`) (`self.Mesh`) "Attack" "SnapToTarget" false)
  (set `self.PlayerTeamNr` 9))