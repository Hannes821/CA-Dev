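; AI controller for pigs that tracks enemies and leader pigs through perception and stores nearby path nodes, shuffled, at construction.
; Perceived "PigEnemy" actors join an enemy list, and followers record a seen leader in the blackboard.
; EnemySelection scores enemies with a distance curve and writes the top one to the blackboard.
; Behavior tree startup, blackboard initialization and the selection and expiry timers are disconnected from Possess, so never run.
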(event `ExpireEnemies`
  ;[1 1 1] Remove Expired Enemies
  (`self.RemoveExpiredEnemies`))

(event `self.ReceivePossess`
  (params (PossessedPawn :type "Pawn Object Reference"))
  ;[1 1 1] On Possess
)

(event `EnemySelection`
  (bind _enemytarget (`self.EnemyTarget`))
  ;[1 1 1] Select a Enemy
  (`|ExecutionSequence`
    (:`then_0`
      (`self.RemoveDeadEnemys`))
    (:`then_1`
      ;;[1 1 1] Enemy Evaluation
      (for (_array_element _array_index) (`self.Enemies`)
        (bind _utility (`self.CalculateDistanceUtility` _array_element))
        (bind (_actor _weight _lastseen) (break `/Game/CA_Units/Gaia/Pigs/AI/Pig_EnemySelection_Structure` _array_element))
        (`KismetArrayLibrary.Array_Set` (`self.Enemies`) _array_index (make `/Game/CA_Units/Gaia/Pigs/AI/Pig_EnemySelection_Structure` _actor (+ _utility 0.0) _lastseen))))
    (:`then_2`
      ;;[1 1 1] Find our Current Highest Enemy Target
      ;;;[1 1 1] Clear settings so we get a clean calculation every time
      (set `self.EnemyTarget` null)
      (set `self.CurrentHighestEnemyTarget` 0.0)
      (for _array_element_2 (`self.Enemies`)
        (bind (_actor_2 _weight_2) (break `/Game/CA_Units/Gaia/Pigs/AI/Pig_EnemySelection_Structure` _array_element_2))
        (if (> _weight_2 (`self.CurrentHighestEnemyTarget`))
          (set `self.EnemyTarget` _actor_2)
          (set `self.CurrentHighestEnemyTarget` _weight_2))))
    (:`then_3`
      ;;[1 1 1] Set our highest Enemy Target as our enemy in the blackboard
      (if (!= (`self.Enemy`) _enemytarget)
        (bind _output_get (set `self.Enemy` _enemytarget))
        (`/Engine/EditorBlueprintResources/StandardMacros.IsValid` _output_get
          (:`Is Valid`
            (`BlackboardComponent.SetValueAsObject` (`AIBlueprintHelperLibrary.GetBlackboard` null) (`self.BlackboardKey_Enemy`) _output_get))
          (:`Is Not Valid`
            ;;[1 1 1] Set Enemy to null
            (`BlackboardComponent.SetValueAsObject` (`AIBlueprintHelperLibrary.GetBlackboard` null) (`self.BlackboardKey_Enemy`) null)))))
    (:`then_4`
      ;;[1 1 1] Set "EnemySpotted?" to true in the Blackboard
      ;; if we have a valid enemy and False if we do not
      (`/Engine/EditorBlueprintResources/StandardMacros.IsValid` (`self.Enemy`)
        (:`Is Valid`
          (`BlackboardComponent.SetValueAsBool` (`self.Blackboard`) (`self.BbKey_EnemySpotted?`) true))
        (:`Is Not Valid`
          (`BlackboardComponent.SetValueAsBool` (`self.Blackboard`) (`self.BbKey_EnemySpotted?`) false))))))

(event `OnEnemyDestroyed` :!signature `self.OnDestroyed`
  (params (DestroyedActor :type "Actor Object Reference"))
  ;[1 1 1] Bind event if enemy is destroyed-
  ; so we can remove non valad Enemies
  ; from the "Enemies" array
  (`KismetSystemLibrary.CollectGarbage`))

(event `self.AIPerception.OnPerceptionUpdated`
  (params (UpdatedActors :type "Array of Actor Object Reference (by ref)"))
  ;[1 1 1] On Perception Update
  (`|ExecutionSequence`
    (:`then_0`
      ;[1 1 1] Any Actor with this tag "PigEnemy"
      (for _array_element UpdatedActors
        (bind _info (`AIPerceptionComponent.GetActorsPerception` (`self.AIPerception`) _array_element))
        (bind _target (break `ActorPerceptionBlueprintInfo` _info))
        (if (`self.ActorHasTag` _target "PigEnemy")
          ;[1 1 1] Add Actor to the "Enemies" array
          (`self.AddActorToEnemiesArray` _target)
          ;[1 1 1] Bind event if enemy is destroyed-
          ; so we can remove non valad Enemies
          ; from the "Enemies" array
          (add `self.OnDestroyed` _target (delegate `OnEnemyDestroyed`)))))
    (:`then_1`
      ;[1 1 1] Did I see a Leader?
      (for _array_element_2 UpdatedActors
        (bind _info_2 (`AIPerceptionComponent.GetActorsPerception` (`self.AIPerception`) _array_element_2))
        (bind _asbp_npc_pig_base (cast `/Game/CA_Units/Gaia/Pigs/Blueprints/ParentClassBlueprints/BP_NPC_Pig_Base` _array_element_2))
        (if (`/Game/CA_Units/Gaia/Pigs/Blueprints/ParentClassBlueprints/BP_NPC_Pig_Base.AmIALeader?` _asbp_npc_pig_base)
          ;[1 1 1] Do I follow leaders?
          (if (`BlackboardComponent.GetValueAsBool` (`AIBlueprintHelperLibrary.GetBlackboard` self) (`self.BbKey_DoIFollowLeaders?`))
            ;[1 1 1] if we have no Actor to follow
            (if (not (`KismetSystemLibrary.IsValid` (`BlackboardComponent.GetValueAsObject` (`AIBlueprintHelperLibrary.GetBlackboard` null) (`self.BBKey_LeaderPigToFollow`))))
              ;[1 1 1] Set Actor to follow
              (`BlackboardComponent.SetValueAsObject` (`AIBlueprintHelperLibrary.GetBlackboard` null) (`self.BBKey_LeaderPigToFollow`) (`.Target` (break `ActorPerceptionBlueprintInfo` _info_2)))
              (`BlackboardComponent.SetValueAsBool` (`AIBlueprintHelperLibrary.GetBlackboard` null) (`self.BbKey_FoundAPigToFollow?`) true))))))))

(fn `AddActorToEnemiesArray`
  (params (InputActor :type "Actor Object Reference"))
  (locals (`IsActorInArray?` :type Boolean))
  (bind (_actor _weight) (break `/Game/CA_Units/Gaia/Pigs/AI/Pig_EnemySelection_Structure` (`|GetArrayItem` (`self.Enemies`) (`self.LastSeenIndex`))))
  (`|ExecutionSequence`
    (:`then_0`
      ;[1 1 1] Check if the Actor is already in the "Enemies" array
      (set `local.IsActorInArray?` false)
      (for (_array_element _array_index) (`self.Enemies`)
        (if (== (`.Actor_2_9F3699F344F7A605C2832DA413AE8B60` (break `/Game/CA_Units/Gaia/Pigs/AI/Pig_EnemySelection_Structure` _array_element)) InputActor)
          (set `local.IsActorInArray?` true)
          (set `self.LastSeenIndex` _array_index)
          (break))))
    (:`then_1`
      (if (`local.IsActorInArray?`)
        ;[1 1 1] Actor is in Array, so just reset the last seen time
        (`KismetArrayLibrary.Array_Set` (`self.Enemies`) (`self.LastSeenIndex`) (make `/Game/CA_Units/Gaia/Pigs/AI/Pig_EnemySelection_Structure` _actor _weight))
        (else
          ;[1 1 1] Actor is new, so add it to the "Enemies" array
          (`KismetArrayLibrary.Array_Add` (`self.Enemies`) (make `/Game/CA_Units/Gaia/Pigs/AI/Pig_EnemySelection_Structure` InputActor)))))))

(fn `ApplyDamageFromActor`
  (params (DamagingActor :type "Actor Object Reference") (Damage :type "Float (double-precision)"))
  (`/Engine/EditorBlueprintResources/StandardMacros.IsValid` DamagingActor
    (:`Is Valid`
      (for (_array_element _array_index) (`self.Enemies`)
        (if (== null DamagingActor)
          (bind (_actor _weight _lastseen) (break `/Game/CA_Units/Gaia/Pigs/AI/Pig_EnemySelection_Structure` _array_element))
          (`KismetArrayLibrary.Array_Set` (`self.Enemies`) _array_index (make `/Game/CA_Units/Gaia/Pigs/AI/Pig_EnemySelection_Structure` _actor _weight _lastseen))
          (break))))))

(fn `CalculateDistanceToActor`
  (params (InputActor :type "Actor Object Reference"))
  (returns (DistanceToActor :type "Float (double-precision)"))
  (if (`KismetSystemLibrary.IsValid` InputActor)
    (return (`KismetMathLibrary.VSize` (- (`self.K2_GetActorLocation` InputActor) (`self.K2_GetActorLocation` (`self.K2_GetPawn`)))))
    (else
      (return 4000.0))))

(fn `CalculateDistanceUtility`
  (params (ThreatStructureInput :type "/Game/CA_Units/Gaia/Pigs/AI/Pig_EnemySelection_Structure Structure"))
  (returns (Utility :type "Float (double-precision)"))
  (return (`CurveFloat.GetFloatValue` (`self.EnemyDistanceCurve`) (`self.CalculateDistanceToActor` (`.Actor_2_9F3699F344F7A605C2832DA413AE8B60` (break `/Game/CA_Units/Gaia/Pigs/AI/Pig_EnemySelection_Structure` ThreatStructureInput))))))

(fn `RemoveDeadEnemys`
  (locals (EnemiesToRemove :type "Array of /Game/CA_Units/Gaia/Pigs/AI/Pig_EnemySelection_Structure Structure"))
  (for _array_element (`self.Enemies`)
    (`|ExecutionSequence`
      (:`then_0`
        (bind _actor (break `/Game/CA_Units/Gaia/Pigs/AI/Pig_EnemySelection_Structure` _array_element))
        ;[1 1 1] Remove this actor if AmIAlive? is false (DeadActor)
        (if (`KismetSystemLibrary.IsValid` _actor)
          (bind _asbp_character_base_with_health (cast `/Game/CA_Units/Gaia/Pigs/Blueprints/ParentClassBlueprints/BP_CharacterBaseWithHealth` _actor))
          (if (not (`/Game/CA_Units/Gaia/Pigs/Blueprints/ParentClassBlueprints/BP_CharacterBaseWithHealth.AmI Alive?` _asbp_character_base_with_health))
            (`KismetArrayLibrary.Array_Add` (`local.EnemiesToRemove`) _array_element))))
      (:`then_1`
        ;[1 1 1] Remove any Enemies that are not valid
        (`/Engine/EditorBlueprintResources/StandardMacros.IsValid` _actor
          (:`Is Not Valid`
            (`KismetArrayLibrary.Array_Add` (`local.EnemiesToRemove`) _array_element))))))
  ;[1 1 1] Remove and clear Local Var
  (for _array_element_2 (`local.EnemiesToRemove`)
    (`KismetArrayLibrary.Array_RemoveItem` (`local.EnemiesToRemove`) _array_element_2))
  (`KismetArrayLibrary.Array_Clear` (`local.EnemiesToRemove`)))

(fn `RemoveExpiredEnemies`
  (locals (EnemiesToRemove :type "Array of /Game/CA_Units/Gaia/Pigs/AI/Pig_EnemySelection_Structure Structure"))
  (for _array_element (`self.Enemies`)
    (`|ExecutionSequence`
      (:`then_0`
        (bind (_actor _weight _lastseen) (break `/Game/CA_Units/Gaia/Pigs/AI/Pig_EnemySelection_Structure` _array_element))
        ;[1 1 1] Expire this actor if last seen time is more than the "EnemyExpirationTime"
        (if (>= _lastseen (`self.EnemyExpirationTime`))
          (`KismetArrayLibrary.Array_Add` (`local.EnemiesToRemove`) _array_element)))
      (:`then_1`
        ;[1 1 1] Remove any threats that are not valid
        (`/Engine/EditorBlueprintResources/StandardMacros.IsValid` _actor
          (:`Is Not Valid`
            (`KismetArrayLibrary.Array_Add` (`local.EnemiesToRemove`) _array_element))))))
  ;[1 1 1] Remove these actors from the "Threats" array
  (for _array_element_2 (`local.EnemiesToRemove`)
    (`KismetArrayLibrary.Array_RemoveItem` (`self.Enemies`) _array_element_2))
  (`KismetArrayLibrary.Array_Clear` (`local.EnemiesToRemove`)))

(fn `UserConstructionScript`
  ;[1 1 1] Store Sky Targets within Distance Range (Distance is set in the AIController variable "StoreTargetsWithinThisRange")
  (bind _outactors (`GameplayStatics.GetAllActorsOfClass` "/Game/CA_Units/Gaia/Pigs/Blueprints/BP_Pig_Path_Node.BP_Pig_Path_Node_C"))
  (for _array_element _outactors
    (if (<= (`self.GetDistanceTo` _array_element self) (`self.StoreTargetsWithinThisRange`))
      (`KismetArrayLibrary.Array_Add` (`self.PigGroundTargets`) _array_element)))
  (`KismetArrayLibrary.Array_Shuffle` (`self.PigGroundTargets`)))