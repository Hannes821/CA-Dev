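; Base character Blueprint with a health component that handles a unit's death and corpse cleanup.
; BeginPlay binds to the component's zero-health event, and OnDeath stops the AI brain logic, disables mesh collision and enables physics simulation for a ragdoll.
; It applies a scaled attack impulse and makes the capsule ignore Pawn and Visibility channels.
; DestroyCorpse then waits out a decay timer, destroys the actor and forces garbage collection.
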(event `self.ReceiveBeginPlay`
  (add `/Game/CA_Code/Blueprints/ActorsComponents/AttributeComponents/HealthComponent.OnZeroHealth` (`self.HealthComponent`) (`|CreateDelegate` :!event `OnDeath`)))

(event `DestroyCorpse`
  (`KismetSystemLibrary.Delay` (`self.CorpseDecayTimer`))
  (`self.K2_DestroyActor`)
  (`KismetSystemLibrary.CollectGarbage`))

(fn `OnDeath`
  (params (Actor :type "Actor Object Reference"))
  (locals (AttackImpulse :type "Vector Structure" :default (70.0 70.0 70.0)))
  (bind _capsulecomponent (`self.CapsuleComponent`))
  (bind _mesh (`self.Mesh`))
  (`BrainComponent.StopLogic` (`AIController.BrainComponent` (`AIBlueprintHelperLibrary.GetAIController` Actor)) "")
  (`KismetSystemLibrary.PrintString` "death")
  ;[0.1978 1 0.1444] ragdoll on death event
  (`PrimitiveComponent.SetCollisionEnabled` _mesh "NoCollision")
  (`PrimitiveComponent.SetSimulatePhysics` _mesh true)
  (`SkeletalMeshComponent.SetAllBodiesSimulatePhysics` (`self.Mesh`) true)
  (`PrimitiveComponent.AddImpulse` _mesh (* (`local.AttackImpulse`) (100.0 100.0 10.0)) "None" false)
  ;[0 0.02764 1] Collission disabled
  (`PrimitiveComponent.SetCollisionResponseToChannel` _capsulecomponent "ECC_Pawn" "ECR_Ignore")
  (`PrimitiveComponent.SetCollisionResponseToChannel` _capsulecomponent "ECC_Visibility" "ECR_Ignore")
  (`self.DestroyCorpse`))

(fn `UserConstructionScript`)