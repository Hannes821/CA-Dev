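; BP_Window is an interactive window with two hinged leaves that the player toggles open and closed with the F key.
; Overlapping either trigger box (Box_L, Box_R) enables input for player controller 0 and leaving disables it, with no check on the overlapping actor.
; Each leaf (Door1, Door2) has its own F handler, where a FlipFlop plays or reverses a timeline driving its relative yaw.
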(event `self.Box_R.OnComponentBeginOverlap`
  (params (OverlappedComponent :type "PrimitiveComponent Object Reference") (OtherActor :type "Actor Object Reference") (OtherComp :type "PrimitiveComponent Object Reference") (OtherBodyIndex :type Integer) (bFromSweep :type Boolean) (SweepResult :type "HitResult Structure (by ref)"))
  ;[1 1 1] Enable_Or_Disable_Input
  (`self.EnableInput` (`GameplayStatics.GetPlayerController` 0) :!label _label))

(event `self.Box_L.OnComponentBeginOverlap`
  (params (OverlappedComponent :type "PrimitiveComponent Object Reference") (OtherActor :type "Actor Object Reference") (OtherComp :type "PrimitiveComponent Object Reference") (OtherBodyIndex :type Integer) (bFromSweep :type Boolean) (SweepResult :type "HitResult Structure (by ref)"))
  ;[1 1 1] Enable_Or_Disable_Input
  (goto _label))

(event `self.Box_L.OnComponentEndOverlap`
  (params (OverlappedComponent :type "PrimitiveComponent Object Reference") (OtherActor :type "Actor Object Reference") (OtherComp :type "PrimitiveComponent Object Reference") (OtherBodyIndex :type Integer))
  ;[1 1 1] Enable_Or_Disable_Input
  (`self.DisableInput` (`GameplayStatics.GetPlayerController` 0) :!label _label_2))

(event `self.Box_R.OnComponentEndOverlap`
  (params (OverlappedComponent :type "PrimitiveComponent Object Reference") (OtherActor :type "Actor Object Reference") (OtherComp :type "PrimitiveComponent Object Reference") (OtherBodyIndex :type Integer))
  ;[1 1 1] Enable_Or_Disable_Input
  (goto _label_2))

(event `Key|F`
  (params (Key :type "Key Structure"))
  ;[1 1 1] Open Doors with F Key
  (:`Pressed`
    (`/Engine/EditorBlueprintResources/StandardMacros.FlipFlop`
      (:`A`
        (bind (_direction _open_door) (`Timeline|Timeline_0` :!label _label_3)
          (:`Update`
            (`SceneComponent.K2_SetRelativeRotation` (`self.Door_1`) (`KismetMathLibrary.MakeRotator` 0.0 0.0 _open_door) false false))))
      (:`B`
        (goto _label_3 :!via `Reverse`)))))

(event `Key|F`
  (params (Key :type "Key Structure"))
  ;[1 1 1] Open Doors with F Key
  (:`Pressed`
    (`/Engine/EditorBlueprintResources/StandardMacros.FlipFlop`
      (:`A`
        (bind (_direction _open_door) (`Timeline|Timeline_1` :!label _label_4)
          (:`Update`
            (`SceneComponent.K2_SetRelativeRotation` (`self.Door_2`) (`KismetMathLibrary.MakeRotator` 0.0 0.0 _open_door) false false))))
      (:`B`
        (goto _label_4 :!via `Reverse`)))))

(fn `UserConstructionScript`)