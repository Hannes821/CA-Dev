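; BP_LakeWater is a placeable lake water surface whose look and size are set from exposed variables.
; Its construction script calls InitialWaterCreation, which creates a dynamic instance of OceanMaterial on the WaterSurface component and scales that component in X and Y.
; It then pushes scale, variation, wave speed, two colours and opacity into the material parameters.
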(fn `UserConstructionScript`
  (bind _watersurface (`self.WaterSurface`))
  (bind _water_material (`self.Water Material`))
  (bind _returnvalue (`PrimitiveComponent.CreateDynamicMaterialInstance` _watersurface 0 (`self.Ocean Material`) "None"))
  (set `self.Water Material` _returnvalue)
  (`SceneComponent.SetRelativeScale3D` _watersurface (`KismetMathLibrary.MakeVector` (`self.Water Scale X`) (`self.Water Scale Y`) 1.0))
  (`MaterialInstanceDynamic.SetScalarParameterValue` _water_material "Water Scale" (`self.Overall Water Scale`))
  (`MaterialInstanceDynamic.SetScalarParameterValue` _water_material "Variation Amount" (`self.Variation Amount`))
  (`MaterialInstanceDynamic.SetScalarParameterValue` _water_material "Wave Speed" (`self.Wave Speed`))
  (`MaterialInstanceDynamic.SetVectorParameterValue` _water_material "WaterColor A" (`self.Primary Water Color`))
  (`MaterialInstanceDynamic.SetVectorParameterValue` _water_material "WaterColor B" (`self.Secondary Water Color`))
  (`MaterialInstanceDynamic.SetScalarParameterValue` _water_material "Opacity" (`self.Opacity`)))