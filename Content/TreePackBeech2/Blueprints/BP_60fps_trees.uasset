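; Control actor for the beech tree pack that drives global wind and seasonal appearance of the trees through two Material Parameter Collections.
; The Icon component's yaw sets wind direction, alongside strength and simple sway amount and speed in MP_WindParameters.
; Day of year and packed threshold vectors for leaf growth, bloom, fall, apples and color shifts go to MPC_Tree_Seasons.
; Values are written in the construction script and again on BeginPlay via UpdateParamters, with no per-tick update.
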(event `self.ReceiveBeginPlay`
  (`self.Update Paramters`))

(fn `Update Paramters`
  (`KismetMaterialLibrary.SetScalarParameterValue` "/Game/TreePackBeech2/Materials/CollectionParamaters/MPC_Tree_Seasons.MPC_Tree_Seasons" "DAY" (`self.Day of year`))
  (`KismetMaterialLibrary.SetScalarParameterValue` "/Game/TreePackBeech2/Materials/CollectionParamaters/MP_WindParameters.MP_WindParameters" "Direction (0-1)" (/ (.yaw (`SceneComponent.K2_GetComponentRotation` (`self.Icon`))) 180.0))
  (`KismetMaterialLibrary.SetScalarParameterValue` "/Game/TreePackBeech2/Materials/CollectionParamaters/MP_WindParameters.MP_WindParameters" "Strenght (0-5)" (`self.Wind Strenght`))
  (`KismetMaterialLibrary.SetScalarParameterValue` "/Game/TreePackBeech2/Materials/CollectionParamaters/MP_WindParameters.MP_WindParameters" "Low Amount(0-5)" (`self.Simple Wind Amount`))
  (`KismetMaterialLibrary.SetScalarParameterValue` "/Game/TreePackBeech2/Materials/CollectionParamaters/MP_WindParameters.MP_WindParameters" "Low Speed(0-5)" (`self.Simple Wind Speed`))
  (`KismetMaterialLibrary.SetVectorParameterValue` "/Game/TreePackBeech2/Materials/CollectionParamaters/MPC_Tree_Seasons.MPC_Tree_Seasons" "Leaves - Growth / Flowers - Bloom" (`KismetMathLibrary.MakeColor` (`self.Leaves Growth Start`) (`self.Leaves Growth End`) (`self.Flowers Bloom Start`) (`self.Flowers Bloom End`)))
  (`KismetMaterialLibrary.SetVectorParameterValue` "/Game/TreePackBeech2/Materials/CollectionParamaters/MPC_Tree_Seasons.MPC_Tree_Seasons" "Leaves Fall / Apples - On" (`KismetMathLibrary.MakeColor` (`self.Leaves Fall Start Shift`) (`self.Leaves Fall Start All`) (`self.Apples Start`) (`self.Apples End`)))
  (`KismetMaterialLibrary.SetVectorParameterValue` "/Game/TreePackBeech2/Materials/CollectionParamaters/MPC_Tree_Seasons.MPC_Tree_Seasons" "Leaves Color Shift" (`KismetMathLibrary.MakeColor` (`self.Spring / Summer`) (`self.Summer / Autumn`) (`self.Autumn01 / Autumn02`) (`self.Autumn02 / Winter`))))

(fn `UserConstructionScript`
  (`KismetMaterialLibrary.SetScalarParameterValue` "/Game/TreePackBeech2/Materials/CollectionParamaters/MP_WindParameters.MP_WindParameters" "Direction (0-1)" (/ (.yaw (`SceneComponent.K2_GetComponentRotation` (`self.Icon`))) 180.0))
  (`KismetMaterialLibrary.SetScalarParameterValue` "/Game/TreePackBeech2/Materials/CollectionParamaters/MP_WindParameters.MP_WindParameters" "Strenght (0-5)" (`self.Wind Strenght`))
  (`KismetMaterialLibrary.SetScalarParameterValue` "/Game/TreePackBeech2/Materials/CollectionParamaters/MP_WindParameters.MP_WindParameters" "Low Amount(0-5)" (`self.Simple Wind Amount`))
  (`KismetMaterialLibrary.SetScalarParameterValue` "/Game/TreePackBeech2/Materials/CollectionParamaters/MP_WindParameters.MP_WindParameters" "Low Speed(0-5)" (`self.Simple Wind Speed`))
  (`KismetMaterialLibrary.SetVectorParameterValue` "/Game/TreePackBeech2/Materials/CollectionParamaters/MPC_Tree_Seasons.MPC_Tree_Seasons" "Leaves - Growth / Flowers - Bloom" (`KismetMathLibrary.MakeColor` (`self.Leaves Growth Start`) (`self.Leaves Growth End`) (`self.Flowers Bloom Start`) (`self.Flowers Bloom End`)))
  (`KismetMaterialLibrary.SetVectorParameterValue` "/Game/TreePackBeech2/Materials/CollectionParamaters/MPC_Tree_Seasons.MPC_Tree_Seasons" "Leaves Fall / Apples - On" (`KismetMathLibrary.MakeColor` (`self.Leaves Fall Start Shift`) (`self.Leaves Fall Start All`) (`self.Apples Start`) (`self.Apples End`)))
  (`KismetMaterialLibrary.SetVectorParameterValue` "/Game/TreePackBeech2/Materials/CollectionParamaters/MPC_Tree_Seasons.MPC_Tree_Seasons" "Leaves Color Shift" (`KismetMathLibrary.MakeColor` (`self.Spring / Summer`) (`self.Summer / Autumn`) (`self.Autumn01 / Autumn02`) (`self.Autumn02 / Winter`)))
  (`KismetMaterialLibrary.SetScalarParameterValue` "/Game/TreePackBeech2/Materials/CollectionParamaters/MPC_Tree_Seasons.MPC_Tree_Seasons" "DAY" (`self.Day of year`)))