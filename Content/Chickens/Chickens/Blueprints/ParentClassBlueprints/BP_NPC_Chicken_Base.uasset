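; Base Character Blueprint for chicken NPCs, covering melee combat and death.
; A Tick-driven gate smoothly turns the chicken toward its Blackboard enemy, while a lunge event launches it forward with temporarily lowered gravity and friction.
; During attacks, Box overlaps knock back "ChickenEnemy"-tagged characters and apply delayed damage, throttled by a DoOnce.
; Any damage received kills it outright, ragdolling the mesh before delayed destruction and garbage collection.
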(event `self.ReceiveBeginPlay`)

(event `RotateToFace_Enemy`
  (bind _returnvalue (`BlackboardComponent.GetValueAsObject` (`AIBlueprintHelperLibrary.GetBlackboard` null) (`self.BBKey_Enemy`)))
  ;[1 1 1] face the Enemy While Attacking
  (goto _label :!via `Open`))

(event `Stop_Facing_Enemy`
  (bind _returnvalue (`BlackboardComponent.GetValueAsObject` (`AIBlueprintHelperLibrary.GetBlackboard` null) (`self.BBKey_Enemy`)))
  ;[1 1 1] face the Enemy While Attacking
  (goto _label :!via `Close`))

(event `self.ReceiveTick`
  (params (DeltaSeconds :type "Float (single-precision)"))
  (bind _returnvalue (`BlackboardComponent.GetValueAsObject` (`AIBlueprintHelperLibrary.GetBlackboard` null) (`self.BBKey_Enemy`)))
  ;[1 1 1] TICK
  ;[1 1 1] face the Enemy While Attacking
  (`/Engine/EditorBlueprintResources/StandardMacros.Gate` true :!label _label
    (:`Exit`
      (if (`KismetSystemLibrary.IsValid` _returnvalue)
        (bind _asactor (cast `Actor` _returnvalue))
        (`self.K2_SetActorRotation` (`KismetMathLibrary.MakeRotator` 0.0 0.0 (.yaw (`KismetMathLibrary.RInterpTo` (`self.K2_GetActorRotation`) (`KismetMathLibrary.FindLookAtRotation` (`self.K2_GetActorLocation`) (`self.K2_GetActorLocation` _asactor)) (`GameplayStatics.GetWorldDeltaSeconds`) 1.0))))))))

(event `self.Box.OnComponentBeginOverlap`
  (params (OverlappedComponent :type "PrimitiveComponent Object Reference") (OtherActor :type "Actor Object Reference") (OtherComp :type "PrimitiveComponent Object Reference") (OtherBodyIndex :type Integer) (bFromSweep :type Boolean) (SweepResult :type "HitResult Structure (by ref)"))
  ;[1 1 1] KnockBack enemy and do damage while playing attack animation
  (if (`self.AmI Alive?`)
    (if (`self.CanHurtTheEnemy?`)
      (for _array_element (`PrimitiveComponent.GetOverlappingActors` (`self.Box`) "/Script/Engine.Actor")
        (if (`self.ActorHasTag` _array_element "ChickenEnemy")
          (bind _ascharacter (cast `Character` _array_element))
          (if (`self.IsAttacking?`)
            (`/Engine/EditorBlueprintResources/StandardMacros.DoOnce` false :!label _label_2
              (:`Completed`
                (`self.LaunchCharacter` _ascharacter (`KismetMathLibrary.ClampVectorSize` (* (- (`self.K2_GetActorLocation` _ascharacter) (`SceneComponent.K2_GetComponentLocation` (`self.Mesh`))) 1.8) 0.0 300.0) true true)
                (`KismetSystemLibrary.Delay` 0.2)
                (`GameplayStatics.ApplyDamage` _ascharacter (`self.MeleeDamageAmount`) null self)
                (`KismetSystemLibrary.RetriggerableDelay` 1.0)
                (goto _label_2 :!via `Reset`)))))))))

(event `self.ReceiveAnyDamage`
  (params (Damage :type "Float (single-precision)") (DamageType :type "DamageType Object Reference") (InstigatedBy :type "Controller Object Reference") (DamageCauser :type "Actor Object Reference"))
  ;[1 1 1] Damage
  (set `self.AmI Alive?` false)
  (`SkeletalMeshComponent.SetAllBodiesSimulatePhysics` (`self.Mesh`) true)
  (`KismetSystemLibrary.Delay` (`self.StayDeadBeforDestroyTime`))
  (`self.K2_DestroyActor`)
  (`KismetSystemLibrary.CollectGarbage`))

(event `self.Box.OnComponentEndOverlap`
  (params (OverlappedComponent :type "PrimitiveComponent Object Reference") (OtherActor :type "Actor Object Reference") (OtherComp :type "PrimitiveComponent Object Reference") (OtherBodyIndex :type Integer))
  ;[1 1 1] KnockBack enemy and do damage while playing attack animation
  (goto _label_2 :!via `Reset`))

(event `LaunchForwardForAttack`
  (bind _charactermovement (`self.CharacterMovement`))
  (bind _updatedcomponent (`MovementComponent.UpdatedComponent` _charactermovement))
  ;[1 1 1] Launch Character Forward during attack animation
  (if (`self.AmI Alive?`)
    (set `CharacterMovementComponent.GravityScale` 0.4 (`self.CharacterMovement`))
    (set `CharacterMovementComponent.GroundFriction` 1.0 (`self.CharacterMovement`))
    (`self.LaunchCharacter` (+ (`MovementComponent.Velocity` _charactermovement) (* (`SceneComponent.GetForwardVector` _updatedcomponent) 1000.0) (* (`SceneComponent.GetUpVector` _updatedcomponent) 40.0)) true true)
    (`KismetSystemLibrary.RetriggerableDelay` 1.0)
    (set `CharacterMovementComponent.GroundFriction` 4.0 (`self.CharacterMovement`))
    (set `CharacterMovementComponent.GravityScale` 1.0 (`self.CharacterMovement`))))

(fn `UserConstructionScript`)