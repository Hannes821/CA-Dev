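; BP_Egg is a health pickup that the player eats by walking into it.
; When its sphere overlaps the player character, it plays a pickup sound and adds health to BP_ThirdPersonCharacter without clamping.
; It then writes the new value straight into the WBP_Health progress bar, destroys itself and prints a message.
; A failed cast to the character or widget stops the chain, leaving the egg in place.
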(event `self.ReceiveBeginPlay`)

(event `self.Sphere.OnComponentBeginOverlap`
  (params (OverlappedComponent :type "PrimitiveComponent Object Reference") (OtherActor :type "Actor Object Reference") (OtherComp :type "PrimitiveComponent Object Reference") (OtherBodyIndex :type Integer) (bFromSweep :type Boolean) (SweepResult :type "HitResult Structure (by ref)"))
  ;[1 1 1] Check if is the Player
  (if (== OtherActor (`GameplayStatics.GetPlayerCharacter` 0))
    (`GameplayStatics.PlaySoundAtLocation` "/Game/Chickens/Demo_Content/Environment/Sounds/Random_Health_Pickup_Cue.Random_Health_Pickup_Cue" (`self.K2_GetActorLocation` OtherActor) (struct) 0.2 0.3 0.0 "/Game/Chickens/Chickens/Sound/Chicken_SoundAttenuation.Chicken_SoundAttenuation" null null null)
    ;[1 1 1] Add some heath to the health widget
    (bind _asbp_third_person_character (cast `/Game/Chickens/Demo_Content/ThirdPersonBP/Blueprints/BP_ThirdPersonCharacter` OtherActor))
    (bind _output_get (set `/Game/Chickens/Chickens/Blueprints/ParentClassBlueprints/BP_CharacterBaseWithHealth.Health` (+ (`/Game/Chickens/Chickens/Blueprints/ParentClassBlueprints/BP_CharacterBaseWithHealth.Health` _asbp_third_person_character) 20.0) _asbp_third_person_character))
    (bind _aswbp_health (cast `/Game/Chickens/Demo_Content/ThirdPersonBP/Blueprints/WBP_Health` (`/Game/Chickens/Demo_Content/ThirdPersonBP/Blueprints/BP_ThirdPersonCharacter.HealthBarWidget` _asbp_third_person_character)))
    (`ProgressBar.SetPercent` (`/Game/Chickens/Demo_Content/ThirdPersonBP/Blueprints/WBP_Health.ProgressBar_46` _aswbp_health) (/ _output_get 100.0))
    ;[1 1 1] Destroy Egg
    (`self.K2_DestroyActor`)
    (`KismetSystemLibrary.PrintString` "Ate an Egg")))

(fn `UserConstructionScript`)