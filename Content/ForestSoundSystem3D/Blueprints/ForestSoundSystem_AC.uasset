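; Forest ambience controller that plays day and night loops plus randomly timed bird, woodpecker, owl, cuckoo and wolf calls.
; Each enabled call re-arms its own one-shot timer, playing with randomized volume at a random bearing 5000 units from the player.
; BeginPlay runs both sets together, using sound mix class overrides to silence night by default.
; The day/night switch logic is present but unconnected, so it never runs.
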(event `EventBird1`
  (bind (_bird1_play _bird1_volume _bird1_intervalrange _bird1_volumerandomness) (break `/Game/ForestSoundSystem3D/Blueprints/SoundSettings` (`self.Bird1`)))
  (bind (_x _y) (`KismetMathLibrary.BreakVector2D` _bird1_intervalrange))
  ;[1 1 1] Day Sounds
  (`KismetSystemLibrary.K2_SetTimerDelegate` (delegate `EventBird1`) (`KismetMathLibrary.RandomFloatInRange` _x _y) :!label _label)
  (`GameplayStatics.PlaySoundAtLocation` "/Game/ForestSoundSystem3D/Sounds/SoundCues/Bird1_Cue.Bird1_Cue" (`self.SoundLocation`) (struct) (* _bird1_volume (`KismetMathLibrary.RandomFloatInRange` (- 1.0 _bird1_volumerandomness) 1.0)) 1.0 0.0 null null null null))

(event `Key|Two`
  (params (Key :type "Key Structure")))

(event `Key|One`
  (params (Key :type "Key Structure")))

(event `BlacbirdEvent`
  (bind (_blackbird_play _blackbird_volume _blackbird_intervalrange _blackbird_volumerandomness) (break `/Game/ForestSoundSystem3D/Blueprints/SoundSettings` (`self.Blackbird`)))
  (bind (_x _y) (`KismetMathLibrary.BreakVector2D` _blackbird_intervalrange))
  ;[1 1 1] Day Sounds
  (`KismetSystemLibrary.K2_SetTimerDelegate` (delegate `BlacbirdEvent`) (`KismetMathLibrary.RandomFloatInRange` _x _y) :!label _label_2)
  (`GameplayStatics.PlaySoundAtLocation` "/Game/ForestSoundSystem3D/Sounds/SoundCues/Blackbird_Cue.Blackbird_Cue" (`self.SoundLocation`) (struct) (* _blackbird_volume (`KismetMathLibrary.RandomFloatInRange` (- 1.0 _blackbird_volumerandomness) 1.0)) 1.0 0.0 null null null null))

(event `EventWoodpecker`
  (bind (_woodpecker_play _woodpecker_volume _woodpecker_intervalrange _woodpecker_volumerandomness) (break `/Game/ForestSoundSystem3D/Blueprints/SoundSettings` (`self.Woodpecker`)))
  (bind (_x _y) (`KismetMathLibrary.BreakVector2D` _woodpecker_intervalrange))
  ;[1 1 1] Day Sounds
  (`KismetSystemLibrary.K2_SetTimerDelegate` (delegate `EventWoodpecker`) (`KismetMathLibrary.RandomFloatInRange` _x _y) :!label _label_3)
  (`GameplayStatics.PlaySoundAtLocation` "/Game/ForestSoundSystem3D/Sounds/SoundCues/Woodpecker_Cue.Woodpecker_Cue" (`self.SoundLocation`) (struct) (* _woodpecker_volume (`KismetMathLibrary.RandomFloatInRange` (- 1.0 _woodpecker_volumerandomness) 1.0)) 1.0 0.0 null null null null))

(event `self.ReceiveBeginPlay`
  (bind (_bird2_play _bird2_volume _bird2_intervalrange _bird2_volumerandomness) (break `/Game/ForestSoundSystem3D/Blueprints/SoundSettings` (`self.Bird2`)))
  (bind (_woodpecker_play _woodpecker_volume _woodpecker_intervalrange _woodpecker_volumerandomness) (break `/Game/ForestSoundSystem3D/Blueprints/SoundSettings` (`self.Woodpecker`)))
  (bind (_owl_play _owl_volume _owl_intervalrange _owl_volumerandomness) (break `/Game/ForestSoundSystem3D/Blueprints/SoundSettings` (`self.Owl`)))
  (bind (_bird1_play _bird1_volume _bird1_intervalrange _bird1_volumerandomness) (break `/Game/ForestSoundSystem3D/Blueprints/SoundSettings` (`self.Bird1`)))
  (bind (_blackbird_play _blackbird_volume _blackbird_intervalrange _blackbird_volumerandomness) (break `/Game/ForestSoundSystem3D/Blueprints/SoundSettings` (`self.Blackbird`)))
  (bind (_cuckoo_play _cuckoo_volume _cuckoo_intervalrange _cuckoo_volumerandomness) (break `/Game/ForestSoundSystem3D/Blueprints/SoundSettings` (`self.Cuckoo`)))
  (bind (_wolf_play _wolf_volume _wolf_intervalrange _wolf_volumerandomness) (break `/Game/ForestSoundSystem3D/Blueprints/SoundSettings` (`self.Wolf`)))
  (bind (_x _y) (`KismetMathLibrary.BreakVector2D` _owl_intervalrange))
  (bind (_x_2 _y_2) (`KismetMathLibrary.BreakVector2D` _wolf_intervalrange))
  (bind (_x_3 _y_3) (`KismetMathLibrary.BreakVector2D` _bird2_intervalrange))
  (bind (_x_4 _y_4) (`KismetMathLibrary.BreakVector2D` _cuckoo_intervalrange))
  ;[1 1 1] Instead of here you can set it up in project settings under "Base Sound Mix"
  (`GameplayStatics.SetBaseSoundMix` "/Game/ForestSoundSystem3D/Sounds/SoundClasses/ForestSoundMix.ForestSoundMix")
  ;[1 1 1] Setting Up Day sounds as default
  (`GameplayStatics.SetSoundMixClassOverride` "/Game/ForestSoundSystem3D/Sounds/SoundClasses/ForestSoundMix.ForestSoundMix" "/Game/ForestSoundSystem3D/Sounds/SoundClasses/NightForest.NightForest" 0.0 1.0 0.0)
  (`GameplayStatics.SetSoundMixClassOverride` "/Game/ForestSoundSystem3D/Sounds/SoundClasses/ForestSoundMix.ForestSoundMix" "/Game/ForestSoundSystem3D/Sounds/SoundClasses/DayForest.DayForest" 1.0 1.0 0.0)
  (bind _returnvalue (`GameplayStatics.SpawnSound2D` "/Game/ForestSoundSystem3D/Sounds/SoundCues/ForestDayLoop_Cue.ForestDayLoop_Cue" 1.0 1.0 0.0 null :!pinned true)) ; Day Loop
  (set `self.ForestDaySoundLoop` _returnvalue)
  (bind _returnvalue_2 (`GameplayStatics.SpawnSound2D` "/Game/ForestSoundSystem3D/Sounds/SoundCues/ForestNightLoop_Cue.ForestNightLoop_Cue" 1.0 1.0 0.0 null :!pinned true)) ; Night Loop
  (set `self.ForestNightSoundLoop` _returnvalue_2)
  (`|ExecutionSequence`
    (:`then_0`
      ;[1 1 1] Day Sounds
      (`|ExecutionSequence`
        (:`then_0`
          (if _bird1_play
            (`KismetSystemLibrary.Delay` (`KismetMathLibrary.RandomFloatInRange` 0.0 (/ (`KismetMathLibrary.BreakVector2D` _bird1_intervalrange) 2.0))) ; Delay of the First sound
            (goto _label)))
        (:`then_1`
          (if _blackbird_play
            (`KismetSystemLibrary.Delay` (`KismetMathLibrary.RandomFloatInRange` 0.0 (/ (`KismetMathLibrary.BreakVector2D` _blackbird_intervalrange) 2.0)))
            (goto _label_2)))
        (:`then_2`
          (if _woodpecker_play
            (`KismetSystemLibrary.Delay` (`KismetMathLibrary.RandomFloatInRange` 0.0 (`KismetMathLibrary.BreakVector2D` _woodpecker_intervalrange)))
            (goto _label_3)))))
    (:`then_1`
      ;[1 1 1] Night Sounds
      (`|ExecutionSequence`
        (:`then_0`
          (if _bird2_play
            (`KismetSystemLibrary.Delay` (`KismetMathLibrary.RandomFloatInRange` 0.0 (/ _x_3 2.0)))
            (`KismetSystemLibrary.K2_SetTimerDelegate` (delegate `EventBird2`) (`KismetMathLibrary.RandomFloatInRange` _x_3 _y_3) :!label _label_4)
            (`GameplayStatics.PlaySoundAtLocation` "/Game/ForestSoundSystem3D/Sounds/SoundCues/Bird2_Cue.Bird2_Cue" (`self.SoundLocation`) (struct) (* _bird2_volume (`KismetMathLibrary.RandomFloatInRange` (- 1.0 _bird2_volumerandomness) 1.0)) 1.0 0.0 null null null null)))
        (:`then_1`
          (if _owl_play
            (`KismetSystemLibrary.Delay` (`KismetMathLibrary.RandomFloatInRange` 0.0 (/ _x 2.0)))
            (`KismetSystemLibrary.K2_SetTimerDelegate` (delegate `EventOwl`) (`KismetMathLibrary.RandomFloatInRange` _x _y) :!label _label_5)
            (`GameplayStatics.PlaySoundAtLocation` "/Game/ForestSoundSystem3D/Sounds/SoundCues/Owl_Cue.Owl_Cue" (`self.SoundLocation`) (struct) (* _owl_volume (`KismetMathLibrary.RandomFloatInRange` (- 1.0 _owl_volumerandomness) 1.0)) 1.0 0.0 null null null null)))
        (:`then_2`
          (if _cuckoo_play
            (`KismetSystemLibrary.Delay` (`KismetMathLibrary.RandomFloatInRange` 0.0 (/ _x_4 4.0)))
            (`KismetSystemLibrary.K2_SetTimerDelegate` (delegate `EventCuckoo`) (`KismetMathLibrary.RandomFloatInRange` _x_4 _y_4) :!label _label_6)
            (`GameplayStatics.PlaySoundAtLocation` "/Game/ForestSoundSystem3D/Sounds/SoundCues/Cocko_Cue.Cocko_Cue" (`self.SoundLocation`) (struct) (* _cuckoo_volume (`KismetMathLibrary.RandomFloatInRange` (- 1.0 _cuckoo_volumerandomness) 1.0)) 1.0 0.0 null null null null)))
        (:`then_3`
          (if _wolf_play
            (`KismetSystemLibrary.Delay` (`KismetMathLibrary.RandomFloatInRange` 0.0 (/ _x_2 4.0)))
            (`KismetSystemLibrary.K2_SetTimerDelegate` (delegate `EventWolf`) (`KismetMathLibrary.RandomFloatInRange` _x_2 _y_2) :!label _label_7)
            (`GameplayStatics.PlaySoundAtLocation` "/Game/ForestSoundSystem3D/Sounds/SoundCues/Wolf_Cue.Wolf_Cue" (`self.SoundLocation`) (struct) (* _wolf_volume (`KismetMathLibrary.RandomFloatInRange` (- 1.0 _wolf_volumerandomness) 1.0)) 1.0 0.0 null null null null)))))))

(event `EventBird2`
  ;[1 1 1] Night Sounds
  (goto _label_4))

(event `EventOwl`
  ;[1 1 1] Night Sounds
  (goto _label_5))

(event `EventCuckoo`
  ;[1 1 1] Night Sounds
  (goto _label_6))

(event `EventWolf`
  ;[1 1 1] Night Sounds
  (goto _label_7))

(fn `SoundLocation`
  (returns (ReturnValue :type "Vector Structure"))
  (return (+ (`Actor.K2_GetActorLocation` (`GameplayStatics.GetPlayerPawn` 0)) (`KismetMathLibrary.GreaterGreater_VectorRotator` (`KismetMathLibrary.MakeVector` 5000.0) (`KismetMathLibrary.MakeRotator` 0.0 0.0 (`KismetMathLibrary.RandomFloatInRange` 0.0 360.0))))))