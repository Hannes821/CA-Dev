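; BP_Chest-10_2 is a configurable medieval chest prop from the menu's 3D furniture assets.
; Its construction script uses shared macros to toggle visibility and collision on the chest body and on two cap meshes, driven by CapEnabled and ChestEnabled.
; It also rotates both cap meshes from the negated CapRotation and CapConnectRotation values to pose the lid.
; The event graph holds only disabled stub events, so there is no runtime logic.
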(fn `UserConstructionScript`
  (bind _staticmeshcomponent02 (`self.StaticMeshComponent02`))
  (bind _cap_enabled (`self.Cap Enabled`))
  (`|ExecutionSequence`
    (:`then_0`
      ;[1 1 1] Enable/disable. Macro (Visibility and Enable/Disable collision)
      (`/Game/CA_UI/MainMenu_3DAssets/Medieval_Props_Furniture/Blueprints/Macros/Enabled_Disabled_Macro.Enabled/Disabled_Macro` _cap_enabled _staticmeshcomponent02
        (:`Resume`
          (`/Game/CA_UI/MainMenu_3DAssets/Medieval_Props_Furniture/Blueprints/Macros/Enabled_Disabled_Macro.Enabled/Disabled_Macro` _cap_enabled (`self.StaticMeshComponent0`)))))
    (:`then_1`
      ;[1 1 1] Set Components Rotation
      (`/Game/CA_UI/MainMenu_3DAssets/Medieval_Props_Furniture/Blueprints/Macros/Rotation_Macro.Relative_Rotation_Macro` _staticmeshcomponent02 (* (`self.Cap Rotation`) -1.0) 0.0 -90.0))
    (:`then_2`
      (`/Game/CA_UI/MainMenu_3DAssets/Medieval_Props_Furniture/Blueprints/Macros/Enabled_Disabled_Macro.Enabled/Disabled_Macro` (`self.Chest Enabled`) (`self.StaticMeshComponent01`)))
    (:`then_3`
      (`/Game/CA_UI/MainMenu_3DAssets/Medieval_Props_Furniture/Blueprints/Macros/Rotation_Macro.Relative_Rotation_Macro` (`self.StaticMeshComponent0`) (* (`self.Cap Connect Rotation`) -1.0)))))