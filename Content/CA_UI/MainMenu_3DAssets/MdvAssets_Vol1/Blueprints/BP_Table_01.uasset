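; BP_Table_01 is a table prop actor with four optional tablecloth components, stored among the main menu 3D assets.
; The construction script reads the ClothA to ClothD booleans and shows or hides the matching cloth component without propagating to children.
; Each toggle is independent, so several cloths can be visible at once.
; The event graph holds only disabled default events, so the actor has no runtime logic.
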(fn `UserConstructionScript`
  (bind _mdv_table_cloth (`self.Mdv_Table_Cloth`))
  (bind _mdv_tableclothb (`self.Mdv_TableClothB`))
  (bind _mdv_tableclothc (`self.Mdv_TableClothC`))
  (bind _mdv_tableclothd (`self.Mdv_TableClothD`))
  (if (`self.Cloth A`)
    (`SceneComponent.SetVisibility` _mdv_table_cloth true false)
    (else
      (`SceneComponent.SetVisibility` _mdv_table_cloth false false)))
  (if (`self.Cloth B`)
    (`SceneComponent.SetVisibility` _mdv_tableclothb true false)
    (else
      (`SceneComponent.SetVisibility` _mdv_tableclothb false false)))
  (if (`self.Cloth C`)
    (`SceneComponent.SetVisibility` _mdv_tableclothc true false)
    (else
      (`SceneComponent.SetVisibility` _mdv_tableclothc false false)))
  (if (`self.Cloth D`)
    (`SceneComponent.SetVisibility` _mdv_tableclothd true false)
    (else
      (`SceneComponent.SetVisibility` _mdv_tableclothd false false))))