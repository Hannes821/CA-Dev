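; Player controller for a game with building and resources, handling local UI setup and camera input.
; BeginPlay creates the main UI for local controllers and sets game-and-UI input.
; Holding Pan opens a gate that feeds mouse X into camera panning while suspending edge scroll.
; The V key is a prototype camera toggle and resource debug print; older construction placement logic remains unconnected, alongside empty test events.
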(event `self.ReceiveBeginPlay`
  ;[1 1 1] spawn widgets on local machines
  (if (`self.IsLocalPlayerController`)
    (bind _returnvalue (`|CreateWidget` "/Game/Core/Widgets/WBP_MainUI.WBP_MainUI_C" self))
    (bind _output_get (set `self.MainUI` _returnvalue))
    (`UserWidget.AddToViewport` _output_get 0)
    (`WidgetBlueprintLibrary.SetInputMode_GameAndUIEx` self _output_get "DoNotLock" false)))

(event `self.ReceiveTick`
  (params (DeltaSeconds :type "Float (single-precision)")))

(event `ROC_Test`
  ;[1 1 1] Testing Events
)

(event `ROS_Test`
  ;[1 1 1] Testing Events
)

(event `MC_Test`
  ;[1 1 1] Testing Events
)

(event `ROC_Test2`
  ;[1 1 1] Testing Events
)

(event `ROS_Test2`
  ;[1 1 1] Testing Events
)

(event `InputAxisKey|MouseX`
  (params (AxisValue :type "Float (single-precision)"))
  ;[1 1 1] Rotate Preview
  (`/Engine/EditorBlueprintResources/StandardMacros.Gate` true :!label _label
    (:`Exit`
      (`CameraMovementComponent.PanCamera` (`self.CameraMovementRef`) (* AxisValue 5.0)))))

(event `InputAction|Pan`
  (params (Key :type "Key Structure"))
  (bind _cameramovementref (`self.CameraMovementRef`))
  ;[1 1 1] Rotate Preview
  (:`Pressed`
    (`CameraMovementComponent.SetDisableEdgeScroll` _cameramovementref true)
    (goto _label :!via `Open`))
  (:`Released`
    (`CameraMovementComponent.SetDisableEdgeScroll` _cameramovementref false)
    (goto _label :!via `Close`)))

(event `Key|Q`
  (params (Key :type "Key Structure"))
  ;[1 1 1] Testing Events
)

(event `Key|X`
  (params (Key :type "Key Structure"))
  ;[1 1 1] Testing Events
)

(event `Key|V`
  (params (Key :type "Key Structure"))
  (bind _resourcemanagerref (`self.ResourceManagerRef`))
  (bind _pawnmovementcomponent (`CameraPawn.PawnMovementComponent` (`self.CameraPawnRef`)))
  ;[0.2186 0.5312 0.2186] CURRENT PROTOTYPES
  ;;[1 1 1] Convert to fully functional C++ later
  (:`Pressed`
    (bind _isa (`/Engine/EditorBlueprintResources/StandardMacros.FlipFlop`)
      (:`A`
        _)
      (:`B`
        _))
    (`CameraMovementComponent.SetCameraDiabled` _pawnmovementcomponent _isa)
    (`CameraMovementComponent.SetDisableEdgeScroll` _pawnmovementcomponent _isa)
    (`self.TestSet` "Clay")
    (`KismetSystemLibrary.PrintString` (`KismetStringLibrary.Concat_StrStr` "Clay In: " (`KismetStringLibrary.Conv_DoubleToString` (`self.DebugValueFloat`))) true true (struct :`G` 0.66 :`B` 1.0 :`A` 1.0) 10.0)
    (`self.TestSet` "WoodBeam")
    (`KismetSystemLibrary.PrintString` (`KismetStringLibrary.Concat_StrStr` "Wood In: " (`KismetStringLibrary.Conv_DoubleToString` (`self.DebugValueFloat`))) true true (struct :`G` 0.66 :`B` 1.0 :`A` 1.0) 10.0)
    (bind _returnvalue (`ResourceManagerBase.GetCurrentResourceAmount` _resourcemanagerref "Clay"))
    (`KismetSystemLibrary.PrintString` (`KismetStringLibrary.Concat_StrStr` "Clay Out: " (`KismetStringLibrary.Conv_DoubleToString` _returnvalue)) true true (struct :`R` 1.0 :`A` 1.0) 10.0)
    (bind _returnvalue_2 (`ResourceManagerBase.GetCurrentResourceAmount` _resourcemanagerref "WoodBeam"))
    (`KismetSystemLibrary.PrintString` (`KismetStringLibrary.Concat_StrStr` "Wood Out: " (`KismetStringLibrary.Conv_DoubleToString` _returnvalue_2)) true true (struct :`R` 1.0 :`A` 1.0) 10.0)))

(event `InputAction|PrimaryAction`
  (params (Key :type "Key Structure"))
  ;[1 0 0] OLD PROTOTYPES
  ;;[1 1 1] Primary Action Construction (no resourcees)
)

(fn `UserConstructionScript`)