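; Prototype Blueprint that rotates the referenced sun actor to match the in-game time of day.
; On BeginPlay it caches the RTSGameState as the clock source.
; Each Tick converts that state's hours, minutes and seconds into fractional hours, maps the negated 24-hour cycle to 360 degrees of pitch, and adds a 90-degree offset.
; A note on the graph marks logic not to be duplicated into the C++ version.
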(event `self.ReceiveBeginPlay`
  ;[1 1 1] DO NOT DUPLICATE INTO THE C++ VERSION!
  (bind _asrtsgame_state (cast `RTSGameState` (`GameplayStatics.GetGameState`)))
  (set `self.GameStateRef` _asrtsgame_state))

(event `self.ReceiveTick`
  (params (DeltaSeconds :type "Float (single-precision)"))
  (bind _datetimestruct (`RTSGameState.DateTimeStruct` (`self.GameStateRef`)))
  (`self.K2_SetActorRotation` (`self.SunRef`) (`KismetMathLibrary.MakeRotator` 0.0 (+ (* (/ (mod (* (+ (`KismetMathLibrary.Conv_IntToDouble` (`KismetMathLibrary.GetHour` _datetimestruct)) (/ (`KismetMathLibrary.Conv_IntToDouble` (`KismetMathLibrary.GetMinute` _datetimestruct)) 60.0) (/ (`KismetMathLibrary.Conv_IntToDouble` (`KismetMathLibrary.GetSecond` _datetimestruct)) 3600.0)) -1.0) 24.0) 24.0) 360.0) 90.0)) false))

(fn `UserConstructionScript`)