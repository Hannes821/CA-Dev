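; BP_UnitMasterBasePrototype is a prototype base Blueprint for units, configured as foot or non-foot by the IsFootUnit flag.
; Its Construction Script makes either the capsule or box collision the DefaultSceneRoot and destroys the other.
; Both branches assign the same mannequin skeletal mesh, which is then attached to the root component with relative transforms.
; The Event Graph contains only disabled placeholder events.
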(fn `UserConstructionScript`
  ;[1 1 1] SetUnitType()
  (if (`self.bIsFootUnit`)
    (set `self.DefaultSceneRoot` (`self.CapsuleCollision`))
    (`ActorComponent.K2_DestroyComponent` (`self.BoxCollision`))
    (`SkinnedMeshComponent.SetSkinnedAssetAndUpdate` (`self.UnitMesh`) "/Game/Meshes/Placeholder/Character/SK_Mannequin.SK_Mannequin" true)
    (else
      (set `self.DefaultSceneRoot` (`self.BoxCollision`))
      (`ActorComponent.K2_DestroyComponent` (`self.CapsuleCollision`))
      (`SkinnedMeshComponent.SetSkinnedAssetAndUpdate` (`self.UnitMesh`) "/Game/Meshes/Placeholder/Character/SK_Mannequin.SK_Mannequin" true)))
  ;[1 1 1] AttachSkelMeshToRoot()
  (`SceneComponent.K2_AttachToComponent` (`self.UnitMesh`) (`self.RootComponent`) "None" "KeepRelative" "KeepRelative" "KeepRelative" true))