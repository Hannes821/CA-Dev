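; Prototype master resource actor that sets up its mesh and amount from data at construction.
; The construction script reads the WoodBeam row of DT_ResourcesProto and applies the first base mesh to ResourceMesh.
; Amount is the row's base amount multiplied by the product of the mesh's world scale axes, so scaled instances hold proportional resources.
; The row name is fixed, and the event graph holds only disabled placeholder events.
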(fn `UserConstructionScript`
  (bind _returnvalue (`|GetDataTableRow` "/Game/Core/PrototypingFolder/Resources/DT_ResourcesProto.DT_ResourcesProto" "WoodBeam")
    (:`then`
      (bind (_resource _basemeshes _baseamount) (break `/Game/Core/PrototypingFolder/Resources/F_ResourcesDetailsPROTO` _returnvalue))
      (`StaticMeshComponent.SetStaticMesh` (`self.ResourceMesh`) (`|GetArrayItem` _basemeshes))
      (set `self.Amount` (* _baseamount (* (.x (`SceneComponent.K2_GetComponentScale` (`self.ResourceMesh`))) (.y (`SceneComponent.K2_GetComponentScale` (`self.ResourceMesh`))) (.z (`SceneComponent.K2_GetComponentScale` (`self.ResourceMesh`)))))))))