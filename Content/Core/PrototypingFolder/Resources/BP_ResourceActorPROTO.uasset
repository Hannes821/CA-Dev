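; BP_ResourceActorPROTO is a prototype harvestable resource actor, currently hard-coded to the Tree row of DT_Resources.
; For non-Building deposits, the construction script picks a static mesh from the row's BaseMesh array using the GameState's season.
; It then sizes the HarvestArea box from the mesh's scaled local bounds, optionally raising it.
; Season and time functions are stubs returning fixed values, and the event graph has no live logic.
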(fn `GetSeason`
  (returns (ReturnValue :type "ESeasons Enum"))
  (return "SeasonWinter"))

(fn `SetGameDateTime`
  (params (TimeStruct :type "DateTime Structure"))
  (returns (ReturnValue :type Boolean))
  (return false))

(fn `SetGameDay`
  (params (GameDay :type Integer))
  (returns (ReturnValue :type Boolean))
  (return false))

(fn `SetGameSpeedInt`
  (params (GameSpeed :type "Float (single-precision)"))
  (returns (ReturnValue :type Boolean))
  (return false))

(fn `SetHarvestableArea`
  (bind _harvestarea (`self.HarvestArea`))
  (bind _returnvalue (* (`.Max` (`StaticMeshComponent.GetLocalBounds` (`self.ResourceMesh`))) (`self.CustomCollisionSize`)))
  (`BoxComponent.SetBoxExtent` _harvestarea _returnvalue true)
  (if (`self.bAdjustCollisionOffset`)
    (`SceneComponent.K2_AddLocalOffset` _harvestarea (`KismetMathLibrary.MakeVector` 0.0 0.0 (.z _returnvalue)) false true)))

(fn `UpdateMesh`
  (params (ResourceStruct :type "ResourceStruct Structure (by ref)"))
  (bind _returnvalue (message `GameTimeInterface.GetSeason` (`GameplayStatics.GetGameState`)))
  (set `self.Season` _returnvalue)
  (`StaticMeshComponent.SetStaticMesh` (`self.ResourceMesh`) (`|GetArrayItem` (`.BaseMesh` (break `ResourceStruct` ResourceStruct)) (select `ESeasons` (`self.Season`) :`SeasonWinter` 3 :`SeasonSpring` 2 :`SeasonFall` 1))))

(fn `UserConstructionScript`
  (bind _returnvalue (`|GetDataTableRow` "/Game/Core/DataTables/DT_Resources.DT_Resources" "Tree")
    (:`then`
      (if (`|EnumInequality` (`.DepositType` (break `ResourceStruct` _returnvalue)) "Building")
        (`self.UpdateMesh` _returnvalue)
        (`self.SetHarvestableArea`)))
    (:`RowNotFound`
      (`KismetSystemLibrary.PrintString` "Resource Error"))))